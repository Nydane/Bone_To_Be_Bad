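; BP_MovingRaft is a raft that travels once along a spline and drops loot on the way.
; On BeginPlay, if CanMove is set, a timeline scaled by Duration sets its location and rotation from the SplineManager's spline.
; Tick watches the timeline alpha, spawning a coin spawner and a grabbable gold bag once near the midpoint, then destroying the raft at the end.
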(event `self.ReceiveBeginPlay`
  (if (`self.CanMove`)
    (`self.MoveRaft`)))

(event `MoveRaft`
  (bind _returnvalue (`KismetMathLibrary.Lerp` 0.0 (`SplineComponent.GetSplineLength` (`/Game/EveryoneProg/Ships/SplineManager.Spline` (`self.SplineManager`))) (`self.Alpha`)))
  ;[1 1 1] Gère seulement le mouvement du Raft, il faudra ajouter d'autres CE ou passer par l'Event Tick pour les autres Behaviours.
  (`TimelineComponent.SetPlayRate` (`self.Movement`) (/ 1.0 (`self.Duration`)))
  (bind (_direction _alpha) (`Timeline|Movement`)
    (:`Update`
      (set `self.Alpha` _alpha)
      (`self.K2_SetActorLocationAndRotation` (`SplineComponent.GetLocationAtDistanceAlongSpline` (`/Game/EveryoneProg/Ships/SplineManager.Spline` (`self.SplineManager`)) _returnvalue "World") (`SplineComponent.GetRotationAtDistanceAlongSpline` (`/Game/EveryoneProg/Ships/SplineManager.Spline` (`self.SplineManager`)) _returnvalue "World")))
    (:`Finished`
      (set `self.CanMove` false))))

(event `self.ReceiveTick`
  (params (DeltaSeconds :type "Float (single-precision)"))
  (bind _numbercoinstospawn (`self.NumberCoinsToSpawn`))
  (`|ExecutionSequence`
    (:`then_0`
      (if (`KismetMathLibrary.NearlyEqual_FloatFloat` (`self.Alpha`) 0.51 0.01)
        (`/Engine/EditorBlueprintResources/StandardMacros.DoOnce` false
          (:`Completed`
            (`|ExecutionSequence`
              (:`then_0`
                (`|SpawnActorFromClass` "/Game/EveryoneProg/Managers/BP_CoinSpawner.BP_CoinSpawner_C" (`KismetMathLibrary.MakeTransform` (`SceneComponent.K2_GetComponentLocation` (`self.Scene`))) "Undefined" "OverrideRootScale" null (70.0 70.0 40.0) 0.05 _numbercoinstospawn _numbercoinstospawn true true null))
              (:`then_1`
                (`|SpawnActorFromClass` "/Game/EveryoneProg/Deliveries/BP_GoldBag_WithGrab.BP_GoldBag_WithGrab_C" (`KismetMathLibrary.MakeTransform` (`SceneComponent.K2_GetComponentLocation` (`self.Scene`))) "Undefined" "OverrideRootScale" null 15 0 null)))))))
    (:`then_1`
      (if (`KismetMathLibrary.NearlyEqual_FloatFloat` (`self.Alpha`) 1.0 0.01)
        (`self.K2_DestroyActor` self)))))

(fn `UserConstructionScript`)