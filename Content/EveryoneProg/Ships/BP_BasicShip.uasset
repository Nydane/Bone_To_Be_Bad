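; Base ship actor whose type sets health, gold reward and movement mode in the construction script.
; Civil and Merchant ships ride a spline via timeline and self-destroy at the end.
; War and Ghost ships interpolate toward a target on Tick, enabling BehaviourAllowed once near it.
; At zero health, gold is split among all ThirdPersonCharacters and KillShip fires, an empty hook for children like ShipBehaviourTarget.
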(event `LerpToTarget`
  (params (DeltaSeconds :type "Float (double-precision)"))
  (bind _hull (`self.Hull`))
  ;[1 1 1] Extremely simple Lerp here, most of the logic will prolly be located within Ships that do use this snippet of  code
  (`SceneComponent.K2_SetWorldLocation` _hull (`KismetMathLibrary.VInterpTo` (`SceneComponent.K2_GetComponentLocation` _hull) (`SceneComponent.K2_GetComponentLocation` (`Actor.RootComponent` (`self.TargetToStopAt`))) DeltaSeconds (`self.InterpSpeed`)) false false)
  (if (== (`SceneComponent.K2_GetComponentLocation` (`self.Hull`)) (`SceneComponent.K2_GetComponentLocation` (`Actor.RootComponent` (`self.TargetToStopAt`))) :`ErrorTolerance` 500.0)
    (`/Engine/EditorBlueprintResources/StandardMacros.DoOnce` false
      (:`Completed`
        (set `self.BehaviourAllowed` true)))))

(event `self.ReceiveBeginPlay`
  ;[1 1 1] Are we Lerping or are we moving through a Timeline ?
  (if (`self.followingSpline`)
    (set `self.LocalSpline` (`/Game/EveryoneProg/Ships/SplineManager.Spline` (`self.SplineToFollow`)))
    (`KismetSystemLibrary.Delay` 2.0)
    (`self.ShipSplineMovement`)
    (else
      (`self.LerpToTarget` 0.0))))

(event `ShipSplineMovement`
  (bind _localspline (`self.LocalSpline`))
  (bind (_returnvalue_roll _returnvalue_pitch _returnvalue_yaw) (`KismetMathLibrary.BreakRotator` (`SplineComponent.GetRotationAtDistanceAlongSpline` (`self.LocalSpline`) 0.0 "Local")))
  ;[1 1 1] Shamelessly stolen from Jonathan!
  ;
  ; Takes each point on a given Spline and makes sure that the object will reach them while mainteaining a logical rotation, so the ships turns to follow the path laid by the Spline.
  (`SceneComponent.K2_SetRelativeRotation` (`self.Hull`) (`KismetMathLibrary.MakeRotator` _returnvalue_roll 0.0 _returnvalue_yaw) false false)
  (bind (_direction _traveldistance) (`Timeline|MoveShip`)
    (:`Update`
      (bind _returnvalue (* _traveldistance (`SplineComponent.GetSplineLength` (`self.LocalSpline`))))
      (`SceneComponent.K2_SetWorldLocation` (`self.Hull`) (`SplineComponent.GetLocationAtDistanceAlongSpline` _localspline _returnvalue "World") false false)
      (bind (_returnvalue_roll_2 _returnvalue_pitch_2 _returnvalue_yaw_2) (`KismetMathLibrary.BreakRotator` (`SplineComponent.GetRotationAtDistanceAlongSpline` _localspline _returnvalue "Local")))
      (`SceneComponent.K2_SetRelativeRotation` (`self.Hull`) (`KismetMathLibrary.MakeRotator` _returnvalue_roll_2 0.0 _returnvalue_yaw_2) false false))
    (:`Finished`
      (`KismetSystemLibrary.Delay` 1.0)
      (`self.K2_DestroyActor` self))))

(event `self.ReceiveTick`
  (params (DeltaSeconds :type "Float (single-precision)"))
  ;[1 1 1] We just check that the ship is alive and play the Lerp - We also take care here of all behaviours shared by all ships upon dying
  ;
  ; (Lerps must be connected to the Tick, otherwise it would only be called once)
  (`|ExecutionSequence`
    (:`then_0`
      (if (<= (`self.Health`) 0)
        (`/Engine/EditorBlueprintResources/StandardMacros.DoOnce` false
          (:`Completed`
            (bind _outactors (`GameplayStatics.GetAllActorsOfClass` "/Game/ThirdPersonBP/Blueprints/ThirdPersonCharacter.ThirdPersonCharacter_C"))
            (for _array_element _outactors
              (set `/Game/ThirdPersonBP/Blueprints/ThirdPersonCharacter.Coins` (+ (/ (`self.ShipGoldGain`) (`KismetArrayLibrary.Array_Length` _outactors)) (`/Game/ThirdPersonBP/Blueprints/ThirdPersonCharacter.Coins` _array_element)) _array_element))
            (`self.KillShip`)))))
    (:`then_1`
      (if (not (`self.followingSpline`))
        (`self.LerpToTarget` DeltaSeconds)))))

(event `KillShip`
  ;[1 1 1] Meant to be empty!
  ;
  ; Has a custom behavior written within each Child Actor
)

(event `ShipBehaviourTarget`
  ;[1 1 1] Meant to be empty!
  ;
  ; Has a custom behavior written within each Child Actor
)

(fn `UserConstructionScript`
  (switch `string` (`self.ShipType`)
    (:`Civil`
      (set `self.Health` 1)
      (set `self.ShipGoldGain` 12)
      (set `self.followingSpline` true))
    (:`Merchant`
      (set `self.Health` 2)
      (set `self.ShipGoldGain` 24)
      (set `self.followingSpline` true))
    (:`War`
      (set `self.Health` 2)
      (set `self.ShipGoldGain` 18)
      (set `self.followingSpline` false))
    (:`Ghost`
      (set `self.Health` 4)
      (set `self.ShipGoldGain` 48)
      (set `self.followingSpline` false))))