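; BP_ShipSpawner is an actor that keeps spawning civil, merchant and war ships at random over time.
; Tick feeds a DoOnce that waits DelaySpawn, rolls a random integer against the spawn thresholds to choose the ship class, then resets after spawning.
; Civil and merchant ships spawn using random ShipSplineArray entries and receive a spline to follow.
; War ships, the fallback, spawn at random SPAWNShipTPArray transforms and receive a random ShipTPArray stop target.
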(event `self.ReceiveTick`
  (params (DeltaSeconds :type "Float (single-precision)"))
  (bind _ship_tp_array (`self.Ship_TP_Array`))
  (bind _spawn_ship_tp_array (`self.SPAWN_Ship_TP_Array`))
  (bind _output (`|GetArrayItem` _spawn_ship_tp_array (`KismetMathLibrary.RandomIntegerInRange` 0 (- (`KismetArrayLibrary.Array_Length` _spawn_ship_tp_array) 1))))
  (bind _output_2 (`|GetArrayItem` (`self.Ship_Spline_Array`) (`KismetMathLibrary.RandomIntegerInRange` 0 (- (`KismetArrayLibrary.Array_Length` (`self.Ship_Spline_Array`)) 1))))
  (bind _returnvalue (`SceneComponent.K2_GetComponentLocation` (`/Game/EveryoneProg/Ships/SplineManager.DefaultSceneRoot` _output_2)))
  (`/Engine/EditorBlueprintResources/StandardMacros.DoOnce` false :!label _label
    (:`Completed`
      (`KismetSystemLibrary.Delay` (`self.delaySpawn`))
      (bind _output_get (set `self.LOC_Int_Rdm` (`KismetMathLibrary.RandomIntegerInRange` 0 10)))
      (if (< _output_get (`self.SpawnCivil`))
        (`|SpawnActorFromClass` "/Game/EveryoneProg/Ships/BP_Ship_Civil.BP_Ship_Civil_C" (`KismetMathLibrary.MakeTransform` _returnvalue) "Undefined" "OverrideRootScale" null _output_2 null 0.15 null)
        (goto _label :!via `Reset`)
        (elif (and (<= (`self.LOC_Int_Rdm`) (`self.SpawnMerchant`)) (< (`self.LOC_Int_Rdm`) (`self.SpawnWar`)))
          (`|SpawnActorFromClass` "/Game/EveryoneProg/Ships/BP_Ship_Merchant.BP_Ship_Merchant_C" (`KismetMathLibrary.MakeTransform` _returnvalue) "Undefined" "OverrideRootScale" null _output_2 null 0.15 null)
          (goto _label :!via `Reset`)
          (elif true
            (`|SpawnActorFromClass` "/Game/EveryoneProg/Ships/BP_Ship_War.BP_Ship_War_C" (`KismetMathLibrary.MakeTransform` (`self.K2_GetActorLocation` _output) (`self.K2_GetActorRotation` _output)) "Undefined" "OverrideRootScale" null null (`|GetArrayItem` _ship_tp_array (`KismetMathLibrary.RandomIntegerInRange` 0 (- (`KismetArrayLibrary.Array_Length` _ship_tp_array) 1))) 0.15 null)
            (goto _label :!via `Reset`)))))))

(fn `UserConstructionScript`)