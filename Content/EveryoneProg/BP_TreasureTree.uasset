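; Treasure tree actor that grows random treasures and releases them when hit.
; Tick waits for a timer while empty, then spawns three random picks from ObjectsToSpawn at top, middle and bottom points.
; GotHit calls FreeTreasures only when treasures are present and 2Players is false.
; FreeTreasures briefly disables collision on three boxes to release the treasures, then clears ObjectsSpawned so Tick refills the tree.
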(event `self.ReceiveTick`
  (params (DeltaSeconds :type "Float (single-precision)"))
  (bind _objectstospawn (`self.ObjectsToSpawn`))
  (bind _objectstospawn_2 (`self.ObjectsToSpawn`))
  (bind _objectstospawn_3 (`self.ObjectsToSpawn`))
  ;[1 1 1] ça fait peur, mais c'est facile !
  ;
  ; On réplique trois fois un Spawn Actor pour setter correctement les objets, et pouvoir les faire bouger avec les Timelines, tout simplement.
  (if (not (`self.ObjectsSpawned`))
    (`/Engine/EditorBlueprintResources/StandardMacros.DoOnce` false :!label _label
      (:`Completed`
        (`KismetSystemLibrary.Delay` (`self.TimerSpawn`))
        (`|ExecutionSequence`
          (:`then_0`
            (`|SpawnActorFromClass` (`|GetArrayItem` _objectstospawn (`KismetMathLibrary.RandomIntegerInRange` 0 (- (`KismetArrayLibrary.Array_Length` _objectstospawn) 1))) (`KismetMathLibrary.MakeTransform` (`SceneComponent.K2_GetComponentLocation` (`self.SpawnTreasureTop`)) (struct) (1.05 1.05 1.05)) "AdjustIfPossibleButAlwaysSpawn" "OverrideRootScale" null null))
          (:`then_1`
            (`|SpawnActorFromClass` (`|GetArrayItem` _objectstospawn_2 (`KismetMathLibrary.RandomIntegerInRange` 0 (- (`KismetArrayLibrary.Array_Length` _objectstospawn_2) 1))) (`KismetMathLibrary.MakeTransform` (`SceneComponent.K2_GetComponentLocation` (`self.SpawnTreasureMid`)) (struct) (1.05 1.05 1.05)) "AdjustIfPossibleButAlwaysSpawn" "OverrideRootScale" null null))
          (:`then_2`
            (`|SpawnActorFromClass` (`|GetArrayItem` _objectstospawn_3 (`KismetMathLibrary.RandomIntegerInRange` 0 (- (`KismetArrayLibrary.Array_Length` _objectstospawn_3) 1))) (`KismetMathLibrary.MakeTransform` (`SceneComponent.K2_GetComponentLocation` (`self.SpawnTreasureBot`)) (struct) (1.05 1.05 1.05)) "AdjustIfPossibleButAlwaysSpawn" "OverrideRootScale" null null)))
        (set `self.ObjectsSpawned` true)
        (goto _label :!via `Reset`)))))

(event `/Game/EveryoneProg/BPI_Interact.GotHit`
  (params (PlayerHitting :type "/Game/ThirdPersonBP/Blueprints/ThirdPersonCharacter Object Reference"))
  ;[1 1 1] ça marche pas encore, dur dur de faire bouger des objets hors de leur propre Blueprint!
  (if (`self.ObjectsSpawned`)
    (if (not (`self.2Players?`))
      (`self.FreeTreasures`))))

(event `FreeTreasures`
  ;[1 1 1] ça marche pas encore, dur dur de faire bouger des objets hors de leur propre Blueprint!
  (`/Engine/EditorBlueprintResources/StandardMacros.DoOnce` false :!label _label_2
    (:`Completed`
      (`PrimitiveComponent.SetCollisionEnabled` (`self.Box1`) "NoCollision")
      (`PrimitiveComponent.SetCollisionEnabled` (`self.Box2`) "NoCollision")
      (`PrimitiveComponent.SetCollisionEnabled` (`self.Box`) "NoCollision")
      (`KismetSystemLibrary.Delay` 1.0)
      (`PrimitiveComponent.SetCollisionEnabled` (`self.Box1`) "QueryAndPhysics")
      (`PrimitiveComponent.SetCollisionEnabled` (`self.Box2`) "QueryAndPhysics")
      (`PrimitiveComponent.SetCollisionEnabled` (`self.Box`) "QueryAndPhysics")
      (set `self.ObjectsSpawned` false)
      (goto _label_2 :!via `Reset`))))

(fn `UserConstructionScript`)