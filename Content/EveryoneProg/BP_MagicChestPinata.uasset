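; Magic chest piñata that periodically opens for players to hit for coins, ending in a coin rain.
; Tick counts seconds toward readiness and toggles lid, gold pile and light through paired DoOnce gates.
; Each hit awards coins with a score popup; the first starts a timer that spawns coins by hit count, then resets the chest.
; CountGold separately totals a quarter of the gold it receives.
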(event `VisChest`
  (bind _rectlight (`self.RectLight`))
  (bind _goldpile (`self.GoldPile`))
  (bind _lid (`self.Lid`))
  ;[1 1 1] VisChest: Only handles how the Magic Chest looks, in order to let players know if they can interact with the item.
  (if (`self.CanPinata`)
    (`/Engine/EditorBlueprintResources/StandardMacros.DoOnce` false :!label _label
      (:`Completed`
        (`LightComponent.SetIntensity` _rectlight 9000.0)
        (`SceneComponent.SetHiddenInGame` _goldpile false false)
        (`SceneComponent.K2_SetRelativeRotation` _lid (struct :`Roll` -65.0) false false)
        (goto _label_2 :!via `Reset`)))
    (else
      (`/Engine/EditorBlueprintResources/StandardMacros.DoOnce` false :!label _label_2
        (:`Completed`
          (`LightComponent.SetIntensity` _rectlight 500.0)
          (`SceneComponent.SetHiddenInGame` _goldpile true false)
          (`SceneComponent.K2_SetRelativeRotation` _lid (struct :`Roll` -10.0) false false)
          (goto _label :!via `Reset`))))))

(event `self.ReceiveTick`
  (params (DeltaSeconds :type "Float (single-precision)"))
  (`|ExecutionSequence`
    (:`then_0`
      (`/Engine/EditorBlueprintResources/StandardMacros.DoOnce` false :!label _label_3
        (:`Completed`
          (`KismetSystemLibrary.Delay` 1.0)
          (`/Engine/EditorBlueprintResources/StandardMacros.IncrementInt` (`self.TimeSinceCoinRain`)
            (:`  `
              (goto _label_3 :!via `Reset`))))))
    (:`then_1`
      (`self.VisChest`))
    (:`then_2`
      (if (>= (`self.TimeSinceCoinRain`) (`self.TimeForCoinRain`))
        (set `self.CanPinata` true)
        (else
          (set `self.CanPinata` false))))))

(event `/Game/EveryoneProg/BPI_Interact.CountGold`
  (params (Gold :type Integer))
  (bind _output_get (set `self.GoldCollected` (+ (`self.GoldCollected`) (/ Gold 4))))
  (`KismetSystemLibrary.PrintString` (`KismetStringLibrary.Concat_StrStr` "Total gold is: " (`KismetStringLibrary.Conv_IntToString` _output_get))))

(event `TimerPinata`
  (`KismetSystemLibrary.Delay` (`KismetMathLibrary.Conv_IntToDouble` (`self.TimeForPinata`)))
  (`/Game/EveryoneProg/Managers/MACROS_Spawners.Spawner In Radius` (`self.timesHit`) (`self.TargetPoint`) (400.0 400.0 50.0) "/Game/EveryoneProg/Coin.Coin_C"
    (:`Completed`
      (`GameplayStatics.PlaySound2D` "/Game/ArtAndMusic/Music/Bruitages/Coffre_-_Fin_Event.Coffre_-_Fin_Event" 0.5 1.0 0.0 null null)
      (set `self.TimeSinceCoinRain` 0)
      (set `self.timesHit` 0)
      (set `self.CanPinata` false)
      (`LightComponent.SetIntensity` (`self.SpotLight`) 0.0))))

(event `/Game/EveryoneProg/BPI_Interact.GotHit`
  (params (PlayerHitting :type "/Game/ThirdPersonBP/Blueprints/ThirdPersonCharacter Object Reference"))
  (if (`self.CanPinata`)
    (`|ExecutionSequence`
      (:`then_0`
        (`GameplayStatics.PlaySound2D` "/Game/ArtAndMusic/Music/Bruitages/HeadLaunch.HeadLaunch" 1.0 1.0 0.0 null null)
        (set `/Game/ThirdPersonBP/Blueprints/ThirdPersonCharacter.Coins` (+ (`/Game/ThirdPersonBP/Blueprints/ThirdPersonCharacter.Coins` PlayerHitting) 4) PlayerHitting)
        (bind _aswbp_player_score_increase (cast `/Game/ThirdPersonBP/Blueprints/UI/WBP_PlayerScoreIncrease` (`WidgetComponent.GetUserWidgetObject` (`/Game/ThirdPersonBP/Blueprints/ThirdPersonCharacter.ScoreIncrease` PlayerHitting))))
        (set `/Game/ThirdPersonBP/Blueprints/UI/WBP_PlayerScoreIncrease.ScoreInt` 4 _aswbp_player_score_increase)
        (`/Game/ThirdPersonBP/Blueprints/UI/WBP_PlayerScoreIncrease.PlayAnimIncrease` _aswbp_player_score_increase)
        (`KismetSystemLibrary.Delay` 0.05)
        (`/Engine/EditorBlueprintResources/StandardMacros.IncrementInt` (`self.timesHit`)))
      (:`then_1`
        (if (<= (`self.timesHit`) 0)
          (`self.TimerPinata`)
          (`LightComponent.SetIntensity` (`self.SpotLight`) 15000.0))))))

(fn `UserConstructionScript`)