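; BP_CoinSpawner is a manager actor that repeatedly spawns batches of coins inside a box-shaped area around itself.
; Tick feeds a DoOnce gate that waits WaitSpawn, rolls a count between the min and max, spawns double-scale coins at random points with short delays between them, then resets.
; The construction script sizes VisBox to BoxSize to show the spawn area.
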(event `self.ReceiveTick`
  (params (DeltaSeconds :type "Float (single-precision)"))
  (`/Engine/EditorBlueprintResources/StandardMacros.DoOnce` false :!label _label
    (:`Completed`
      (`KismetSystemLibrary.Delay` (`self.WaitSpawn`))
      (bind _output_get (set `self.CountSpawn` (`KismetMathLibrary.RandomIntegerInRange` (`self.MinCoinSpawn`) (`self.MaxCoinSpawn`))))
      (for _ (range 1 (+ _output_get 1))
        (`|SpawnActorFromClass` "/Game/EveryoneProg/Coin.Coin_C" (`KismetMathLibrary.MakeTransform` (`KismetMathLibrary.RandomPointInBoundingBox` (`self.K2_GetActorLocation` self) (`self.BoxSize`)) (struct) (2.0 2.0 2.0)) "Undefined" "OverrideRootScale" null null)
        (`KismetSystemLibrary.Delay` 0.3))
      (goto _label :!via `Reset`))))

(fn `UserConstructionScript`
  (`BoxComponent.SetBoxExtent` (`self.VisBox`) (`self.BoxSize`) true))