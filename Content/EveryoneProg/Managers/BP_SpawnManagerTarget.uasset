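; BP_SpawnManagerTarget is a spawn target marker that tracks whether a sellable actor occupies it.
; On BeginPlay it replaces its tags with TagFoodToSpawn, labelling which food the spot is for.
; An overlap with a "Sell"-tagged actor stores it as Filler and sets Filled.
; Tick polls whether the Sphere still overlaps Filler, otherwise resetting it to FillerNone and clearing Filled.
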(event `self.ReceiveBeginPlay`
  (set `self.Tags` (`|MakeArray` (`self.TagFoodToSpawn`))))

(event `self.ReceiveTick`
  (params (DeltaSeconds :type "Float (single-precision)"))
  (if (`PrimitiveComponent.IsOverlappingActor` (`self.Sphere`) (`self.Filler`))
    (set `self.Filled` true)
    (else
      (set `self.Filler` (`self.FillerNone`))
      (set `self.Filled` false))))

(event `self.ReceiveActorBeginOverlap`
  (params (OtherActor :type "Actor Object Reference"))
  (if (`self.ActorHasTag` OtherActor "Sell")
    (set `self.Filler` OtherActor)
    (set `self.Filled` true)))

(fn `UserConstructionScript`)