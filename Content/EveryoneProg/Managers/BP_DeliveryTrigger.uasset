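; Delivery point for the cursed chalice that lights nearby torches while active and removes itself when the chalice arrives.
; On BeginPlay it loops its actor sequence and sphere-traces around its box to unhide the light and flame of each Dynamic_LitTorch found.
; When BP_WS_CursedChalice2P overlaps its chalice mesh, it repeats the trace to hide those torch effects and destroys itself after a short delay.
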(event `self.ReceiveBeginPlay`
  (bind _returnvalue (`SceneComponent.K2_GetComponentLocation` (`self.Box`)))
  (`MovieSceneSequencePlayer.PlayLooping` (`ActorSequenceComponent.SequencePlayer` (`self.ActorSequence`)) -1)
  (bind _outhits (`KismetSystemLibrary.SphereTraceMultiForObjects` _returnvalue (+ _returnvalue 1.0) 600.0 (`|MakeArray` "ObjectTypeQuery1" :!type "EObjectTypeQuery Enum")))
  (for _array_element _outhits
    (bind (_bblockinghit _binitialoverlap _time _distance _location _impactpoint _normal _impactnormal _physmat _hitactor) (`GameplayStatics.BreakHitResult` _array_element))
    (if (== (`GameplayStatics.GetObjectClass` _hitactor) "/Game/EveryoneProg/Art/Dynamic_LitTorch.Dynamic_LitTorch_C")
      (bind _asdynamic_lit_torch (cast `/Game/EveryoneProg/Art/Dynamic_LitTorch` _hitactor))
      (`SceneComponent.SetHiddenInGame` (`/Game/EveryoneProg/Art/Dynamic_LitTorch.PointLight` _asdynamic_lit_torch) false false)
      (`SceneComponent.SetHiddenInGame` (`/Game/EveryoneProg/Art/Dynamic_LitTorch.Flames (Tiny)` _asdynamic_lit_torch) false false))))

(event `self.SM_Item_Chalice_02.OnComponentBeginOverlap`
  (params (OverlappedComponent :type "PrimitiveComponent Object Reference") (OtherActor :type "Actor Object Reference") (OtherComp :type "PrimitiveComponent Object Reference") (OtherBodyIndex :type Integer) (bFromSweep :type Boolean) (SweepResult :type "HitResult Structure (by ref)"))
  (bind _returnvalue (`SceneComponent.K2_GetComponentLocation` (`self.Box`)))
  (if (== (`GameplayStatics.GetObjectClass` OtherActor) "/Game/EveryoneProg/Deliveries/BP_WS_CursedChalice2P.BP_WS_CursedChalice2P_C")
    (`|ExecutionSequence`
      (:`then_0`
        (`KismetSystemLibrary.Delay` 0.2)
        (`self.K2_DestroyActor`))
      (:`then_1`
        (bind _outhits (`KismetSystemLibrary.SphereTraceMultiForObjects` _returnvalue (+ _returnvalue 1.0) 600.0 (`|MakeArray` "ObjectTypeQuery1" :!type "EObjectTypeQuery Enum")))
        (for _array_element _outhits
          (bind (_bblockinghit _binitialoverlap _time _distance _location _impactpoint _normal _impactnormal _physmat _hitactor) (`GameplayStatics.BreakHitResult` _array_element))
          (if (== (`GameplayStatics.GetObjectClass` _hitactor) "/Game/EveryoneProg/Art/Dynamic_LitTorch.Dynamic_LitTorch_C")
            (bind _asdynamic_lit_torch (cast `/Game/EveryoneProg/Art/Dynamic_LitTorch` _hitactor))
            (`SceneComponent.SetHiddenInGame` (`/Game/EveryoneProg/Art/Dynamic_LitTorch.PointLight` _asdynamic_lit_torch) true false)
            (`SceneComponent.SetHiddenInGame` (`/Game/EveryoneProg/Art/Dynamic_LitTorch.Flames (Tiny)` _asdynamic_lit_torch) true false)))))))

(fn `UserConstructionScript`)