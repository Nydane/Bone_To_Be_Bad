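; BP_GoldBagSpawner keeps the level supplied with gold bags, spawning them at random points inside a box.
; A DoOnce-gated Tick loop waits, counts bags without LvStart set, and spawns if below the cap, otherwise waits before retrying.
; Spawns are preceded by a brief particle effect, and SpawnBag triggers one directly, bypassing the count.
; The construction script sizes the visualization box to the spawn area.
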(event `self.ReceiveTick`
  (params (DeltaSeconds :type "Float (single-precision)"))
  (`/Engine/EditorBlueprintResources/StandardMacros.DoOnce` false :!label _label
    (:`Completed`
      (`KismetSystemLibrary.Delay` (`self.WaitSpawn`))
      (bind _outactors (`GameplayStatics.GetAllActorsOfClass` "/Game/EveryoneProg/Deliveries/BP_GoldBag_WithGrab.BP_GoldBag_WithGrab_C"))
      (for _array_element _outactors
        (if (not (`/Game/EveryoneProg/Deliveries/BP_GoldBag_WithGrab.LvStart` _array_element))
          (`KismetArrayLibrary.Array_AddUnique` (`self.BagsAllowed`) _array_element)))
      (if (< (`KismetArrayLibrary.Array_Length` (`self.BagsAllowed`)) (`self.MaxBagAllowed`))
        (`KismetArrayLibrary.Array_Clear` (`self.BagsAllowed`))
        (bind _returnvalue (`GameplayStatics.SpawnEmitterAtLocation` "/Game/VFXapprentice/Spawner/spawner2/VFX_Spawner2.VFX_Spawner2" (`KismetMathLibrary.RandomPointInBoundingBox` (`self.K2_GetActorLocation` self) (`self.SpawnSize`)) :!label _label_2))
        (`KismetSystemLibrary.Delay` 0.3)
        (`|SpawnActorFromClass` "/Game/EveryoneProg/Deliveries/BP_GoldBag_WithGrab.BP_GoldBag_WithGrab_C" (`KismetMathLibrary.MakeTransform` (`SceneComponent.K2_GetComponentLocation` _returnvalue) (struct) (1.2 1.2 1.2)) "Undefined" "OverrideRootScale" null 4 0 false null)
        (`KismetSystemLibrary.Delay` 0.2)
        (`ActorComponent.Deactivate` _returnvalue)
        (goto _label :!via `Reset`)
        (else
          (`KismetArrayLibrary.Array_Clear` (`self.BagsAllowed`))
          (`KismetSystemLibrary.Delay` (`self.FailWaitSpawn`))
          (goto _label :!via `Reset`))))))

(event `SpawnBag`
  (goto _label_2))

(fn `UserConstructionScript`
  (`BoxComponent.SetBoxExtent` (`self.VisSpawn`) (`self.SpawnSize`) true))