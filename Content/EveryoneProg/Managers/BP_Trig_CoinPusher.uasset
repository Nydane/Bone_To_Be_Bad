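; BP_Trig_CoinPusher is a trigger volume that pulls overlapping Coin actors toward a target point.
; The construction script sizes the Pusher box from BoxSize, and BeginPlay caches the Billboard's world location as the destination.
; Each Tick eases every overlapping coin toward that point with VInterpTo, setting its location without sweep or teleport.
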(event `self.ReceiveBeginPlay`
  (set `self.EndLocationVector` (`SceneComponent.K2_GetComponentLocation` (`self.Billboard`))))

(event `self.Pusher.OnComponentBeginOverlap`
  (params (OverlappedComponent :type "PrimitiveComponent Object Reference") (OtherActor :type "Actor Object Reference") (OtherComp :type "PrimitiveComponent Object Reference") (OtherBodyIndex :type Integer) (bFromSweep :type Boolean) (SweepResult :type "HitResult Structure (by ref)")))

(event `self.ReceiveTick`
  (params (DeltaSeconds :type "Float (single-precision)"))
  (for _array_element (`self.GetOverlappingActors` "/Game/EveryoneProg/Coin.Coin_C")
    (`self.K2_SetActorLocation` _array_element (`KismetMathLibrary.VInterpTo` (`self.K2_GetActorLocation` _array_element) (`self.EndLocationVector`) DeltaSeconds 0.9) false false)))

(fn `UserConstructionScript`
  (`BoxComponent.SetBoxExtent` (`self.Pusher`) (`self.BoxSize`) true))