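; Rake trap that swings when a living player steps on its trigger, knocking them into the Headless state and launching them.
; An overlap starts a Timeline that lerps the Base rotation, gated by a DoOnce that resets shortly after the swing.
; The kill trigger records the victim, and Tick applies the hit if they still overlap at the end pitch.
; A second DoOnce with a delay prevents launching every frame.
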(event `self.Activ_Trigger.OnComponentBeginOverlap`
  (params (OverlappedComponent :type "PrimitiveComponent Object Reference") (OtherActor :type "Actor Object Reference") (OtherComp :type "PrimitiveComponent Object Reference") (OtherBodyIndex :type Integer) (bFromSweep :type Boolean) (SweepResult :type "HitResult Structure (by ref)"))
  ;[1 1 1] This is the part of the script that will make our Rake strike a Player.
  ;;[1 1 1] Is there a Player Character within the Trigger?
  (`/Engine/EditorBlueprintResources/StandardMacros.DoOnce` false :!label _label
    (:`Completed`
      (if (== (`GameplayStatics.GetObjectClass` OtherActor) "/Game/ThirdPersonBP/Blueprints/ThirdPersonCharacter.ThirdPersonCharacter_C")
        ;;[1 1 1] What's this Player's Current State? If they're not Dead, we can move on.
        (bind _asthird_person_character (cast `/Game/ThirdPersonBP/Blueprints/ThirdPersonCharacter` OtherActor))
        (if (`|EnumEquality` (`/Game/ThirdPersonBP/Blueprints/ThirdPersonCharacter.CurrentState` _asthird_person_character) "NewEnumerator0")
          ;;[1 1 1] Create a Timeline which will rotate what we need.
          (bind (_direction _newtrack_0) (`Timeline|RotateRake` :!via `PlayFromStart`)
            (:`Update`
              (`SceneComponent.K2_SetRelativeRotation` (`self.Base`) (`KismetMathLibrary.RLerp` (`self.StartRotation`) (`self.EndRotation`) _newtrack_0) false false))
            (:`Finished`
              ;;[1 1 1] Stops the Timeline from restarting before reaching the end of its loop.
              (`KismetSystemLibrary.Delay` 0.2)
              (goto _label :!via `Reset`)))
          (else
            (goto _label :!via `Reset`)))
        (else
          (goto _label :!via `Reset`))))))

(event `self.Kill_Trigger.OnComponentBeginOverlap`
  (params (OverlappedComponent :type "PrimitiveComponent Object Reference") (OtherActor :type "Actor Object Reference") (OtherComp :type "PrimitiveComponent Object Reference") (OtherBodyIndex :type Integer) (bFromSweep :type Boolean) (SweepResult :type "HitResult Structure (by ref)"))
  ;[1 1 1] Have we hit a Player with the actual Kill Trigger? If so, we set this player as the object within the variable "Player Hit", to make sure that they're the victim.
  (if (== (`GameplayStatics.GetObjectClass` OtherActor) "/Game/ThirdPersonBP/Blueprints/ThirdPersonCharacter.ThirdPersonCharacter_C")
    (set `self.PlayerHit` OtherActor)))

(event `self.ReceiveTick`
  (params (DeltaSeconds :type "Float (single-precision)"))
  (bind (_endrotation_roll _endrotation_pitch) (`KismetMathLibrary.BreakRotator` (`self.EndRotation`)))
  (bind (_relativerotation_roll _relativerotation_pitch) (`KismetMathLibrary.BreakRotator` (`SceneComponent.RelativeRotation` (`self.Base`))))
  ;[1 1 1] Checks the rotation of our trap and if the player is still overlapping "Kill Trigger".
  (if (and (`PrimitiveComponent.IsOverlappingActor` (`self.Kill_Trigger`) (`self.PlayerHit`)) (== _relativerotation_pitch _endrotation_pitch))
    ;[1 1 1] If it's true, then we can rake the snot out of our poor fella! Also, gets them to the Headless State.
    (bind _asthird_person_character (cast `/Game/ThirdPersonBP/Blueprints/ThirdPersonCharacter` (`self.PlayerHit`)))
    (`/Engine/EditorBlueprintResources/StandardMacros.DoOnce` false :!label _label_2
      (:`Completed`
        ;;[1 1 1] We set the victim's State to "Headless" and call "Check State"
        (set `/Game/ThirdPersonBP/Blueprints/ThirdPersonCharacter.CurrentState` "NewEnumerator1" _asthird_person_character)
        (`/Game/ThirdPersonBP/Blueprints/ThirdPersonCharacter.Check State` _asthird_person_character)
        (bind (_returnvalue_x _returnvalue_y) (`self.LaunchDirection` _asthird_person_character))
        (`Character.LaunchCharacter` _asthird_person_character (`KismetMathLibrary.MakeVector` _returnvalue_x _returnvalue_y 100.0) false false)
        ;[1 1 1] Here, the Delay makes sure that we can't Launch a Character at each frame drawn.
        (`KismetSystemLibrary.Delay` 1.0)
        (goto _label_2 :!via `Reset`)))))

(fn `UserConstructionScript`)