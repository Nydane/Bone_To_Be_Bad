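; Dynamic torch actor that can be lit and extinguished through its LightUp and LightOff events.
; LightUp activates the fire and smoke particles and raises the candle and environment lights to fixed intensities, while LightOff deactivates the particles and zeroes both lights.
; The AllowExtEvents flag gates both events, including the LightOff call at BeginPlay, so the torch starts unlit only when that flag is set.
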(event `self.ReceiveBeginPlay`
  (`self.LightOff`))

(event `LightUp`
  (if (`self.AllowExtEvents`)
    (`ActorComponent.Activate` (`self.FirePart`) false)
    (`ActorComponent.Activate` (`self.SmokePart`) false)
    (`LightComponent.SetIntensity` (`self.CandleLight`) 84.0)
    (`LightComponent.SetIntensity` (`self.EnviLight`) 24.0)))

(event `LightOff`
  (if (`self.AllowExtEvents`)
    (`ActorComponent.Deactivate` (`self.FirePart`))
    (`ActorComponent.Deactivate` (`self.SmokePart`))
    (`LightComponent.SetIntensity` (`self.CandleLight`) 0.0)
    (`LightComponent.SetIntensity` (`self.EnviLight`) 0.0)))

(fn `UserConstructionScript`)