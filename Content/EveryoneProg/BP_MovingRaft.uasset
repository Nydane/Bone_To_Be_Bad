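; BP_MovingRaft is a raft that travels once along the spline of its SplineManager and drops coins around the midpoint.
; If CanMove is set at BeginPlay, a Timeline scaled by Duration drives location and rotation along the spline.
; Tick watches for Alpha near 0.5, then spawns a short-lived BP_CoinSpawner at the Scene component with NumberCoinsToSpawn.
; A DoOnce with delayed reset throttles repeat spawns.
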(event `self.ReceiveBeginPlay`
  (if (`self.CanMove`)
    (`self.MoveRaft`)))

(event `MoveRaft`
  (bind _returnvalue (`KismetMathLibrary.Lerp` 0.0 (`SplineComponent.GetSplineLength` (`/Game/EveryoneProg/Ships/SplineManager.Spline` (`self.SplineManager`))) (`self.Alpha`)))
  ;[1 1 1] Gère seulement le mouvement du Raft, il faudra ajouter d'autres CE ou passer par l'Event Tick pour les autres Behaviours.
  (`TimelineComponent.SetPlayRate` (`self.Movement`) (/ 1.0 (`self.Duration`)))
  (bind (_direction _alpha) (`Timeline|Movement`)
    (:`Update`
      (set `self.Alpha` _alpha)
      (`self.K2_SetActorLocationAndRotation` (`SplineComponent.GetLocationAtDistanceAlongSpline` (`/Game/EveryoneProg/Ships/SplineManager.Spline` (`self.SplineManager`)) _returnvalue "World") (`SplineComponent.GetRotationAtDistanceAlongSpline` (`/Game/EveryoneProg/Ships/SplineManager.Spline` (`self.SplineManager`)) _returnvalue "World")))
    (:`Finished`
      (set `self.CanMove` false))))

(event `self.ReceiveTick`
  (params (DeltaSeconds :type "Float (single-precision)"))
  (bind _numbercoinstospawn (`self.NumberCoinsToSpawn`))
  (`|ExecutionSequence`
    (:`then_0`
      (if (`KismetMathLibrary.NearlyEqual_FloatFloat` (`self.Alpha`) 0.5 0.05)
        (`/Engine/EditorBlueprintResources/StandardMacros.DoOnce` false :!label _label
          (:`Completed`
            (bind _returnvalue (`|SpawnActorFromClass` "/Game/EveryoneProg/Managers/BP_CoinSpawner.BP_CoinSpawner_C" (`KismetMathLibrary.MakeTransform` (`SceneComponent.K2_GetComponentLocation` (`self.Scene`))) "Undefined" "OverrideRootScale" null (100.0 100.0 25.0) 0.05 _numbercoinstospawn _numbercoinstospawn null))
            (`KismetSystemLibrary.Delay` 0.06)
            (`self.K2_DestroyActor` _returnvalue)
            (`KismetSystemLibrary.Delay` 1.0)
            (goto _label :!via `Reset`)))))))

(fn `UserConstructionScript`)