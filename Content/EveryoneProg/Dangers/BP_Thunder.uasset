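; BP_Thunder is a lightning hazard that telegraphs a strike, hits an area once, then destroys itself.
; A Duration-scaled timeline ramps the point light during preparation particles; Tick fires the strike once its Alpha nears 1.6.
; The strike triggers effects, random thunder audio and camera shake, then sphere-traces StrikeRadius to change ThirdPersonCharacter state and zero RedBarrel health.
; The construction script sizes the light to StrikeRadius.
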(event `self.ReceiveBeginPlay`
  (`ActorComponent.Activate` (`self.ThunderPrepare`) true)
  (`self.VisPrepareStrike`)
  (`AudioComponent.SetSound` (`self.Audio`) (`KismetArrayLibrary.Array_Random` (`self.SoundArray`))))

(event `VisPrepareStrike`
  (`TimelineComponent.SetPlayRate` (`self.LightIntensity`) (/ 1.0 (`self.Duration`)))
  (bind (_direction _alpha) (`Timeline|LightIntensity` :!via `PlayFromStart`)
    (:`Update`
      (set `self.Alpha` _alpha)
      (`LightComponent.SetIntensity` (`self.PointLight`) (`KismetMathLibrary.Lerp` 0.0 (`self.LightIntensityLerp`) (`self.Alpha`))))))

(event `self.ReceiveTick`
  (params (DeltaSeconds :type "Float (single-precision)"))
  (if (`KismetMathLibrary.NearlyEqual_FloatFloat` (`self.Alpha`) 1.6 0.1)
    (`/Engine/EditorBlueprintResources/StandardMacros.DoOnce` false
      (:`Completed`
        (`self.LightningStrike`)))))

(event `LightningStrike`
  (bind _returnvalue (`SceneComponent.K2_GetComponentLocation` (`self.ThunderOrigin`)))
  (`|ExecutionSequence`
    (:`then_0`
      (`ActorComponent.Activate` (`self.Dust`) false)
      (`ActorComponent.Activate` (`self.ThunderStrike`) false)
      (`ActorComponent.Activate` (`self.Impact`) false)
      (`GameplayStatics.PlayWorldCameraShake` "/Game/EveryoneProg/BP_ScreenShakeThunder.BP_ScreenShakeThunder_C" (0.0 0.0 0.0) 5000.0 10000.0)
      (`AudioComponent.Play` (`self.Audio`) 0.0)
      (`LightComponent.SetIntensity` (`self.PointLight`) 0.0))
    (:`then_1`
      (bind _outhits (`KismetSystemLibrary.SphereTraceMultiForObjects` _returnvalue (+ _returnvalue (0.5 0.5 0.5)) (`self.StrikeRadius`) (`|MakeArray` "ObjectTypeQuery3" "ObjectTypeQuery4" :!type "EObjectTypeQuery Enum")))
      (for _array_element _outhits
        (bind (_bblockinghit _binitialoverlap _time _distance _location _impactpoint _normal _impactnormal _physmat _hitactor) (`GameplayStatics.BreakHitResult` _array_element))
        (bind _returnvalue_2 (`GameplayStatics.GetObjectClass` _hitactor))
        (if (== _returnvalue_2 "/Game/ThirdPersonBP/Blueprints/ThirdPersonCharacter.ThirdPersonCharacter_C")
          (bind _asthird_person_character (cast `/Game/ThirdPersonBP/Blueprints/ThirdPersonCharacter` _hitactor))
          (if (`|EnumInequality` (`/Game/ThirdPersonBP/Blueprints/ThirdPersonCharacter.CurrentState` _asthird_person_character) "NewEnumerator1")
            (set `/Game/ThirdPersonBP/Blueprints/ThirdPersonCharacter.CurrentState` (`self.PlayerStateOnHit`) _asthird_person_character)
            (`/Game/ThirdPersonBP/Blueprints/ThirdPersonCharacter.Check State` _asthird_person_character))
          (elif (== _returnvalue_2 "/Game/EveryoneProg/Dangers/RedBarrel.RedBarrel_C")
            (bind _asred_barrel (cast `/Game/EveryoneProg/Dangers/RedBarrel` _hitactor))
            (set `/Game/EveryoneProg/Dangers/RedBarrel.Health` 0 _asred_barrel)
            (`/Game/EveryoneProg/Dangers/RedBarrel.CheckHealth` _asred_barrel))))
      (`KismetSystemLibrary.Delay` 1.0)
      (`ActorComponent.Deactivate` (`self.Impact`))
      (`ActorComponent.Deactivate` (`self.ThunderStrike`))
      (`ActorComponent.Deactivate` (`self.Dust`))
      (`ActorComponent.Deactivate` (`self.ThunderPrepare`))
      (`KismetSystemLibrary.Delay` 10.0)
      (`self.K2_DestroyActor`))))

(fn `UserConstructionScript`
  (bind _pointlight (`self.PointLight`))
  (bind _strikeradius (`self.StrikeRadius`))
  (`LocalLightComponent.SetAttenuationRadius` _pointlight _strikeradius)
  (`PointLightComponent.SetSourceRadius` _pointlight _strikeradius))