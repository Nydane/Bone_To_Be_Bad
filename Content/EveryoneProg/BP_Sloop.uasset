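; BP_Sloop is a drop-off point that turns gold bags into coins for the player it is assigned to.
; When a BP_GoldBag_WithGrab actor enters its Trigger, it adds GoldBagGain to the ThirdPersonCharacter whose LocalID matches PlayerIndex and destroys the bag.
; It then counts the gold bags in the level and asks SpawnerBagRef to spawn another if the count is below MaxBagAllowed.
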(event `self.ReceiveBeginPlay`
  (set `self.AuthorizedGoldAug` "/Game/EveryoneProg/Deliveries/BP_GoldBag_WithGrab.BP_GoldBag_WithGrab_C"))

(event `self.Trigger.OnComponentBeginOverlap`
  (params (OverlappedComponent :type "PrimitiveComponent Object Reference") (OtherActor :type "Actor Object Reference") (OtherComp :type "PrimitiveComponent Object Reference") (OtherBodyIndex :type Integer) (bFromSweep :type Boolean) (SweepResult :type "HitResult Structure (by ref)"))
  (if (== (`GameplayStatics.GetObjectClass` OtherActor) (`self.AuthorizedGoldAug`))
    (bind _outactors (`GameplayStatics.GetAllActorsOfClass` "/Game/ThirdPersonBP/Blueprints/ThirdPersonCharacter.ThirdPersonCharacter_C"))
    (for _array_element _outactors
      (if (== (`/Game/ThirdPersonBP/Blueprints/ThirdPersonCharacter.LocalID` _array_element) (`self.PlayerIndex`))
        (set `/Game/ThirdPersonBP/Blueprints/ThirdPersonCharacter.Coins` (+ (`/Game/ThirdPersonBP/Blueprints/ThirdPersonCharacter.Coins` _array_element) (`self.GoldBagGain`)) _array_element)
        (`self.K2_DestroyActor` OtherActor)))
    (bind _outactors_2 (`GameplayStatics.GetAllActorsOfClass` (`self.AuthorizedGoldAug`)))
    (if (< (`KismetArrayLibrary.Array_Length` _outactors_2) (`/Game/EveryoneProg/Managers/BP_GoldBagSpawner.MaxBagAllowed` (`self.SpawnerBagRef`)))
      (`/Game/EveryoneProg/Managers/BP_GoldBagSpawner.SpawnBag` (`self.SpawnerBagRef`)))))

(fn `UserConstructionScript`)