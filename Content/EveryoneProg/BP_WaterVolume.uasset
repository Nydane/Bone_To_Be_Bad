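; Water volume that breaks any gold bag entering its box, scattering it as coins.
; On overlap, it clears the IsCarrying flag on the carrying ThirdPersonCharacter and detaches the bag's Carrier reference.
; After a short delay it spawns BagGoldToSpawn enlarged coins at random points above the bag's bucket mesh, then destroys the bag.
; A DoOnce gate blocks further bag overlaps until that destruction resets it.
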(event `self.Box.OnComponentBeginOverlap`
  (params (OverlappedComponent :type "PrimitiveComponent Object Reference") (OtherActor :type "Actor Object Reference") (OtherComp :type "PrimitiveComponent Object Reference") (OtherBodyIndex :type Integer) (bFromSweep :type Boolean) (SweepResult :type "HitResult Structure (by ref)"))
  (if (== (`GameplayStatics.GetObjectClass` OtherActor) "/Game/EveryoneProg/Deliveries/BP_GoldBag_WithGrab.BP_GoldBag_WithGrab_C")
    (`/Engine/EditorBlueprintResources/StandardMacros.DoOnce` false :!label _label
      (:`Completed`
        (bind _asbp_gold_bag_with_grab (cast `/Game/EveryoneProg/Deliveries/BP_GoldBag_WithGrab` OtherActor))
        (`|ExecutionSequence`
          (:`then_0`
            (bind _asthird_person_character (cast `/Game/ThirdPersonBP/Blueprints/ThirdPersonCharacter` (`/Game/EveryoneProg/Deliveries/BP_GoldBag_WithGrab.Carrier` _asbp_gold_bag_with_grab)))
            (set `/Game/ThirdPersonBP/Blueprints/ThirdPersonCharacter.IsCarrying` false _asthird_person_character))
          (:`then_1`
            (set `/Game/EveryoneProg/Deliveries/BP_GoldBag_WithGrab.Carrier` (`/Game/EveryoneProg/Deliveries/BP_GoldBag_WithGrab.CarrierNone` _asbp_gold_bag_with_grab) _asbp_gold_bag_with_grab)
            (`KismetSystemLibrary.Delay` 0.2)
            (for _ (range 1 (+ (`self.Bag_GoldToSpawn`) 1))
              (`|SpawnActorFromClass` "/Game/EveryoneProg/Treasures/Coin.Coin_C" (`KismetMathLibrary.MakeTransform` (`KismetMathLibrary.RandomPointInBoundingBox` (+ (`SceneComponent.K2_GetComponentLocation` (`/Game/EveryoneProg/Deliveries/BP_GoldBag_WithGrab.bucketMesh` _asbp_gold_bag_with_grab)) (0.0 0.0 100.0)) (`self.SpawnRadius`)) (struct) (3.0 3.0 3.0)) "Undefined" "OverrideRootScale" null true null))
            (`self.K2_DestroyActor` _asbp_gold_bag_with_grab)
            (goto _label :!via `Reset`)))))))

(fn `UserConstructionScript`)