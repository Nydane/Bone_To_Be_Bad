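; BP_TreasureDig is a diggable sand mound that yields coins and a treasure when dug out.
; Each GotHit decrements DigHealth, sinking the actor, shrinking the sand and flashing a brief steam puff.
; At zero it spawns a coin spawner and TreasureToSpawn, plays a burst effect and disables Sand and Box collision.
; The sink and shrink steps are hard-coded, so they depend on tuning against the chosen health.
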(event `/Game/EveryoneProg/BPI_Interact.GotHit`
  (params (PlayerHitting :type "/Game/ThirdPersonBP/Blueprints/ThirdPersonCharacter Object Reference"))
  (bind _defaultsceneroot (`self.DefaultSceneRoot`))
  (bind _sand (`self.Sand`))
  (bind _posdigparticle (`self.PosDigParticle`))
  (bind _coinstospawn (`self.CoinsToSpawn`))
  (bind _posdigparticle_2 (`self.PosDigParticle`))
  (if (> (`self.DigHealth`) 0)
    (bind _result (`/Engine/EditorBlueprintResources/StandardMacros.DecrementInt` (`self.DigHealth`))
      (:`  `
        (if (<= _result 0)
          (`|ExecutionSequence`
            (:`then_0`
              (`|SpawnActorFromClass` "/Game/EveryoneProg/Managers/BP_CoinSpawner.BP_CoinSpawner_C" (`KismetMathLibrary.MakeTransform` (+ (`SceneComponent.K2_GetComponentLocation` (`self.PosDigParticle`)) (0.0 0.0 200.0))) "Undefined" "OverrideRootScale" null (300.0 300.0 75.0) 0.05 _coinstospawn _coinstospawn true true null))
            (:`then_1`
              (`|SpawnActorFromClass` (`self.TreasureToSpawn`) (`KismetMathLibrary.MakeTransform` (`SceneComponent.K2_GetComponentLocation` (`self.PosDigParticle`))) "Undefined" "OverrideRootScale" null null))
            (:`then_2`
              (`GameplayStatics.SpawnEmitterAttached` "/Game/PolygonPack/PolygonPirates/ParticleFX/P_FX_MusketFire.P_FX_MusketFire" _posdigparticle "None" (`SceneComponent.K2_GetComponentLocation` _posdigparticle) (struct :`Pitch` 90.0) (1.5 1.5 1.5) "KeepWorldPosition"))
            (:`then_3`
              (`PrimitiveComponent.SetCollisionEnabled` (`self.Sand`) "NoCollision")
              (`PrimitiveComponent.SetCollisionEnabled` (`self.Box`) "NoCollision")))
          (else
            (`|ExecutionSequence`
              (:`then_0`
                ;[1 1 1] Il faudra bidouiller ces valeurs selon le nombre de PV souhaités pour l'objet.
                (`SceneComponent.K2_SetWorldLocation` _defaultsceneroot (- (`SceneComponent.K2_GetComponentLocation` _defaultsceneroot) (0.0 0.0 7.5)) false false))
              (:`then_1`
                (`SceneComponent.SetWorldScale3D` _sand (- (`SceneComponent.K2_GetComponentScale` _sand) (0.02 0.02 0.0))))
              (:`then_2`
                (bind _returnvalue (`GameplayStatics.SpawnEmitterAttached` "/Game/StarterContent/Particles/P_Steam_Lit.P_Steam_Lit" _posdigparticle_2 "None" (`SceneComponent.K2_GetComponentLocation` _posdigparticle_2) (struct :`Pitch` 90.0) (1.0 1.0 1.0) "KeepWorldPosition"))
                (`KismetSystemLibrary.Delay` 0.1)
                (`ActorComponent.Deactivate` _returnvalue)))))))))

(fn `UserConstructionScript`)