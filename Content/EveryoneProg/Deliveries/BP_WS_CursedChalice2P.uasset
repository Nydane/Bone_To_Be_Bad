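; Cursed chalice delivery object that one or two players carry to a delivery trigger for coins.
; Tick registers carriers through front and back handles, lerps the chalice toward them, and sets CarrySpeedMalus for solo carrying or by distance between the pair.
; Delivery plays the skeleton animation, pays or splits the value with score popup and rumble, optionally spawns coin spawners, then destroys itself.
; An input prompt and wiggle react to nearby players.
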(event `self.Trigger.OnComponentBeginOverlap`
  (params (OverlappedComponent :type "PrimitiveComponent Object Reference") (OtherActor :type "Actor Object Reference") (OtherComp :type "PrimitiveComponent Object Reference") (OtherBodyIndex :type Integer) (bFromSweep :type Boolean) (SweepResult :type "HitResult Structure (by ref)"))
  (bind _skeletondeliveryref (`self.SkeletonDeliveryRef`))
  (bind _returnvalue (`KismetMathLibrary.RandomPointInBoundingBox` (+ (`SceneComponent.K2_GetComponentLocation` (`self.Base`)) (0.0 0.0 200.0)) (50.0 50.0 50.0)))
  (if (== (`GameplayStatics.GetObjectClass` OtherActor) "/Game/EveryoneProg/Managers/BP_DeliveryTrigger.BP_DeliveryTrigger_C")
    (set `/Game/EveryoneProg/Art/SkeletonDelivery.AnimDeliveryPlay` true _skeletondeliveryref)
    (`/Game/EveryoneProg/Art/SkeletonDelivery.PlayAnimDelivery` _skeletondeliveryref)
    (switch `int` (`KismetArrayLibrary.Array_Length` (`self.Carriers`))
      (:`1`
        (bind _asthird_person_character (cast `/Game/ThirdPersonBP/Blueprints/ThirdPersonCharacter` (`|GetArrayItem` (`self.Carriers`))))
        (set `/Game/ThirdPersonBP/Blueprints/ThirdPersonCharacter.Coins` (+ (`/Game/ThirdPersonBP/Blueprints/ThirdPersonCharacter.Coins` _asthird_person_character) (`self.CaliceValue`)) _asthird_person_character)
        (set `/Game/ThirdPersonBP/Blueprints/ThirdPersonCharacter.IsCarrying` false _asthird_person_character)
        (`PlayerController.K2_ClientPlayForceFeedback` (`GameplayStatics.GetPlayerController` (`/Game/ThirdPersonBP/Blueprints/ThirdPersonCharacter.LocalID` _asthird_person_character)) "/Game/ArtAndMusic/Rumbles/ValidateChalice.ValidateChalice" "Chalice" false false false)
        (set `CharacterMovementComponent.MaxWalkSpeed` (`/Game/ThirdPersonBP/Blueprints/ThirdPersonCharacter.BaseWalkSpeed` _asthird_person_character) (`Character.CharacterMovement` _asthird_person_character))
        (bind _aswbp_player_score_increase (cast `/Game/ThirdPersonBP/Blueprints/UI/WBP_PlayerScoreIncrease` (`WidgetComponent.GetUserWidgetObject` (`/Game/ThirdPersonBP/Blueprints/ThirdPersonCharacter.ScoreIncrease` _asthird_person_character))))
        (set `/Game/ThirdPersonBP/Blueprints/UI/WBP_PlayerScoreIncrease.ScoreInt` (`self.CaliceValue`) _aswbp_player_score_increase)
        (`/Game/ThirdPersonBP/Blueprints/UI/WBP_PlayerScoreIncrease.PlayAnimIncrease` _aswbp_player_score_increase))
      (:`2`
        (for _array_element (`self.Carriers`)
          (bind _asthird_person_character_2 (cast `/Game/ThirdPersonBP/Blueprints/ThirdPersonCharacter` _array_element))
          (set `/Game/ThirdPersonBP/Blueprints/ThirdPersonCharacter.Coins` (+ (`/Game/ThirdPersonBP/Blueprints/ThirdPersonCharacter.Coins` _asthird_person_character_2) (/ (`self.CaliceValue`) 2)) _asthird_person_character_2)
          (set `/Game/ThirdPersonBP/Blueprints/ThirdPersonCharacter.IsCarrying` false _asthird_person_character_2)
          (`PlayerController.K2_ClientPlayForceFeedback` (`GameplayStatics.GetPlayerController` (`/Game/ThirdPersonBP/Blueprints/ThirdPersonCharacter.LocalID` _asthird_person_character_2)) "/Game/ArtAndMusic/Rumbles/ValidateChalice.ValidateChalice" "Chalice" false false false)
          (set `CharacterMovementComponent.MaxWalkSpeed` (`/Game/ThirdPersonBP/Blueprints/ThirdPersonCharacter.BaseWalkSpeed` _asthird_person_character_2) (`Character.CharacterMovement` _asthird_person_character_2))
          (bind _aswbp_player_score_increase_2 (cast `/Game/ThirdPersonBP/Blueprints/UI/WBP_PlayerScoreIncrease` (`WidgetComponent.GetUserWidgetObject` (`/Game/ThirdPersonBP/Blueprints/ThirdPersonCharacter.ScoreIncrease` _asthird_person_character_2))))
          (set `/Game/ThirdPersonBP/Blueprints/UI/WBP_PlayerScoreIncrease.ScoreInt` (/ (`self.CaliceValue`) 2) _aswbp_player_score_increase_2)
          (`/Game/ThirdPersonBP/Blueprints/UI/WBP_PlayerScoreIncrease.PlayAnimIncrease` _aswbp_player_score_increase_2))))
    (`KismetArrayLibrary.Array_Clear` (`self.Carriers`))
    (`SceneComponent.K2_DetachFromComponent` (`self.HandleConstraintFront`) "KeepWorld" "KeepWorld" "KeepWorld" true)
    (`SceneComponent.K2_DetachFromComponent` (`self.HandleConstraintBack`) "KeepWorld" "KeepWorld" "KeepWorld" true)
    (if (`self.SpawnGold`)
      (`|ExecutionSequence`
        (:`then_0`
          (`|SpawnActorFromClass` "/Game/EveryoneProg/Managers/BP_CoinSpawner.BP_CoinSpawner_C" (`KismetMathLibrary.MakeTransform` _returnvalue) "AdjustIfPossibleButAlwaysSpawn" "OverrideRootScale" null (150.0 100.0 150.0) 1.0 10 10 true true true null)
          (`self.setSpeedBack` :!label _label)
          (`KismetSystemLibrary.Delay` 0.1)
          (`self.K2_DestroyActor`))
        (:`then_1`
          (`|SpawnActorFromClass` "/Game/EveryoneProg/Managers/BP_CoinSpawner.BP_CoinSpawner_C" (`KismetMathLibrary.MakeTransform` _returnvalue) "AdjustIfPossibleButAlwaysSpawn" "OverrideRootScale" null (150.0 100.0 150.0) 1.0 10 10 true true true null)))
      (else
        (goto _label)))))

(event `setSpeedBack`
  (`|ExecutionSequence`
    (:`then_0`
      (bind _asthird_person_character (cast `/Game/ThirdPersonBP/Blueprints/ThirdPersonCharacter` (`self.BackCarrier`)))
      (set `/Game/ThirdPersonBP/Blueprints/ThirdPersonCharacter.CarrySpeedMalus` 175.0 _asthird_person_character))
    (:`then_1`
      (bind _asthird_person_character_2 (cast `/Game/ThirdPersonBP/Blueprints/ThirdPersonCharacter` (`self.FrontCarrier`)))
      (set `/Game/ThirdPersonBP/Blueprints/ThirdPersonCharacter.CarrySpeedMalus` 175.0 _asthird_person_character_2))))

(event `CheckSpeed`
  (params (Carrier :type "Actor Object Reference") (switch :type Integer))
  (bind _asthird_person_character (cast `/Game/ThirdPersonBP/Blueprints/ThirdPersonCharacter` Carrier))
  (switch `int` switch
    (:`Default`
      (set `/Game/ThirdPersonBP/Blueprints/ThirdPersonCharacter.CarrySpeedMalus` 750.0 _asthird_person_character))
    (:`0`
      (set `/Game/ThirdPersonBP/Blueprints/ThirdPersonCharacter.CarrySpeedMalus` 175.0 _asthird_person_character))
    (:`1`
      (set `/Game/ThirdPersonBP/Blueprints/ThirdPersonCharacter.CarrySpeedMalus` 350.0 _asthird_person_character))
    (:`2`
      (set `/Game/ThirdPersonBP/Blueprints/ThirdPersonCharacter.CarrySpeedMalus` 525.0 _asthird_person_character))))

(event `SpawnChestAnim`
  (bind (_direction _chestscale) (`Timeline|SpawnChest` :!via `PlayFromStart`)
    (:`Update`
      (`SceneComponent.SetRelativeScale3D` (`self.Root`) _chestscale))))

(event `self.ReceiveBeginPlay`
  ;[1 1 1] Setting up everything needed on Begin Play
  (`self.SpawnChestAnim`)
  (set `self.Tags` (`|MakeArray` "Sell" :!type "Name"))
  (set `ActorComponent.ComponentTags` (`|MakeArray` "CarryFront" :!type "Name") (`self.HandleConstraintFront`))
  (set `ActorComponent.ComponentTags` (`|MakeArray` "CarryBack" :!type "Name") (`self.HandleConstraintBack`))
  (`CableComponent.SetAttachEndToComponent` (`self.CableFront`) (`self.HandleConstraintFront`) "None")
  (`CableComponent.SetAttachEndToComponent` (`self.CableBack`) (`self.HandleConstraintBack`) "None")
  (bind _outactors (`GameplayStatics.GetAllActorsOfClass` "/Game/EveryoneProg/Treasures/BP_MagicChestPinata.BP_MagicChestPinata_C"))
  (set `self.MagicChestRef` (`|GetArrayItem` _outactors))
  (set `/Game/EveryoneProg/Art/SkeletonDelivery.ActiveChestRef` self (`self.SkeletonDeliveryRef`))
  (`AudioComponent.FadeIn` (`self.Audio`) 1.0 0.5 3.349 "Linear"))

(event `self.ReceiveTick`
  (params (DeltaSeconds :type "Float (single-precision)"))
  ;[1 1 1 1 123] Promis je commente plus tard, pas taper s'il vous plait !
  (if (`KismetSystemLibrary.IsValid` self)
    (`|ExecutionSequence`
      (:`then_0`
        (if (== (`KismetArrayLibrary.Array_Length` (`self.Carriers`)) 2)
          (set `self.PreviousLocationMarmite` (`SceneComponent.K2_GetComponentLocation` (`self.Root`)))
          (bind _returnvalue (`GameplayStatics.GetActorArrayAverageLocation` (`self.Carriers`)))
          (`SceneComponent.K2_AddRelativeLocation` (`self.Root`) (`KismetMathLibrary.MakeVector` (.x (`KismetMathLibrary.GetVectorArrayAverage` (`|MakeArray` (`SceneComponent.K2_GetComponentLocation` (`self.HandleConstraintBack`)) (`SceneComponent.K2_GetComponentLocation` (`self.HandleConstraintFront`))))) (+ (.y (`KismetMathLibrary.GetVectorArrayAverage` (`|MakeArray` (`SceneComponent.K2_GetComponentLocation` (`self.HandleConstraintBack`)) (`SceneComponent.K2_GetComponentLocation` (`self.HandleConstraintFront`))))) 200.0) (.z (`KismetMathLibrary.GetVectorArrayAverage` (`|MakeArray` (`SceneComponent.K2_GetComponentLocation` (`self.HandleConstraintBack`)) (`SceneComponent.K2_GetComponentLocation` (`self.HandleConstraintFront`)))))) false false)
          (`SceneComponent.K2_SetWorldLocation` (`self.Root`) (`KismetMathLibrary.VLerp` (`self.PreviousLocationMarmite`) _returnvalue 0.3) false false)
          (bind _output_get (set `self.fDistance` (`self.GetDistanceTo` (`self.BackCarrier`) (`self.FrontCarrier`))))
          (`|ExecutionSequence`
            (:`then_0`
              (bind _returnvalue_2 (`KismetMathLibrary.FTrunc` (/ _output_get 200.0)))
              (`self.CheckSpeed` (`self.FrontCarrier`) _returnvalue_2))
            (:`then_1`
              (`self.CheckSpeed` (`self.BackCarrier`) _returnvalue_2)))))
      (:`then_1`
        (if (== (`KismetArrayLibrary.Array_Length` (`self.Carriers`)) 1)
          (`|ExecutionSequence`
            (:`then_0`
              (bind _asthird_person_character (cast `/Game/ThirdPersonBP/Blueprints/ThirdPersonCharacter` (`|GetArrayItem` (`self.Carriers`))))
              (set `/Game/ThirdPersonBP/Blueprints/ThirdPersonCharacter.CarrySpeedMalus` 600.0 _asthird_person_character)
              (bind _output_get_2 (set `self.PreviousLocationMarmite` (`SceneComponent.K2_GetComponentLocation` (`self.Root`))))
              (`SceneComponent.K2_SetWorldLocation` (`self.Root`) (`KismetMathLibrary.VLerp` _output_get_2 (`SceneComponent.K2_GetComponentLocation` (`/Game/ThirdPersonBP/Blueprints/ThirdPersonCharacter.CaliceHelper` _asthird_person_character)) 0.5) false true))
            (:`then_1`
              (goto _label_2 :!via `Reset`)))
          (else
            (`/Engine/EditorBlueprintResources/StandardMacros.DoOnce` false :!label _label_2
              (:`Completed`
                (for _array_element (`self.Carriers`)
                  (bind _asthird_person_character_2 (cast `/Game/ThirdPersonBP/Blueprints/ThirdPersonCharacter` _array_element))
                  (set `/Game/ThirdPersonBP/Blueprints/ThirdPersonCharacter.CarrySpeedMalus` 175.0 _asthird_person_character_2)))))))
      (:`then_2`
        (if (!= (`self.FrontCarrier`) (`self.FrontCarrierNone`))
          (bind _asthird_person_character_3 (cast `/Game/ThirdPersonBP/Blueprints/ThirdPersonCharacter` (`self.FrontCarrier`)))
          (if (`/Game/ThirdPersonBP/Blueprints/ThirdPersonCharacter.IsCarrying` _asthird_person_character_3)
            (`KismetArrayLibrary.Array_AddUnique` (`self.Carriers`) _asthird_person_character_3)
            (`SceneComponent.K2_SetWorldLocation` (`self.HandleConstraintFront`) (`SceneComponent.K2_GetComponentLocation` (`/Game/ThirdPersonBP/Blueprints/ThirdPersonCharacter.GrabLocation` _asthird_person_character_3)) false false)
            (`PrimitiveComponent.SetConstraintMode` (`self.HandleConstraintFront`) "XYPlane")
            (else
              (set `/Game/ThirdPersonBP/Blueprints/ThirdPersonCharacter.CarrySpeedMalus` 175.0 _asthird_person_character_3)
              (set `self.FrontCarrier` (`self.FrontCarrierNone`))
              (`KismetArrayLibrary.Array_RemoveItem` (`self.Carriers`) _asthird_person_character_3)
              (`PrimitiveComponent.SetConstraintMode` (`self.HandleConstraintFront`) "Default")
              (`SceneComponent.K2_SetRelativeLocation` (`self.HandleConstraintFront`) (-17.299999 0.0 9.0) false true)))))
      (:`then_3`
        (if (!= (`self.BackCarrier`) (`self.BackCarrierNone`))
          (bind _asthird_person_character_4 (cast `/Game/ThirdPersonBP/Blueprints/ThirdPersonCharacter` (`self.BackCarrier`)))
          (if (`/Game/ThirdPersonBP/Blueprints/ThirdPersonCharacter.IsCarrying` _asthird_person_character_4)
            (`KismetArrayLibrary.Array_AddUnique` (`self.Carriers`) _asthird_person_character_4)
            (`SceneComponent.K2_SetWorldLocation` (`self.HandleConstraintBack`) (`SceneComponent.K2_GetComponentLocation` (`/Game/ThirdPersonBP/Blueprints/ThirdPersonCharacter.GrabLocation` _asthird_person_character_4)) false false)
            (`PrimitiveComponent.SetConstraintMode` (`self.HandleConstraintBack`) "XYPlane")
            (else
              (set `/Game/ThirdPersonBP/Blueprints/ThirdPersonCharacter.CarrySpeedMalus` 175.0 _asthird_person_character_4)
              (set `self.BackCarrier` (`self.BackCarrierNone`))
              (`KismetArrayLibrary.Array_RemoveItem` (`self.Carriers`) _asthird_person_character_4)
              (`PrimitiveComponent.SetConstraintMode` (`self.HandleConstraintBack`) "Default")
              (`SceneComponent.K2_SetRelativeLocation` (`self.HandleConstraintBack`) (17.299999 0.0 9.0) false true)))))
      (:`then_4`
        (`self.ShowButton`)))))

(event `self.ShowInputTrigger.OnComponentBeginOverlap`
  (params (OverlappedComponent :type "PrimitiveComponent Object Reference") (OtherActor :type "Actor Object Reference") (OtherComp :type "PrimitiveComponent Object Reference") (OtherBodyIndex :type Integer) (bFromSweep :type Boolean) (SweepResult :type "HitResult Structure (by ref)"))
  (if (== (`GameplayStatics.GetObjectClass` OtherActor) "/Game/ThirdPersonBP/Blueprints/ThirdPersonCharacter.ThirdPersonCharacter_C")
    (if (< (`KismetArrayLibrary.Array_Length` (`self.Carriers`)) 2)
      (`self.WiggleCalice`))))

(event `ShowButton`
  (bind _input (`self.Input`))
  (if (and (> (`KismetArrayLibrary.Array_Length` (`PrimitiveComponent.GetOverlappingActors` (`self.ShowInputTrigger`) "/Game/ThirdPersonBP/Blueprints/ThirdPersonCharacter.ThirdPersonCharacter_C")) 0) (< (`KismetArrayLibrary.Array_Length` (`self.Carriers`)) 2))
    (`SceneComponent.SetVisibility` _input true false)
    (else
      (`SceneComponent.SetVisibility` _input false false))))

(event `WiggleCalice`
  (bind (_relativescale3d_x _relativescale3d_y _relativescale3d_z) (`KismetMathLibrary.BreakVector` (`SceneComponent.RelativeScale3D` (`self.Base`))))
  (bind (_direction _alpha _scalex _scaley _scalez) (`Timeline|WigglePlayers` :!via `PlayFromStart`)
    (:`Update`
      (set `self.Alpha` _alpha)
      (`SceneComponent.SetRelativeScale3D` (`self.Base`) (`KismetMathLibrary.MakeVector` (`KismetMathLibrary.Lerp` _relativescale3d_x _scalex (`self.Alpha`)) (`KismetMathLibrary.Lerp` _relativescale3d_y _scaley (`self.Alpha`)) (`KismetMathLibrary.Lerp` _relativescale3d_z _scalez (`self.Alpha`)))))))

(fn `UserConstructionScript`)