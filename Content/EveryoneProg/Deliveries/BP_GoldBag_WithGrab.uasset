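; Carryable gold bag tagged for carrying and selling, which players grab and which cannot be stolen mid-carry.
; Tick polls the attach parent to pin the mesh to the carrier's grab point; on release it detaches and restores walk speed unless state forbids.
; A proximity trigger shows a grab icon alternating B/Y sprites and wiggles the bag.
; DoOnce pairs gate state changes; the timed destroy-into-coins logic is disconnected.
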(event `ChangeButton`
  (bind _icongrab (`self.IconGrab`))
  (`/Engine/EditorBlueprintResources/StandardMacros.DoOnce` false :!label _label
    (:`Completed`
      (`KismetSystemLibrary.Delay` 1.5)
      (`/Engine/EditorBlueprintResources/StandardMacros.FlipFlop`
        (:`A`
          (`BillboardComponent.SetSprite` _icongrab "/Game/ArtAndMusic/Art/B_Button_NEW.B_Button_NEW")
          (goto _label :!via `Reset`))
        (:`B`
          (`BillboardComponent.SetSprite` _icongrab "/Game/ArtAndMusic/Art/Y_Button_NEW.Y_Button_NEW")
          (goto _label :!via `Reset`))))))

(event `self.ReceiveBeginPlay`
  (set `self.Tags` (`|MakeArray` "Carry" "Sell" :!type "Name"))
  (bind _outactors (`GameplayStatics.GetAllActorsOfClass` "/Game/EveryoneProg/Treasures/BP_MagicChestPinata.BP_MagicChestPinata_C"))
  (set `self.MagicChestRef` (`|GetArrayItem` _outactors)))

(event `self.ReceiveTick`
  (params (DeltaSeconds :type "Float (single-precision)"))
  (bind _icongrab (`self.IconGrab`))
  (`|ExecutionSequence`
    (:`then_0`
      (if (== (`GameplayStatics.GetObjectClass` (`self.GetAttachParentActor` self)) "/Game/ThirdPersonBP/Blueprints/ThirdPersonCharacter.ThirdPersonCharacter_C")
        (`PrimitiveComponent.SetCollisionEnabled` (`self.TriggerVisGrab`) "NoCollision")
        (bind _asthird_person_character (cast `/Game/ThirdPersonBP/Blueprints/ThirdPersonCharacter` (`self.GetAttachParentActor` self)))
        (if (`/Game/ThirdPersonBP/Blueprints/ThirdPersonCharacter.IsCarrying` _asthird_person_character)
          (set `self.Carrier` _asthird_person_character)
          (`SceneComponent.K2_SetWorldLocation` (`self.BagMesh`) (`SceneComponent.K2_GetComponentLocation` (`/Game/ThirdPersonBP/Blueprints/ThirdPersonCharacter.GrabLocation` _asthird_person_character)) false true)
          (if (`KismetSystemLibrary.IsValid` self)
            (`PrimitiveComponent.SetConstraintMode` (`self.BagMesh`) "XYPlane")
            ;[1 1 1] This Tag allows us to make sure that the object cannot be "stolen" simply by pressing the Grab Button.
            (`/Engine/EditorBlueprintResources/StandardMacros.DoOnce` false :!label _label_2
              (:`Completed`
                (`KismetArrayLibrary.Array_AddUnique` (`self.Tags`) (`self.CarriedTag`))
                (set `self.isCarried` true)
                (goto _label_3 :!via `Reset`))))
          (else
            ;[1 1 1] A terme, détruire le Seau !
            (`SceneComponent.K2_DetachFromComponent` (`self.BagMesh`) "KeepWorld" "KeepWorld" "KeepWorld" true)
            (`SceneComponent.K2_DetachFromComponent` (`self.RootComponent`) "KeepWorld" "KeepWorld" "KeepWorld" true)
            (`PrimitiveComponent.SetConstraintMode` (`self.BagMesh`) "Default")
            (bind _asthird_person_character_2 (cast `/Game/ThirdPersonBP/Blueprints/ThirdPersonCharacter` (`self.Carrier`)))
            (if (not (`|EnumEquality` (`/Game/ThirdPersonBP/Blueprints/ThirdPersonCharacter.CurrentState` _asthird_person_character_2) "NewEnumerator2"))
              (set `CharacterMovementComponent.MaxWalkSpeed` (`/Game/ThirdPersonBP/Blueprints/ThirdPersonCharacter.BaseWalkSpeed` _asthird_person_character_2) (`Character.CharacterMovement` _asthird_person_character_2)))
            (`KismetSystemLibrary.Delay` 0.1)
            (set `self.Carrier` (`self.CarrierNone`))
            (`/Engine/EditorBlueprintResources/StandardMacros.DoOnce` false :!label _label_3
              (:`Completed`
                (`KismetArrayLibrary.Array_RemoveItem` (`self.Tags`) (`self.CarriedTag`))
                (set `self.isCarried` false)
                (goto _label_2 :!via `Reset`)))))
        (else
          (`PrimitiveComponent.SetCollisionEnabled` (`self.TriggerVisGrab`) "QueryAndPhysics"))))
    (:`then_1`
      (if (`KismetSystemLibrary.IsValid` self)
        (if (> (`KismetArrayLibrary.Array_Length` (`PrimitiveComponent.GetOverlappingActors` (`self.TriggerVisGrab`) "/Game/ThirdPersonBP/Blueprints/ThirdPersonCharacter.ThirdPersonCharacter_C")) 0)
          (`/Engine/EditorBlueprintResources/StandardMacros.DoOnce` false :!label _label_4
            (:`Completed`
              (`KismetSystemLibrary.PrintString` "Hello")
              (`self.PlayerClose`)
              (`SceneComponent.SetHiddenInGame` _icongrab false false)
              (goto _label_5 :!via `Reset`)))
          (else
            (`/Engine/EditorBlueprintResources/StandardMacros.DoOnce` false :!label _label_5
              (:`Completed`
                (`SceneComponent.SetHiddenInGame` _icongrab true false)
                (goto _label_4 :!via `Reset`)))))))
    (:`then_2`
      (`self.ChangeButton`))))

(event `PlayerClose`
  (bind (_relativescale3d_x _relativescale3d_y _relativescale3d_z) (`KismetMathLibrary.BreakVector` (`SceneComponent.RelativeScale3D` (`self.BagMesh`))))
  (bind (_direction _alpha _scalex _scaley _scalez) (`Timeline|WiggleGoldBag` :!via `PlayFromStart`)
    (:`Update`
      (set `self.Alpha` _alpha)
      (`SceneComponent.SetRelativeScale3D` (`self.BagMesh`) (`KismetMathLibrary.MakeVector` (`KismetMathLibrary.Lerp` _relativescale3d_x _scalex (`self.Alpha`)) (`KismetMathLibrary.Lerp` _relativescale3d_y _scaley (`self.Alpha`)) (`KismetMathLibrary.Lerp` _relativescale3d_z _scalez (`self.Alpha`)))))))

(fn `UserConstructionScript`)