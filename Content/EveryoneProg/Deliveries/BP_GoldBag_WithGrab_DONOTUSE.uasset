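; Carryable gold bag pickup, marked DONOTUSE, that players grab and deliver to BP_IntroSloop, triggering a zero-score popup, sound and self-destruction.
; Tick polls the attach parent to follow the carrier's grab point, toggling physics and carried tag through cross-reset DoOnce gates; release detaches it and restores walk speed.
; Nearby players trigger a wiggle and grab icon.
; Button-icon flipping and uncarried timeout into coins are disconnected.
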(event `self.Trigger.OnComponentBeginOverlap`
  (params (OverlappedComponent :type "PrimitiveComponent Object Reference") (OtherActor :type "Actor Object Reference") (OtherComp :type "PrimitiveComponent Object Reference") (OtherBodyIndex :type Integer) (bFromSweep :type Boolean) (SweepResult :type "HitResult Structure (by ref)"))
  (if (== (`GameplayStatics.GetObjectClass` OtherActor) "/Game/EveryoneProg/Treasures/BP_IntroSloop.BP_IntroSloop_C")
    (bind _asthird_person_character (cast `/Game/ThirdPersonBP/Blueprints/ThirdPersonCharacter` (`self.Carrier`)))
    (bind _aswbp_player_score_increase (cast `/Game/ThirdPersonBP/Blueprints/UI/WBP_PlayerScoreIncrease` (`WidgetComponent.GetUserWidgetObject` (`/Game/ThirdPersonBP/Blueprints/ThirdPersonCharacter.ScoreIncrease` _asthird_person_character))))
    (set `/Game/ThirdPersonBP/Blueprints/UI/WBP_PlayerScoreIncrease.ScoreInt` 0 _aswbp_player_score_increase)
    (`/Game/ThirdPersonBP/Blueprints/UI/WBP_PlayerScoreIncrease.PlayAnimIncrease` _aswbp_player_score_increase)
    (`GameplayStatics.PlaySound2D` "/Game/ArtAndMusic/Music/Bruitages/Service_validé.Service_validé" 0.5 1.0 0.0 null null)
    (`self.StopCarry`)
    (`KismetSystemLibrary.Delay` 0.11)
    (`self.K2_DestroyActor` self)))

(event `ChangeButton`
  (bind _icongrab (`self.IconGrab`))
  (`/Engine/EditorBlueprintResources/StandardMacros.DoOnce` false :!label _label
    (:`Completed`
      (`KismetSystemLibrary.Delay` 1.5)
      (`/Engine/EditorBlueprintResources/StandardMacros.FlipFlop`
        (:`A`
          (`BillboardComponent.SetSprite` _icongrab "/Game/ArtAndMusic/Art/B_Button_NEW.B_Button_NEW")
          (goto _label :!via `Reset`))
        (:`B`
          (`BillboardComponent.SetSprite` _icongrab "/Game/ArtAndMusic/Art/Y_Button_NEW.Y_Button_NEW")
          (goto _label :!via `Reset`))))))

(event `self.ReceiveBeginPlay`
  (set `self.Tags` (`|MakeArray` "Carry" "Sell" :!type "Name"))
  (bind _outactors (`GameplayStatics.GetAllActorsOfClass` "/Game/EveryoneProg/Treasures/BP_MagicChestPinata.BP_MagicChestPinata_C"))
  (set `self.MagicChestRef` (`|GetArrayItem` _outactors)))

(event `self.ReceiveTick`
  (params (DeltaSeconds :type "Float (single-precision)"))
  (bind _bagmesh (`self.BagMesh`))
  (bind _bagmesh_2 (`self.BagMesh`))
  (bind _bagmesh_3 (`self.BagMesh`))
  (bind _bagmesh_4 (`self.BagMesh`))
  (bind _icongrab (`self.IconGrab`))
  (`|ExecutionSequence`
    (:`then_0`
      (if (== (`GameplayStatics.GetObjectClass` (`self.GetAttachParentActor` self)) "/Game/ThirdPersonBP/Blueprints/ThirdPersonCharacter.ThirdPersonCharacter_C")
        (`PrimitiveComponent.SetCollisionEnabled` (`self.TriggerVisGrab`) "NoCollision")
        (bind _asthird_person_character (cast `/Game/ThirdPersonBP/Blueprints/ThirdPersonCharacter` (`self.GetAttachParentActor` self)))
        (if (`/Game/ThirdPersonBP/Blueprints/ThirdPersonCharacter.IsCarrying` _asthird_person_character)
          (set `self.Carrier` _asthird_person_character)
          (`SceneComponent.K2_SetWorldLocation` (`self.BagMesh`) (`SceneComponent.K2_GetComponentLocation` (`/Game/ThirdPersonBP/Blueprints/ThirdPersonCharacter.GrabLocation` _asthird_person_character)) false true)
          (if (`KismetSystemLibrary.IsValid` self)
            (`PrimitiveComponent.SetConstraintMode` _bagmesh "XYPlane")
            (`SceneComponent.K2_SetWorldRotation` :`self` _bagmesh)
            ;[1 1 1] This Tag allows us to make sure that the object cannot be "stolen" simply by pressing the Grab Button.
            (`/Engine/EditorBlueprintResources/StandardMacros.DoOnce` false :!label _label_2
              (:`Completed`
                (`PrimitiveComponent.SetCollisionEnabled` _bagmesh_4 "NoCollision")
                (`PrimitiveComponent.SetSimulatePhysics` _bagmesh_4 false)
                (`KismetArrayLibrary.Array_AddUnique` (`self.Tags`) (`self.CarriedTag`))
                (set `self.isCarried` true)
                (goto _label_4 :!via `Reset`))))
          (else
            ;[1 1 1] A terme, détruire le Seau !
            (`SceneComponent.K2_DetachFromComponent` (`self.BagMesh`) "KeepWorld" "KeepWorld" "KeepWorld" true :!label _label_3)
            (`SceneComponent.K2_DetachFromComponent` (`self.RootComponent`) "KeepWorld" "KeepWorld" "KeepWorld" true)
            (`PrimitiveComponent.SetConstraintMode` _bagmesh_2 "Default")
            (`SceneComponent.K2_SetWorldRotation` :`self` _bagmesh_2)
            (bind _asthird_person_character_2 (cast `/Game/ThirdPersonBP/Blueprints/ThirdPersonCharacter` (`self.Carrier`)))
            (if (not (`|EnumEquality` (`/Game/ThirdPersonBP/Blueprints/ThirdPersonCharacter.CurrentState` _asthird_person_character_2) "NewEnumerator2"))
              (set `CharacterMovementComponent.MaxWalkSpeed` (`/Game/ThirdPersonBP/Blueprints/ThirdPersonCharacter.BaseWalkSpeed` _asthird_person_character_2) (`Character.CharacterMovement` _asthird_person_character_2)))
            (`KismetSystemLibrary.Delay` 0.1)
            (set `self.Carrier` (`self.CarrierNone`))
            (`/Engine/EditorBlueprintResources/StandardMacros.DoOnce` false :!label _label_4
              (:`Completed`
                (`PrimitiveComponent.SetCollisionEnabled` _bagmesh_3 "QueryAndPhysics")
                (`PrimitiveComponent.SetSimulatePhysics` _bagmesh_3 true)
                (`KismetArrayLibrary.Array_RemoveItem` (`self.Tags`) (`self.CarriedTag`))
                (set `self.isCarried` false)
                (goto _label_2 :!via `Reset`)))))
        (else
          (`PrimitiveComponent.SetCollisionEnabled` (`self.TriggerVisGrab`) "QueryAndPhysics"))))
    (:`then_1`
      (if (`KismetSystemLibrary.IsValid` self)
        (if (> (`KismetArrayLibrary.Array_Length` (`PrimitiveComponent.GetOverlappingActors` (`self.TriggerVisGrab`) "/Game/ThirdPersonBP/Blueprints/ThirdPersonCharacter.ThirdPersonCharacter_C")) 0)
          (`/Engine/EditorBlueprintResources/StandardMacros.DoOnce` false :!label _label_5
            (:`Completed`
              (`self.PlayerClose`)
              (`SceneComponent.SetHiddenInGame` _icongrab false false)
              (goto _label_6 :!via `Reset`)))
          (else
            (`/Engine/EditorBlueprintResources/StandardMacros.DoOnce` false :!label _label_6
              (:`Completed`
                (`SceneComponent.SetHiddenInGame` _icongrab true false)
                (goto _label_5 :!via `Reset`)))))))))

(event `StopCarry`
  (goto _label_3))

(event `PlayerClose`
  (bind (_relativescale3d_x _relativescale3d_y _relativescale3d_z) (`KismetMathLibrary.BreakVector` (`SceneComponent.RelativeScale3D` (`self.BagMesh`))))
  (bind (_direction _alpha _scalex _scaley _scalez) (`Timeline|WiggleGoldBag` :!via `PlayFromStart`)
    (:`Update`
      (set `self.Alpha` _alpha)
      (`SceneComponent.SetRelativeScale3D` (`self.BagMesh`) (`KismetMathLibrary.MakeVector` (`KismetMathLibrary.Lerp` _relativescale3d_x _scalex (`self.Alpha`)) (`KismetMathLibrary.Lerp` _relativescale3d_y _scaley (`self.Alpha`)) (`KismetMathLibrary.Lerp` _relativescale3d_z _scalez (`self.Alpha`)))))))

(fn `UserConstructionScript`)