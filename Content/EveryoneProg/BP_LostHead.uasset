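; BP_LostHead is a detached player head that hops around the level until a headless player touches it, restoring them to alive and destroying itself.
; Tick periodically sphere-traces for a nearby headless player, otherwise targeting the first TargetPoint tagged "HeadLost".
; Each hop plays squash-scale and rotation timelines, then applies a velocity-change impulse with upward lift to CubeHelper.
; A timeline pulses the colored point light.
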(event `self.ReceiveBeginPlay`
  (`TimelineComponent.SetPlayRate` (`self.LightPulse`) 0.2)
  (`self.PulseLight`)
  (`LightComponent.SetLightColor` (`self.PointLight`) (`self.HeadLightColor`) true)
  (bind _outactors (`GameplayStatics.GetAllActorsOfClassWithTag` "/Script/Engine.TargetPoint" "HeadLost"))
  (set `self.TargetPoint` (`|GetArrayItem` _outactors)))

(event `BumpToTargetPoint`
  (bind (_returnvalue_x _returnvalue_y _returnvalue_z) (`KismetMathLibrary.BreakVector` (* (`KismetMathLibrary.GetDirectionUnitVector` (`SceneComponent.K2_GetComponentLocation` (`self.HeadMesh`)) (`SceneComponent.K2_GetComponentLocation` (`Actor.RootComponent` (`self.TargetPoint`)))) (`self.StrengthBump`))))
  ;[1 1 1 1 36] Possibilité d'ajouter une animation ici !
  ; Mais sera dur de faire Rotate la tête sans casser la logique de l'Impulse, il faut plus creuser pour qu'on réussisse à obtenir un résultat satisfaisant.
  (`/Engine/EditorBlueprintResources/StandardMacros.DoOnce` false :!label _label
    (:`Completed`
      (`self.SkullJumpAnim`)
      (`self.RotateTP`)
      (`KismetSystemLibrary.Delay` 0.5)
      (`PrimitiveComponent.AddImpulse` (`self.CubeHelper`) (`KismetMathLibrary.MakeVector` _returnvalue_x _returnvalue_y (+ _returnvalue_z 300.0)) "None" true)
      (goto _label :!via `Reset`))))

(event `self.Box.OnComponentBeginOverlap`
  (params (OverlappedComponent :type "PrimitiveComponent Object Reference") (OtherActor :type "Actor Object Reference") (OtherComp :type "PrimitiveComponent Object Reference") (OtherBodyIndex :type Integer) (bFromSweep :type Boolean) (SweepResult :type "HitResult Structure (by ref)"))
  ;[1 1 1] Has the Head come into contact with a Player? We check this first since it is the only Actor that would interact with the Head.
  (if (== (`GameplayStatics.GetObjectClass` OtherActor) (`self.PlayerClass`))
    (bind _output_get (set `self.PlayerHit` OtherActor))
    ;[1 1 1] This part allows us to change the State of a Headless Player and give their Head back.
    (bind _asthird_person_character (cast `/Game/ThirdPersonBP/Blueprints/ThirdPersonCharacter` _output_get))
    (if (`|EnumEquality` (`/Game/ThirdPersonBP/Blueprints/ThirdPersonCharacter.CurrentState` _asthird_person_character) "NewEnumerator1")
      ;;[1 1 1] If they're Headless, we change their State to "Alive"
      (set `/Game/ThirdPersonBP/Blueprints/ThirdPersonCharacter.CurrentState` "NewEnumerator0" _asthird_person_character)
      ;;[1 1 1] We then call "Check State" to set everything up within the Player.
      (`/Game/ThirdPersonBP/Blueprints/ThirdPersonCharacter.Check State` _asthird_person_character)
      (`GameplayStatics.PlaySound2D` "/Game/ArtAndMusic/Music/Bruitages/Perte_tête_4.Perte_tête_4" 0.5 0.75 0.0 null null)
      ;;[1 1 1] We then destroy the Head.
      (`self.K2_DestroyActor` self))))

(event `BumpToPlayer`
  (bind (_returnvalue_x _returnvalue_y _returnvalue_z) (`KismetMathLibrary.BreakVector` (* (`KismetMathLibrary.GetDirectionUnitVector` (`SceneComponent.K2_GetComponentLocation` (`self.HeadMesh`)) (`SceneComponent.K2_GetComponentLocation` (`Actor.RootComponent` (`self.HeadlessPlayer`)))) (`self.StrengthBump`))))
  ;[1 1 1 1 36] Possibilité d'ajouter une animation ici !
  ; Mais sera dur de faire Rotate la tête sans casser la logique de l'Impulse, il faut plus creuser pour qu'on réussisse à obtenir un résultat satisfaisant.
  (`/Engine/EditorBlueprintResources/StandardMacros.DoOnce` false :!label _label_2
    (:`Completed`
      (`self.SkullJumpAnim`)
      (`self.RotateToPlayer`)
      (`KismetSystemLibrary.Delay` 0.5)
      (`PrimitiveComponent.AddImpulse` (`self.CubeHelper`) (`KismetMathLibrary.MakeVector` _returnvalue_x _returnvalue_y (+ _returnvalue_z 300.0)) "None" true)
      (set `self.HeadlessPlayer` (`self.PlayerNone`))
      (goto _label_2 :!via `Reset`))))

(event `PulseLight`
  ;[1 1 1] VIS : Pulse Light
  (bind (_direction _alpha _intensity) (`Timeline|LightPulse`)
    (:`Update`
      (set `self.Alpha` _alpha)
      (`LightComponent.SetIntensity` (`self.PointLight`) (`KismetMathLibrary.Lerp` (`LightComponentBase.Intensity` (`self.PointLight`)) (* 16.0 _intensity) (`self.Alpha`))))))

(event `SkullJumpAnim`
  (bind (_relativescale3d_x _relativescale3d_y _relativescale3d_z) (`KismetMathLibrary.BreakVector` (`SceneComponent.RelativeScale3D` (`self.HeadMesh`))))
  (bind (_direction _alphascale _scalex _scaley _scalez) (`Timeline|SkullJump` :!via `PlayFromStart`)
    (:`Update`
      (set `self.Alpha Scale` _alphascale)
      (`SceneComponent.SetRelativeScale3D` (`self.HeadMesh`) (`KismetMathLibrary.MakeVector` (`KismetMathLibrary.Lerp` _relativescale3d_x _scalex (`self.Alpha Scale`)) (`KismetMathLibrary.Lerp` _relativescale3d_y _scaley (`self.Alpha Scale`)) (`KismetMathLibrary.Lerp` _relativescale3d_z _scalez (`self.Alpha Scale`)))))))

(event `self.ReceiveTick`
  (params (DeltaSeconds :type "Float (single-precision)"))
  (bind _returnvalue (`SceneComponent.K2_GetComponentLocation` (`self.CubeHelper`)))
  ;[1 1 1 1 36] Logique gérant où le crâne ira :
  ; S'il détecte un joueur Headless, il saute vers lui.
  ; S'il n'en détecte pas, il saute vers un TargetPoint ayant le "HeadLost" en Tag.
  (`|ExecutionSequence`
    (:`then_0`
      (`KismetSystemLibrary.Delay` 2.0)
      (`/Engine/EditorBlueprintResources/StandardMacros.DoOnce` false :!label _label_3
        (:`Completed`
          (bind (_outhits _returnvalue_2) (`KismetSystemLibrary.SphereTraceMultiForObjects` _returnvalue _returnvalue 600.0 (`|MakeArray` "ObjectTypeQuery3" :!type "EObjectTypeQuery Enum")))
          (if _returnvalue_2
            (for _array_element _outhits
              (bind (_bblockinghit _binitialoverlap _time _distance _location _impactpoint _normal _impactnormal _physmat _hitactor) (`GameplayStatics.BreakHitResult` _array_element))
              (if (== (`GameplayStatics.GetObjectClass` _hitactor) "/Game/ThirdPersonBP/Blueprints/ThirdPersonCharacter.ThirdPersonCharacter_C")
                (bind _asthird_person_character (cast `/Game/ThirdPersonBP/Blueprints/ThirdPersonCharacter` _hitactor))
                (if (`|EnumEquality` (`/Game/ThirdPersonBP/Blueprints/ThirdPersonCharacter.CurrentState` _asthird_person_character) "NewEnumerator1")
                  (set `self.HeadlessPlayer` _asthird_person_character)
                  (break))))
            (if (!= (`self.HeadlessPlayer`) (`self.PlayerNone`))
              (`self.BumpToPlayer`)
              (goto _label_3 :!via `Reset`)
              (else
                (`self.BumpToTargetPoint`)
                (goto _label_3 :!via `Reset`)))
            (else
              (`self.BumpToTargetPoint`)
              (goto _label_3 :!via `Reset`))))))
    (:`then_1`
      (if (`KismetSystemLibrary.IsValid` (`self.HeadlessPlayer`))
        _))))

(event `RotateTP`
  (bind (_direction _alphatargetpoint) (`Timeline|RotateToTargetPoint` :!via `PlayFromStart`)
    (:`Finished`
      (bind (_returnvalue_roll _returnvalue_pitch _returnvalue_yaw) (`KismetMathLibrary.BreakRotator` (`KismetMathLibrary.RLerp` (`SceneComponent.K2_GetComponentRotation` (`self.HeadMesh`)) (`KismetMathLibrary.FindLookAtRotation` (`SceneComponent.K2_GetComponentLocation` (`self.HeadMesh`)) (`SceneComponent.K2_GetComponentLocation` (`Actor.RootComponent` (`self.TargetPoint`)))) _alphatargetpoint)))
      (`SceneComponent.K2_SetRelativeRotation` (`self.HeadMesh`) (`KismetMathLibrary.MakeRotator` _returnvalue_roll _returnvalue_pitch _returnvalue_yaw) false false))))

(event `RotateToPlayer`
  (bind (_direction _newtrack_0) (`Timeline|RotateTowardsPlayer` :!via `PlayFromStart`)
    (:`Update`
      (bind (_returnvalue_roll _returnvalue_pitch _returnvalue_yaw) (`KismetMathLibrary.BreakRotator` (`KismetMathLibrary.RLerp` (`SceneComponent.K2_GetComponentRotation` (`self.HeadMesh`)) (`KismetMathLibrary.FindLookAtRotation` (`SceneComponent.K2_GetComponentLocation` (`self.HeadMesh`)) (`SceneComponent.K2_GetComponentLocation` (`Actor.RootComponent` (`self.HeadlessPlayer`)))) _newtrack_0)))
      (`SceneComponent.K2_SetRelativeRotation` (`self.HeadMesh`) (`KismetMathLibrary.MakeRotator` _returnvalue_roll _returnvalue_pitch _returnvalue_yaw) false false))))

(fn `UserConstructionScript`)