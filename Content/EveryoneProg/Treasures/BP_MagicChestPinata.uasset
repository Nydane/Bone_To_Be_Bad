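; Treasure chest piñata that, once its cooldown ends, lets players headbutt it for gold during a timed window.
; Tick counts cooldown seconds and uses paired DoOnce gates to toggle the ready visuals and nearby button prompt.
; Each hit awards coins, plays feedback and grows a hit counter.
; The first hit starts the timer, which ends by spawning coins equal to the hit count and restarting the cooldown.
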(event `VisChest`
  (bind _rectlight (`self.RectLight`))
  (bind _goldpile (`self.GoldPile`))
  (bind _headbuttnumber (`self.HeadbuttNumber`))
  (bind _lid (`self.Lid`))
  ;[1 1 1] VisChest: Only handles how the Magic Chest looks, in order to let players know if they can interact with the item.
  (if (`self.CanPinata`)
    (`/Engine/EditorBlueprintResources/StandardMacros.DoOnce` false :!label _label
      (:`Completed`
        (`LightComponent.SetIntensity` _rectlight 9000.0)
        (`SceneComponent.SetHiddenInGame` _goldpile false false)
        (`self.PlayChestAnimActive`)
        (`SceneComponent.SetVisibility` _headbuttnumber true false)
        (`SceneComponent.K2_SetRelativeRotation` _lid (struct :`Roll` -30.0) false false)
        (goto _label_2 :!via `Reset`)))
    (else
      (`/Engine/EditorBlueprintResources/StandardMacros.DoOnce` false :!label _label_2
        (:`Completed`
          (`LightComponent.SetIntensity` _rectlight 500.0)
          (`SceneComponent.SetHiddenInGame` _goldpile true false)
          (`SceneComponent.SetVisibility` _headbuttnumber false false)
          (`SceneComponent.K2_SetRelativeRotation` _lid (struct :`Roll` -10.0) false false)
          (goto _label :!via `Reset`))))))

(event `PlayChestAnimActive`
  (bind (_relativescale3d_x _relativescale3d_y _relativescale3d_z) (`KismetMathLibrary.BreakVector` (`SceneComponent.RelativeScale3D` (`self.BotChest`))))
  ;[1 1 1] Anim Chest Active: Tiny wiggle to let the players know that the Chest can be used
  (bind (_direction _alpha _scalechest) (`Timeline|ChestActive` :!via `PlayFromStart`)
    (:`Update`
      (set `self.AlphaChestActive` _alpha)
      (`SceneComponent.SetRelativeScale3D` (`self.BotChest`) (`KismetMathLibrary.MakeVector` (`KismetMathLibrary.Lerp` _relativescale3d_x _scalechest (`self.AlphaChestActive`)) (`KismetMathLibrary.Lerp` _relativescale3d_y _scalechest (`self.AlphaChestActive`)) (`KismetMathLibrary.Lerp` _relativescale3d_z _scalechest (`self.AlphaChestActive`)))))))

(event `self.ReceiveTick`
  (params (DeltaSeconds :type "Float (single-precision)"))
  (bind _buttonshow (`self.ButtonShow`))
  (`|ExecutionSequence`
    (:`then_0`
      (`/Engine/EditorBlueprintResources/StandardMacros.DoOnce` false :!label _label_3
        (:`Completed`
          (`KismetSystemLibrary.Delay` 1.0)
          (`/Engine/EditorBlueprintResources/StandardMacros.IncrementInt` (`self.CooldownIntern`)
            (:`  `
              (goto _label_3 :!via `Reset`))))))
    (:`then_1`
      (`self.VisChest`))
    (:`then_2`
      (if (>= (`self.CooldownIntern`) (`self.DelayBeforeActive`))
        (set `self.CanPinata` true)
        (else
          (set `self.CanPinata` false))))
    (:`then_3`
      (if (and (> (`KismetArrayLibrary.Array_Length` (`PrimitiveComponent.GetOverlappingActors` (`self.HeadbuttVis`) "/Game/ThirdPersonBP/Blueprints/ThirdPersonCharacter.ThirdPersonCharacter_C")) 0) (`self.CanPinata`))
        (`/Engine/EditorBlueprintResources/StandardMacros.DoOnce` false :!label _label_4
          (:`Completed`
            (`SceneComponent.SetHiddenInGame` _buttonshow false false)
            (goto _label_5 :!via `Reset`)))
        (else
          (`/Engine/EditorBlueprintResources/StandardMacros.DoOnce` false :!label _label_5
            (:`Completed`
              (`SceneComponent.SetHiddenInGame` _buttonshow true false)
              (goto _label_4 :!via `Reset`))))))
    (:`then_4`
      (`self.TextSize`))))

(event `/Game/EveryoneProg/BPI_Interact.CountGold`
  (params (Gold :type Integer))
  (set `self.GoldCollected` (+ (`self.GoldCollected`) (/ Gold 4))))

(event `TimerPinata`
  (bind _timeshit (`self.timesHit`))
  (`KismetSystemLibrary.Delay` (`KismetMathLibrary.Conv_IntToDouble` (`self.ActivationDuration`)))
  (`|SpawnActorFromClass` "/Game/EveryoneProg/Managers/BP_CoinSpawner.BP_CoinSpawner_C" (`KismetMathLibrary.MakeTransform` (`SceneComponent.K2_GetComponentLocation` (`self.Scene`))) "Undefined" "OverrideRootScale" null (100.0 100.0 25.0) 1.0 _timeshit _timeshit true true null)
  (`GameplayStatics.PlaySound2D` "/Game/ArtAndMusic/Music/Bruitages/Coffre_-_Fin_Event.Coffre_-_Fin_Event" 0.5 1.0 0.0 null null)
  (set `self.CooldownIntern` 0)
  (set `self.timesHit` 0)
  (`TextRenderComponent.K2_SetText` (`self.HeadbuttNumber`) " ")
  (set `self.CanPinata` false)
  (`LightComponent.SetIntensity` (`self.SpotLight`) 0.0))

(event `AnimChestReactHit`
  (bind (_direction _scale) (`Timeline|ChestHit` :!via `PlayFromStart`)
    (:`Update`
      (`SceneComponent.SetRelativeScale3D` (`self.BotChest`) (`KismetMathLibrary.MakeVector` _scale _scale _scale)))))

(event `/Game/EveryoneProg/BPI_Interact.GotHit`
  (params (PlayerHitting :type "/Game/ThirdPersonBP/Blueprints/ThirdPersonCharacter Object Reference"))
  (if (`self.CanPinata`)
    (`/Game/ThirdPersonBP/Blueprints/ThirdPersonCharacter.RumbleObjectHeadbutt` PlayerHitting)
    (`|ExecutionSequence`
      (:`then_0`
        (`GameplayStatics.PlaySound2D` "/Game/ArtAndMusic/Music/Bruitages/HeadLaunch.HeadLaunch" 1.0 1.0 0.0 null null)
        (`self.AnimChestReactHit`)
        (set `/Game/ThirdPersonBP/Blueprints/ThirdPersonCharacter.Coins` (+ (`/Game/ThirdPersonBP/Blueprints/ThirdPersonCharacter.Coins` PlayerHitting) (`self.GoldGain`)) PlayerHitting)
        (bind _aswbp_player_score_increase (cast `/Game/ThirdPersonBP/Blueprints/UI/WBP_PlayerScoreIncrease` (`WidgetComponent.GetUserWidgetObject` (`/Game/ThirdPersonBP/Blueprints/ThirdPersonCharacter.ScoreIncrease` PlayerHitting))))
        (set `/Game/ThirdPersonBP/Blueprints/UI/WBP_PlayerScoreIncrease.ScoreInt` (`self.GoldGain`) _aswbp_player_score_increase)
        (`/Game/ThirdPersonBP/Blueprints/UI/WBP_PlayerScoreIncrease.PlayAnimIncrease` _aswbp_player_score_increase)
        (`KismetSystemLibrary.Delay` 0.05)
        (bind _result (`/Engine/EditorBlueprintResources/StandardMacros.IncrementInt` (`self.timesHit`))
          (:`  `
            (`TextRenderComponent.K2_SetText` (`self.HeadbuttNumber`) (`KismetTextLibrary.Conv_IntToText` _result))
            (`self.AnimText`))))
      (:`then_1`
        (if (<= (`self.timesHit`) 0)
          (`self.TimerPinata`)
          (`LightComponent.SetIntensity` (`self.SpotLight`) 15000.0))))))

(event `AnimText`
  (bind _headbuttnumber (`self.HeadbuttNumber`))
  (bind (_direction _scaleadd) (`Timeline|TextReaction` :!via `PlayFromStart`)
    (:`Update`
      (`SceneComponent.SetRelativeScale3D` _headbuttnumber (+ (`SceneComponent.RelativeScale3D` _headbuttnumber) (`KismetMathLibrary.MakeVector` _scaleadd _scaleadd _scaleadd))))))

(event `TextSize`
  (bind _returnvalue (/ (`KismetMathLibrary.Conv_IntToDouble` (`self.timesHit`)) 2.0))
  (`SceneComponent.SetRelativeScale3D` (`self.HeadbuttNumber`) (+ (1.0 1.0 1.0) (`KismetMathLibrary.MakeVector` _returnvalue _returnvalue _returnvalue))))

(fn `UserConstructionScript`)