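; A player's sloop, the drop-off point that turns gold bags into coins and displays that player's wealth.
; BeginPlay finds the character whose LocalID matches PlayerIndex after a short delay.
; A gold bag entering the trigger pays that player, plays score feedback, is destroyed and prompts the spawner to refill below its cap.
; Tick shows a bag mesh while the player carries one and toggles treasure and light tiers against coin thresholds.
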(event `self.ReceiveBeginPlay`
  (set `self.AuthorizedGoldAug` "/Game/EveryoneProg/Deliveries/BP_GoldBag_WithGrab.BP_GoldBag_WithGrab_C")
  (`KismetSystemLibrary.Delay` 1.0)
  (bind _outactors (`GameplayStatics.GetAllActorsOfClass` "/Game/ThirdPersonBP/Blueprints/ThirdPersonCharacter.ThirdPersonCharacter_C"))
  (for _array_element _outactors
    (if (== (`/Game/ThirdPersonBP/Blueprints/ThirdPersonCharacter.LocalID` _array_element) (`self.PlayerIndex`))
      (set `self.PlayerRef` _array_element)
      (set `self.playerFound` true))))

(event `self.Trigger.OnComponentBeginOverlap`
  (params (OverlappedComponent :type "PrimitiveComponent Object Reference") (OtherActor :type "Actor Object Reference") (OtherComp :type "PrimitiveComponent Object Reference") (OtherBodyIndex :type Integer) (bFromSweep :type Boolean) (SweepResult :type "HitResult Structure (by ref)"))
  (if (== (`GameplayStatics.GetObjectClass` OtherActor) (`self.AuthorizedGoldAug`))
    (bind _outactors (`GameplayStatics.GetAllActorsOfClass` "/Game/ThirdPersonBP/Blueprints/ThirdPersonCharacter.ThirdPersonCharacter_C"))
    (for _array_element _outactors
      (if (== (`/Game/ThirdPersonBP/Blueprints/ThirdPersonCharacter.LocalID` _array_element) (`self.PlayerIndex`))
        (set `/Game/ThirdPersonBP/Blueprints/ThirdPersonCharacter.Coins` (+ (`/Game/ThirdPersonBP/Blueprints/ThirdPersonCharacter.Coins` _array_element) (`self.GoldBagGain`)) _array_element)
        (bind _aswbp_player_score_increase (cast `/Game/ThirdPersonBP/Blueprints/UI/WBP_PlayerScoreIncrease` (`WidgetComponent.GetUserWidgetObject` (`/Game/ThirdPersonBP/Blueprints/ThirdPersonCharacter.ScoreIncrease` _array_element))))
        (set `/Game/ThirdPersonBP/Blueprints/UI/WBP_PlayerScoreIncrease.ScoreInt` (`self.GoldBagGain`) _aswbp_player_score_increase)
        (`/Game/ThirdPersonBP/Blueprints/UI/WBP_PlayerScoreIncrease.PlayAnimIncrease` _aswbp_player_score_increase)
        (`GameplayStatics.PlaySound2D` "/Game/ArtAndMusic/Music/Bruitages/Service_validé.Service_validé" 1.0 1.0 0.0 null null)
        (`self.K2_DestroyActor` OtherActor)))
    (bind _outactors_2 (`GameplayStatics.GetAllActorsOfClass` (`self.AuthorizedGoldAug`)))
    (if (< (`KismetArrayLibrary.Array_Length` _outactors_2) (`/Game/EveryoneProg/Managers/BP_GoldBagSpawner.MaxBagAllowed` (`self.SpawnerBagRef`)))
      (`/Game/EveryoneProg/Managers/BP_GoldBagSpawner.SpawnBag` (`self.SpawnerBagRef`)))))

(event `self.ReceiveTick`
  (params (DeltaSeconds :type "Float (single-precision)"))
  (bind _playerref (`self.PlayerRef`))
  (bind _sm_item_bag_03 (`self.SM_Item_Bag_03`))
  (bind _carriedactor (`/Game/ThirdPersonBP/Blueprints/ThirdPersonCharacter.CarriedActor` _playerref))
  (if (`self.playerFound`)
    (`|ExecutionSequence`
      (:`then_0`
        (if (`/Game/ThirdPersonBP/Blueprints/ThirdPersonCharacter.IsCarrying` _playerref)
          (if (and (`KismetSystemLibrary.IsValid` _carriedactor) (== (`GameplayStatics.GetObjectClass` _carriedactor) "/Game/EveryoneProg/Deliveries/BP_GoldBag_WithGrab.BP_GoldBag_WithGrab_C"))
            (`SceneComponent.SetVisibility` _sm_item_bag_03 true true)
            (else
              (`SceneComponent.SetVisibility` _sm_item_bag_03 false true :!label _label)))
          (else
            (goto _label))))
      (:`then_1`
        (if (>= (`/Game/ThirdPersonBP/Blueprints/ThirdPersonCharacter.Coins` (`self.PlayerRef`)) (`self.RichestCheck`))
          (`SceneComponent.SetVisibility` (`self.Richest`) true true)
          (`SceneComponent.SetVisibility` (`self.RectLight3`) true true)
          (`SceneComponent.SetVisibility` (`self.SM_Item_Gem_02`) true true)
          (`SceneComponent.SetVisibility` (`self.SM_Item_Chalice_01`) true true)
          (`SceneComponent.SetVisibility` (`self.SM_Item_Gem_03`) true true)
          (`SceneComponent.SetVisibility` (`self.SM_Prop_TreasurePile_04`) true true)
          (`SceneComponent.SetVisibility` (`self.RichestGlint`) true true)
          (`SceneComponent.SetVisibility` (`self.SM_Prop_TreasurePile_05`) true true)
          (else
            (`SceneComponent.SetVisibility` (`self.Richest`) false true)
            (`SceneComponent.SetVisibility` (`self.RectLight3`) false true)
            (`SceneComponent.SetVisibility` (`self.SM_Item_Gem_02`) false true)
            (`SceneComponent.SetVisibility` (`self.SM_Item_Chalice_01`) false true)
            (`SceneComponent.SetVisibility` (`self.SM_Item_Gem_03`) false true)
            (`SceneComponent.SetVisibility` (`self.SM_Prop_TreasurePile_04`) false true)
            (`SceneComponent.SetVisibility` (`self.RichestGlint`) false true)
            (`SceneComponent.SetVisibility` (`self.SM_Prop_TreasurePile_05`) false true)
            (if (>= (`/Game/ThirdPersonBP/Blueprints/ThirdPersonCharacter.Coins` (`self.PlayerRef`)) (`self.RichCheck`))
              (`SceneComponent.SetVisibility` (`self.Rich`) true true)
              (`SceneComponent.SetVisibility` (`self.SM_Prop_Sack_04`) true true)
              (`SceneComponent.SetVisibility` (`self.SM_Prop_TreasurePile_03`) true true)
              (`SceneComponent.SetVisibility` (`self.SM_Wep_Pistol_DoubleBarrel_01`) true true)
              (`SceneComponent.SetVisibility` (`self.SM_Wep_Cutlass_02_Sheath`) true true)
              (`SceneComponent.SetVisibility` (`self.SM_Wep_Cutlass_02`) true true)
              (`SceneComponent.SetVisibility` (`self.SM_Prop_Lantern_01`) true true)
              (`SceneComponent.SetVisibility` (`self.RectLight2`) true true)
              (else
                (`SceneComponent.SetVisibility` (`self.Rich`) false true)
                (`SceneComponent.SetVisibility` (`self.SM_Prop_Sack_04`) false true)
                (`SceneComponent.SetVisibility` (`self.SM_Prop_TreasurePile_03`) false true)
                (`SceneComponent.SetVisibility` (`self.SM_Wep_Pistol_DoubleBarrel_01`) false true)
                (`SceneComponent.SetVisibility` (`self.SM_Wep_Cutlass_02_Sheath`) false true)
                (`SceneComponent.SetVisibility` (`self.SM_Wep_Cutlass_02`) false true)
                (`SceneComponent.SetVisibility` (`self.SM_Prop_Lantern_01`) false true)
                (`SceneComponent.SetVisibility` (`self.RectLight2`) false true)
                (if (>= (`/Game/ThirdPersonBP/Blueprints/ThirdPersonCharacter.Coins` (`self.PlayerRef`)) (`self.JustPoorCheck`))
                  (`SceneComponent.SetVisibility` (`self.JustPoor`) true false)
                  (`SceneComponent.SetVisibility` (`self.StaticMesh`) true false)
                  (`SceneComponent.SetVisibility` (`self.StaticMesh15`) true false)
                  (`SceneComponent.SetVisibility` (`self.StaticMesh12`) true false)
                  (`SceneComponent.SetVisibility` (`self.SM_Prop_Chest_Treasure_03`) true false)
                  (`SceneComponent.SetVisibility` (`self.SM_Prop_Crate_02`) true false)
                  (`SceneComponent.SetVisibility` (`self.StaticMesh13`) true false)
                  (`SceneComponent.SetVisibility` (`self.StaticMesh14`) true false)
                  (`SceneComponent.SetVisibility` (`self.StaticMesh11`) true false)
                  (`SceneComponent.SetVisibility` (`self.SM_Prop_TreasurePile_01`) true false)
                  (`SceneComponent.SetVisibility` (`self.RectLight1`) true false)
                  (else
                    (`SceneComponent.SetVisibility` (`self.JustPoor`) false false)
                    (`SceneComponent.SetVisibility` (`self.StaticMesh`) false false)
                    (`SceneComponent.SetVisibility` (`self.StaticMesh15`) false false)
                    (`SceneComponent.SetVisibility` (`self.StaticMesh12`) false false)
                    (`SceneComponent.SetVisibility` (`self.SM_Prop_Chest_Treasure_03`) false false)
                    (`SceneComponent.SetVisibility` (`self.SM_Prop_Crate_02`) false false)
                    (`SceneComponent.SetVisibility` (`self.StaticMesh13`) false false)
                    (`SceneComponent.SetVisibility` (`self.StaticMesh14`) false false)
                    (`SceneComponent.SetVisibility` (`self.StaticMesh11`) false false)
                    (`SceneComponent.SetVisibility` (`self.SM_Prop_TreasurePile_01`) false false)
                    (`SceneComponent.SetVisibility` (`self.RectLight1`) false false)
                    (if (>= (`/Game/ThirdPersonBP/Blueprints/ThirdPersonCharacter.Coins` (`self.PlayerRef`)) (`self.DirtPoorCheck`))
                      (`/Engine/EditorBlueprintResources/StandardMacros.DoOnce` false :!label _label_2
                        (:`Completed`
                          (`SceneComponent.SetVisibility` (`self.DirtPoorVis`) true false)
                          (`SceneComponent.SetVisibility` (`self.StaticMesh5`) true false)
                          (`SceneComponent.SetVisibility` (`self.StaticMesh2`) true false)
                          (`SceneComponent.SetVisibility` (`self.StaticMesh3`) true false)
                          (`SceneComponent.SetVisibility` (`self.StaticMesh4`) true false)
                          (`SceneComponent.SetVisibility` (`self.StaticMesh1`) true false)
                          (`SceneComponent.SetVisibility` (`self.StaticMesh6`) true false)
                          (`SceneComponent.SetVisibility` (`self.StaticMesh7`) true false)
                          (`SceneComponent.SetVisibility` (`self.StaticMesh8`) true false)
                          (`SceneComponent.SetVisibility` (`self.RectLight`) true false)
                          (goto _label_3 :!via `Reset`)))
                      (else
                        (`/Engine/EditorBlueprintResources/StandardMacros.DoOnce` false :!label _label_3
                          (:`Completed`
                            (`SceneComponent.SetVisibility` (`self.DirtPoorVis`) false false)
                            (`SceneComponent.SetVisibility` (`self.StaticMesh5`) false false)
                            (`SceneComponent.SetVisibility` (`self.StaticMesh2`) false false)
                            (`SceneComponent.SetVisibility` (`self.StaticMesh3`) false false)
                            (`SceneComponent.SetVisibility` (`self.StaticMesh4`) false false)
                            (`SceneComponent.SetVisibility` (`self.StaticMesh1`) false false)
                            (`SceneComponent.SetVisibility` (`self.StaticMesh6`) false false)
                            (`SceneComponent.SetVisibility` (`self.StaticMesh7`) false false)
                            (`SceneComponent.SetVisibility` (`self.StaticMesh8`) false false)
                            (`SceneComponent.SetVisibility` (`self.RectLight`) false false)
                            (goto _label_2 :!via `Reset`)))))))))))))))

(fn `UserConstructionScript`)