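; Treasure tree that, after a timed delay, plays a scale-wiggle timeline and spawns a BP_CoinSpawner at its middle spawn point.
; Tick drives that spawn through DoOnce gates and, outside two-player mode, toggles a billboard from character overlap with the headbutt volume.
; A hit on a loaded tree outside two-player mode fades in audio, briefly disables Box collision and clears the spawned flag, restarting the cycle.
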(event `PlayTimelineTreasure`
  (bind (_relativescale3d_x _relativescale3d_y _relativescale3d_z) (`KismetMathLibrary.BreakVector` (`SceneComponent.RelativeScale3D` (`self.BaseTree`))))
  (`TimelineComponent.SetPlayRate` (`self.TreeReceiveTreasure`) 2.0)
  (bind (_direction _alpha _wiggletree) (`Timeline|TreeReceiveTreasure` :!via `PlayFromStart`)
    (:`Update`
      (set `self.Alpha` _alpha)
      (`SceneComponent.SetRelativeScale3D` (`self.BaseTree`) (`KismetMathLibrary.MakeVector` (`KismetMathLibrary.Lerp` _relativescale3d_x _wiggletree (`self.Alpha`)) (`KismetMathLibrary.Lerp` _relativescale3d_y _wiggletree (`self.Alpha`)) (`KismetMathLibrary.Lerp` _relativescale3d_z _wiggletree (`self.Alpha`)))))))

(event `self.ReceiveBeginPlay`
  (`AudioComponent.SetSound` (`self.Audio`) "/Game/ArtAndMusic/Music/SoundsWreckedShip/Treasure_Tree.Treasure_Tree"))

(event `self.ReceiveTick`
  (params (DeltaSeconds :type "Float (single-precision)"))
  (bind _billboard (`self.Billboard`))
  ;[1 1 1] ça fait peur, mais c'est facile !
  ;
  ; On réplique trois fois un Spawn Actor pour setter correctement les objets, et pouvoir les faire bouger avec les Timelines, tout simplement.
  (if (`self.ObjectsSpawned`)
    (if (`self.2Players?`)
      _
      (elif (> (`KismetArrayLibrary.Array_Length` (`PrimitiveComponent.GetOverlappingActors` (`self.HeadbuttVis`) "/Game/ThirdPersonBP/Blueprints/ThirdPersonCharacter.ThirdPersonCharacter_C")) 0)
        (`/Engine/EditorBlueprintResources/StandardMacros.DoOnce` false :!label _label
          (:`Completed`
            (`SceneComponent.SetHiddenInGame` _billboard false false)
            (goto _label_2 :!via `Reset`)))
        (else
          (`/Engine/EditorBlueprintResources/StandardMacros.DoOnce` false :!label _label_2
            (:`Completed`
              (`SceneComponent.SetHiddenInGame` _billboard true false)
              (goto _label :!via `Reset`))))))
    (else
      (`/Engine/EditorBlueprintResources/StandardMacros.DoOnce` false :!label _label_3
        (:`Completed`
          (`KismetSystemLibrary.Delay` (`self.TimerSpawn`))
          (`self.PlayTimelineTreasure`)
          (`|SpawnActorFromClass` "/Game/EveryoneProg/Managers/BP_CoinSpawner.BP_CoinSpawner_C" (`KismetMathLibrary.MakeTransform` (`SceneComponent.K2_GetComponentLocation` (`self.SpawnTreasureMid`)) (struct) (1.05 1.05 1.05)) "AdjustIfPossibleButAlwaysSpawn" "OverrideRootScale" null (`self.Box Size`) (`self.Wait Spawn`) (`self.Min Coin Spawn`) (`self.Max Coin Spawn`) (`self.Give Random Value`) (`self.Spawn Once Only`) null)
          (set `self.ObjectsSpawned` true)
          (goto _label_3 :!via `Reset`))))))

(event `/Game/EveryoneProg/BPI_Interact.GotHit`
  (params (PlayerHitting :type "/Game/ThirdPersonBP/Blueprints/ThirdPersonCharacter Object Reference"))
  ;[1 1 1] ça marche pas encore, dur dur de faire bouger des objets hors de leur propre Blueprint!
  (if (`self.ObjectsSpawned`)
    (if (not (`self.2Players?`))
      (`self.FreeTreasures`))))

(event `FreeTreasures`
  ;[1 1 1] ça marche pas encore, dur dur de faire bouger des objets hors de leur propre Blueprint!
  (`/Engine/EditorBlueprintResources/StandardMacros.DoOnce` false :!label _label_4
    (:`Completed`
      (`AudioComponent.FadeIn` (`self.Audio`) 1.0 1.0 0.0 "Linear")
      (`PrimitiveComponent.SetCollisionEnabled` (`self.Box`) "NoCollision")
      (`KismetSystemLibrary.Delay` 1.0)
      (`PrimitiveComponent.SetCollisionEnabled` (`self.Box`) "QueryAndPhysics")
      (set `self.ObjectsSpawned` false)
      (goto _label_4 :!via `Reset`))))

(fn `UserConstructionScript`)