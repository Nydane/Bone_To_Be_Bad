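; BP_IntroSloop is the intro sloop, which shows an item bag mesh while any intro gold bag is carried.
; On BeginPlay it sets both player light particle components to a grey fire-head effect.
; Tick runs a DoOnce and short Delay as a throttled poll of the gold bag array, counting carried bags and removing invalid entries mid-loop.
; That count toggles the bag mesh's visibility, then resets for the next pass.
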(event `self.ReceiveBeginPlay`
  (`ParticleSystemComponent.SetTemplate` (`self.LightPlayer1`) "/Game/PolygonPack/PolygonPirates/ParticleFX/HeadThrowPlayer/P_FX_FireHeadGrey.P_FX_FireHeadGrey")
  (`ParticleSystemComponent.SetTemplate` (`self.LightPlayer`) "/Game/PolygonPack/PolygonPirates/ParticleFX/HeadThrowPlayer/P_FX_FireHeadGrey.P_FX_FireHeadGrey"))

(event `self.ReceiveTick`
  (params (DeltaSeconds :type "Float (single-precision)"))
  (bind _sm_item_bag_03 (`self.SM_Item_Bag_03`))
  (`/Engine/EditorBlueprintResources/StandardMacros.DoOnce` false :!label _label
    (:`Completed`
      (`KismetSystemLibrary.Delay` 0.06)
      (for _array_element (`self.IntroGoldBagArray`)
        (if (`KismetSystemLibrary.IsValid` _array_element)
          (if (`/Game/EveryoneProg/Deliveries/BP_GoldBag_WithGrab.isCarried` _array_element)
            (`/Engine/EditorBlueprintResources/StandardMacros.IncrementInt` (`self.BagsCarried`)))
          (else
            (`KismetArrayLibrary.Array_RemoveItem` (`self.IntroGoldBagArray`) _array_element))))
      (if (>= (`self.BagsCarried`) 1)
        (`SceneComponent.SetVisibility` _sm_item_bag_03 true true)
        (else
          (`SceneComponent.SetVisibility` _sm_item_bag_03 false true)))
      (set `self.BagsCarried` 0)
      (goto _label :!via `Reset`))))

(fn `UserConstructionScript`)