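; PvE event raft that travels along a spline while handing out treasure to players, then destroys itself at the end.
; A timeline scaled by Duration moves it along the SplineManager spline; Tick detects arrival and ends the event message on the EventVis-tagged actor.
; Overlapping characters in the required state receive coins through a DoOnce cooldown with a particle burst.
; Each grant shrinks the gold pile mesh until it hides and the light fades.
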(event `self.ReceiveBeginPlay`
  (bind _audio (`self.Audio`))
  (if (`self.CanMove`)
    (`AudioComponent.SetSound` _audio "/Game/ArtAndMusic/Music/SoundsWreckedShip/Moving_Raft__annonce_.Moving_Raft__annonce_")
    (`AudioComponent.FadeIn` _audio 0.0 1.0 0.0 "Linear")
    (`self.MoveRaft`)))

(event `MoveRaft`
  (bind _returnvalue (`KismetMathLibrary.Lerp` 0.0 (`SplineComponent.GetSplineLength` (`/Game/EveryoneProg/Ships/SplineManager.Spline` (`self.SplineManager`))) (`self.Alpha`)))
  ;[1 1 1] Gère seulement le mouvement du Raft, il faudra ajouter d'autres CE ou passer par l'Event Tick pour les autres Behaviours.
  (`TimelineComponent.SetPlayRate` (`self.Movement`) (/ 1.0 (`self.Duration`)))
  (bind (_direction _alpha) (`Timeline|Movement`)
    (:`Update`
      (set `self.Alpha` _alpha)
      (`self.K2_SetActorLocationAndRotation` (`SplineComponent.GetLocationAtDistanceAlongSpline` (`/Game/EveryoneProg/Ships/SplineManager.Spline` (`self.SplineManager`)) _returnvalue "World") (`SplineComponent.GetRotationAtDistanceAlongSpline` (`/Game/EveryoneProg/Ships/SplineManager.Spline` (`self.SplineManager`)) _returnvalue "World")))
    (:`Finished`
      (set `self.CanMove` false))))

(event `self.ReceiveTick`
  (params (DeltaSeconds :type "Float (single-precision)"))
  (if (`KismetMathLibrary.NearlyEqual_FloatFloat` (`self.Alpha`) 1.0 0.01)
    (bind _outactors (`GameplayStatics.GetAllActorsWithTag` "EventVis"))
    (message `/Game/EveryoneProg/BPI_Interact.EndEvent` (`|GetArrayItem` _outactors))
    (`KismetSystemLibrary.Delay` 0.2)
    (`self.K2_DestroyActor`)))

(event `self.TreasureGiver.OnComponentBeginOverlap`
  (params (OverlappedComponent :type "PrimitiveComponent Object Reference") (OtherActor :type "Actor Object Reference") (OtherComp :type "PrimitiveComponent Object Reference") (OtherBodyIndex :type Integer) (bFromSweep :type Boolean) (SweepResult :type "HitResult Structure (by ref)"))
  (if (== (`GameplayStatics.GetObjectClass` OtherActor) "/Game/ThirdPersonBP/Blueprints/ThirdPersonCharacter.ThirdPersonCharacter_C")
    (if (> (`self.GiveTreasuresNumber`) 0)
      (`/Engine/EditorBlueprintResources/StandardMacros.DoOnce` false :!label _label
        (:`Completed`
          (bind _asthird_person_character (cast `/Game/ThirdPersonBP/Blueprints/ThirdPersonCharacter` OtherActor))
          (if (`|EnumEquality` (`/Game/ThirdPersonBP/Blueprints/ThirdPersonCharacter.CurrentState` _asthird_person_character) "NewEnumerator0")
            (`|ExecutionSequence`
              (:`then_0`
                (set `/Game/ThirdPersonBP/Blueprints/ThirdPersonCharacter.Coins` (+ (`/Game/ThirdPersonBP/Blueprints/ThirdPersonCharacter.Coins` _asthird_person_character) (`self.NumberCoinsToGive`)) _asthird_person_character)
                (bind _aswbp_player_score_increase (cast `/Game/ThirdPersonBP/Blueprints/UI/WBP_PlayerScoreIncrease` (`WidgetComponent.GetUserWidgetObject` (`/Game/ThirdPersonBP/Blueprints/ThirdPersonCharacter.ScoreIncrease` _asthird_person_character))))
                (set `/Game/ThirdPersonBP/Blueprints/UI/WBP_PlayerScoreIncrease.ScoreInt` (`self.NumberCoinsToGive`) _aswbp_player_score_increase)
                (`/Engine/EditorBlueprintResources/StandardMacros.DecrementInt` (`self.GiveTreasuresNumber`)))
              (:`then_1`
                (set `ParticleSystemComponent.CustomTimeDilation` 2.0 (`self.ParticleSystem`))
                (`self.ChangeGoldPile`)
                (`KismetSystemLibrary.Delay` 0.4)
                (set `ParticleSystemComponent.CustomTimeDilation` 0.15 (`self.ParticleSystem`))
                (`KismetSystemLibrary.Delay` 1.6)
                (goto _label :!via `Reset`)))))))))

(event `ChangeGoldPile`
  (bind _goldpile (`self.GoldPile`))
  (bind _goldpile_2 (`self.GoldPile`))
  (switch `int` (`self.GiveTreasuresNumber`)
    (:`0`
      (`SceneComponent.SetVisibility` _goldpile false false)
      (`ActorComponent.Deactivate` (`self.ParticleSystem`))
      (bind (_direction _alpha) (`Timeline|TurnOffLight`)
        (:`Update`
          (bind _output_get (set `self.AlphaIntensity` _alpha))
          (`LightComponent.SetIntensity` (`self.RectLight`) (`KismetMathLibrary.Lerp` (`LightComponentBase.Intensity` (`self.RectLight`)) 0.0 _output_get)))))
    (:`1`
      (`StaticMeshComponent.SetStaticMesh` _goldpile "/Game/PolygonPack/PolygonPirates/Meshes/Props/SM_Prop_TreasurePile_01.SM_Prop_TreasurePile_01"))
    (:`2`
      (`StaticMeshComponent.SetStaticMesh` _goldpile_2 "/Game/PolygonPack/PolygonPirates/Meshes/Props/SM_Prop_TreasurePile_02.SM_Prop_TreasurePile_02"))
    (:`3`
      (`StaticMeshComponent.SetStaticMesh` _goldpile_2 "/Game/PolygonPack/PolygonPirates/Meshes/Props/SM_Prop_TreasurePile_03.SM_Prop_TreasurePile_03"))))

(fn `UserConstructionScript`)