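; Ship-damaging cannon that fires when hit while loaded, with muzzle particles, recoil and lever timelines.
; A DoOnce blocks refiring until recoil finishes, while Tick shows the lit wick and plays the lever whenever loaded.
; Firing sphere-traces for Vehicle objects and takes one Health from a Civil, Merchant, War or Ghost ship through chained class checks.
; An unconnected multi-trace for gathering ship distances never runs.
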(event `/Game/EveryoneProg/BPI_Interact.GotHit`
  (params (PlayerHitting :type "/Game/ThirdPersonBP/Blueprints/ThirdPersonCharacter Object Reference"))
  (if (`self.isLoaded`)
    (`/Engine/EditorBlueprintResources/StandardMacros.DoOnce` false :!label _label
      (:`Completed`
        (set `self.Firing` true)
        (`self.TraceForShips`)
        (`GameplayStatics.SpawnEmitterAttached` "/Game/PolygonPack/PolygonPirates/ParticleFX/P_FX_Cannon_Fire.P_FX_Cannon_Fire" (`self.CannonShot`) "None" (0.0 0.0 0.0) (struct :`Yaw` 90.0))
        (`|ExecutionSequence`
          (:`then_0`
            (bind (_direction _recoildistance) (`Timeline|Recoil` :!via `PlayFromStart`)
              (:`Update`
                (`SceneComponent.K2_SetRelativeLocation` (`self.Cannon`) (`KismetMathLibrary.VLerp` (`self.StartLoc`) (`self.RecoilLoc`) _recoildistance) false false)
                (`SceneComponent.SetHiddenInGame` (`self.WickLitFire`) true true)
                (set `self.isLoaded` false))
              (:`Finished`
                (set `self.Firing` false)
                (goto _label :!via `Reset`))))
          (:`then_1`
            (bind (_direction_2 _lever) (`Timeline|Lever` :!via `ReverseFromEnd` :!label _label_2)
              (:`Update`
                (`SceneComponent.K2_SetRelativeRotation` (`self.FiringLever`) (`KismetMathLibrary.RLerp` (`self.LeverUnloadedRot`) (`self.LeverLoadedRot`) _lever) false false)))))))))

(event `self.ReceiveBeginPlay`)

(event `self.ReceiveTick`
  (params (DeltaSeconds :type "Float (single-precision)"))
  (if (`self.isLoaded`)
    (`SceneComponent.SetHiddenInGame` (`self.WickLitFire`) false true)
    (goto _label_2)))

(event `TraceForShips`
  ;[1 1 1] OH MY GOD I'M SO SORRY
  (bind _outhit (`KismetSystemLibrary.SphereTraceSingleForObjects` :`Start` (`SceneComponent.K2_GetComponentLocation` (`self.OriginTraceSphere`)) :`End` (`SceneComponent.K2_GetComponentLocation` (`self.EndTraceSphere`)) :`Radius` 1500.0 :`ObjectTypes` (`|MakeArray` "ObjectTypeQuery5" :!type "EObjectTypeQuery Enum") :`DrawDebugType` "ForDuration"))
  (if (== (`GameplayStatics.GetObjectClass` (`.HitActor` (`GameplayStatics.BreakHitResult` _outhit))) "/Game/EveryoneProg/Ships/BP_Ship_Civil.BP_Ship_Civil_C")
    (bind _asbp_ship_civil (cast `/Game/EveryoneProg/Ships/BP_Ship_Civil` (`.HitActor` (`GameplayStatics.BreakHitResult` _outhit))))
    (`/Engine/EditorBlueprintResources/StandardMacros.DecrementInt` (`/Game/EveryoneProg/Ships/BP_BasicShip.Health` _asbp_ship_civil))
    (elif (== (`GameplayStatics.GetObjectClass` (`.HitActor` (`GameplayStatics.BreakHitResult` _outhit))) "/Game/EveryoneProg/Ships/BP_Ship_Merchant.BP_Ship_Merchant_C")
      (bind _asbp_ship_merchant (cast `/Game/EveryoneProg/Ships/BP_Ship_Merchant` (`.HitActor` (`GameplayStatics.BreakHitResult` _outhit))))
      (`/Engine/EditorBlueprintResources/StandardMacros.DecrementInt` (`/Game/EveryoneProg/Ships/BP_BasicShip.Health` _asbp_ship_merchant))
      (elif (== (`GameplayStatics.GetObjectClass` (`.HitActor` (`GameplayStatics.BreakHitResult` _outhit))) "/Game/EveryoneProg/Ships/BP_Ship_War.BP_Ship_War_C")
        (bind _asbp_ship_war (cast `/Game/EveryoneProg/Ships/BP_Ship_War` (`.HitActor` (`GameplayStatics.BreakHitResult` _outhit))))
        (`/Engine/EditorBlueprintResources/StandardMacros.DecrementInt` (`/Game/EveryoneProg/Ships/BP_BasicShip.Health` _asbp_ship_war))
        (elif (== (`GameplayStatics.GetObjectClass` (`.HitActor` (`GameplayStatics.BreakHitResult` _outhit))) "/Game/EveryoneProg/Ships/BP_Ship_Ghost.BP_Ship_Ghost_C")
          (bind _asbp_ship_ghost (cast `/Game/EveryoneProg/Ships/BP_Ship_Ghost` (`.HitActor` (`GameplayStatics.BreakHitResult` _outhit))))
          (`/Engine/EditorBlueprintResources/StandardMacros.DecrementInt` (`/Game/EveryoneProg/Ships/BP_BasicShip.Health` _asbp_ship_ghost)))))))

(fn `UserConstructionScript`)