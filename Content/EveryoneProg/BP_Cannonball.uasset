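; Carryable cannonball that players grab and load into a BP_Cannon, destroying itself when carried into the trigger of an unloaded cannon.
; Tick polls the attach parent: while carried it follows the character's GrabLocation with physics off and a tag preventing theft.
; On release it detaches, restores physics and usually the carrier's walk speed.
; Tick also toggles a grab-button sprite for nearby characters; the sprite-alternating ChangeButton event is never called.
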(event `ChangeButton`
  (bind _grabvis (`self.GrabVis`))
  (`/Engine/EditorBlueprintResources/StandardMacros.DoOnce` false :!label _label
    (:`Completed`
      (`KismetSystemLibrary.Delay` 1.5)
      (`/Engine/EditorBlueprintResources/StandardMacros.FlipFlop`
        (:`A`
          (`BillboardComponent.SetSprite` _grabvis "/Game/Menus/Assets/XboxOne_B.XboxOne_B")
          (goto _label :!via `Reset`))
        (:`B`
          (`BillboardComponent.SetSprite` _grabvis "/Game/ArtAndMusic/Art/Y_Button_NEW.Y_Button_NEW")
          (goto _label :!via `Reset`))))))

(event `self.ReceiveActorBeginOverlap`
  (params (OtherActor :type "Actor Object Reference"))
  (if (== (`GameplayStatics.GetObjectClass` OtherActor) (`self.CannonVar`))
    (bind _asbp_cannon (cast `/Game/EveryoneProg/BP_Cannon` OtherActor))
    (if (`/Game/EveryoneProg/BP_Cannon.isLoaded` _asbp_cannon)
      _
      (elif (`PrimitiveComponent.IsOverlappingActor` (`/Game/EveryoneProg/BP_Cannon.Boulet_Trigger` _asbp_cannon) self)
        (if (`self.isCarried`)
          (set `/Game/EveryoneProg/BP_Cannon.isLoaded` true _asbp_cannon)
          (`self.K2_DestroyActor` self))))))

(event `self.ReceiveBeginPlay`)

(event `self.ReceiveTick`
  (params (DeltaSeconds :type "Float (single-precision)"))
  (bind _grabvis (`self.GrabVis`))
  (bind _cannonball (`self.Cannonball`))
  (bind _cannonball_2 (`self.Cannonball`))
  (`|ExecutionSequence`
    (:`then_0`
      (if (== (`GameplayStatics.GetObjectClass` (`self.GetAttachParentActor` self)) "/Game/ThirdPersonBP/Blueprints/ThirdPersonCharacter.ThirdPersonCharacter_C")
        (`PrimitiveComponent.SetCollisionEnabled` (`self.TriggerGrabVis`) "NoCollision")
        (bind _asthird_person_character (cast `/Game/ThirdPersonBP/Blueprints/ThirdPersonCharacter` (`self.GetAttachParentActor` self)))
        (if (`/Game/ThirdPersonBP/Blueprints/ThirdPersonCharacter.IsCarrying` _asthird_person_character)
          (set `self.Carrier` _asthird_person_character)
          (`SceneComponent.K2_SetWorldLocation` (`self.Cannonball`) (`SceneComponent.K2_GetComponentLocation` (`/Game/ThirdPersonBP/Blueprints/ThirdPersonCharacter.GrabLocation` _asthird_person_character)) false true)
          (if (`KismetSystemLibrary.IsValid` self)
            (`PrimitiveComponent.SetConstraintMode` (`self.Cannonball`) "XYPlane")
            ;[1 1 1] This Tag allows us to make sure that the object cannot be "stolen" simply by pressing the Grab Button.
            (`/Engine/EditorBlueprintResources/StandardMacros.DoOnce` false :!label _label_2
              (:`Completed`
                (`PrimitiveComponent.SetCollisionEnabled` _cannonball "NoCollision")
                (`PrimitiveComponent.SetSimulatePhysics` _cannonball false)
                (`KismetArrayLibrary.Array_AddUnique` (`self.Tags`) (`self.CarriedTag`))
                (set `self.isCarried` true)
                (goto _label_3 :!via `Reset`))))
          (else
            ;[1 1 1] A terme, détruire le Seau !
            (`SceneComponent.K2_DetachFromComponent` (`self.Cannonball`) "KeepWorld" "KeepWorld" "KeepWorld" true)
            (`SceneComponent.K2_DetachFromComponent` (`self.RootComponent`) "KeepWorld" "KeepWorld" "KeepWorld" true)
            (`PrimitiveComponent.SetConstraintMode` (`self.Cannonball`) "Default")
            (bind _asthird_person_character_2 (cast `/Game/ThirdPersonBP/Blueprints/ThirdPersonCharacter` (`self.Carrier`)))
            (if (not (`|EnumEquality` (`/Game/ThirdPersonBP/Blueprints/ThirdPersonCharacter.CurrentState` _asthird_person_character_2) "NewEnumerator2"))
              (set `CharacterMovementComponent.MaxWalkSpeed` (`/Game/ThirdPersonBP/Blueprints/ThirdPersonCharacter.BaseWalkSpeed` _asthird_person_character_2) (`Character.CharacterMovement` _asthird_person_character_2)))
            (`KismetSystemLibrary.Delay` 0.1)
            (set `self.Carrier` (`self.CarrierNone`))
            (`/Engine/EditorBlueprintResources/StandardMacros.DoOnce` false :!label _label_3
              (:`Completed`
                (`PrimitiveComponent.SetCollisionEnabled` _cannonball_2 "QueryAndPhysics")
                (`PrimitiveComponent.SetSimulatePhysics` _cannonball_2 true)
                (`KismetArrayLibrary.Array_RemoveItem` (`self.Tags`) (`self.CarriedTag`))
                (set `self.isCarried` false)
                (goto _label_2 :!via `Reset`)))))
        (else
          (`PrimitiveComponent.SetCollisionEnabled` (`self.TriggerGrabVis`) "QueryOnly"))))
    (:`then_1`
      (if (`KismetSystemLibrary.IsValid` self)
        (if (>= (`KismetArrayLibrary.Array_Length` (`PrimitiveComponent.GetOverlappingActors` (`self.TriggerGrabVis`) "/Game/ThirdPersonBP/Blueprints/ThirdPersonCharacter.ThirdPersonCharacter_C")) 1)
          (`/Engine/EditorBlueprintResources/StandardMacros.DoOnce` false :!label _label_4
            (:`Completed`
              (`SceneComponent.SetHiddenInGame` _grabvis false false)
              (goto _label_5 :!via `Reset`)))
          (else
            (`/Engine/EditorBlueprintResources/StandardMacros.DoOnce` false :!label _label_5
              (:`Completed`
                (`SceneComponent.SetHiddenInGame` _grabvis true false)
                (goto _label_4 :!via `Reset`)))))))))

(fn `UserConstructionScript`)