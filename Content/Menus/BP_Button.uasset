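; BP_Button is a menu button that keeps its visual style in sync with mouse hover and keyboard focus.
; Start sets a fast looping timer on Check Focus, a makeshift Tick because the button has no tick event.
; Check Focus gives a hovered button keyboard focus and the mouse style, otherwise choosing the key-selected or unselected style based on focus.
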(fn `Check Focus`
  ;[1 1 1] Check si la souris est sur un bouton
  (if (`self.IsHovered`)
    ;[1 1 1] si Oui, on utilise le mouse style
    (`self.SetKeyboardFocus`)
    (`self.SetStyle` (`self.MouseStyle`))
    (else
      ;[1 1 1] Si non, on utilise le keyselected style, en regardant si une touche est select ou pas
      (`self.SetStyle` (select `bool` (`self.HasKeyboardFocus`) :`false` (`self.KeyNotSelected`) :`true` (`self.KeySelected`))))))

(fn `Start`
  ;[1 1 1] un 'Event Tick' de fortune car on ne peut pas mettre de tick dans un bouton
  (`KismetSystemLibrary.K2_SetTimer` self "Check Focus" 0.06 true))