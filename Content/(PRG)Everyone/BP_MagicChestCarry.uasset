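; Magic chest that players carry by front and back handles, paying coins out of its gold to both carriers at intervals while two hold it.
; Tick snaps handles to each carrier's grab point and lerps the chest between them, releasing handles when carrying stops.
; Walk speed is adjusted by carrier separation, or cut for a lone carrier.
; Once gold runs out, the chest shrinks, dims its lights, spawns an effect and destroys itself.
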(event `self.ReceiveBeginPlay`
  ;[1 1 1] Setting up everything needed on Begin Play
  (set `self.Tags` (`|MakeArray` "Sell" :!type "Name"))
  (set `ActorComponent.ComponentTags` (`|MakeArray` "CarryFront" :!type "Name") (`self.HandleConstraintFront`))
  (set `ActorComponent.ComponentTags` (`|MakeArray` "CarryBack" :!type "Name") (`self.HandleConstraintBack`))
  (`CableComponent.SetAttachEndToComponent` (`self.CableFront`) (`self.HandleConstraintFront`) "None")
  (`CableComponent.SetAttachEndToComponent` (`self.CableBack`) (`self.HandleConstraintBack`) "None")
  (bind _outactors (`GameplayStatics.GetAllActorsOfClass` "/Game/(PRG)Everyone/BP_MagicChestPinata.BP_MagicChestPinata_C"))
  (set `self.MagicChestRef` (`|GetArrayItem` _outactors)))

(event `self.ReceiveTick`
  (params (DeltaSeconds :type "Float (single-precision)"))
  ;[1 1 1 1 123] Promis je commente plus tard, pas taper s'il vous plait !
  (`|ExecutionSequence`
    (:`then_0`
      (if (== (`KismetArrayLibrary.Array_Length` (`self.Carriers`)) 2)
        (set `self.PreviousLocationChest` (`SceneComponent.K2_GetComponentLocation` (`self.ChestBot`)))
        (bind _returnvalue (`GameplayStatics.GetActorArrayAverageLocation` (`self.Carriers`)))
        (`SceneComponent.K2_AddRelativeLocation` (`self.ChestBot`) (`KismetMathLibrary.MakeVector` (.x (`KismetMathLibrary.GetVectorArrayAverage` (`|MakeArray` (`SceneComponent.K2_GetComponentLocation` (`self.HandleConstraintBack`)) (`SceneComponent.K2_GetComponentLocation` (`self.HandleConstraintFront`))))) (+ (.y (`KismetMathLibrary.GetVectorArrayAverage` (`|MakeArray` (`SceneComponent.K2_GetComponentLocation` (`self.HandleConstraintBack`)) (`SceneComponent.K2_GetComponentLocation` (`self.HandleConstraintFront`))))) 200.0) (.z (`KismetMathLibrary.GetVectorArrayAverage` (`|MakeArray` (`SceneComponent.K2_GetComponentLocation` (`self.HandleConstraintBack`)) (`SceneComponent.K2_GetComponentLocation` (`self.HandleConstraintFront`)))))) false false)
        (`SceneComponent.K2_SetWorldLocation` (`self.ChestBot`) (`KismetMathLibrary.VLerp` (`self.PreviousLocationChest`) _returnvalue 0.3) false false)
        (for (_array_element _array_index) (`self.Carriers`)
          (set `self.Referent` _array_element)
          (for _index (range (+ _array_index 1) (`KismetArrayLibrary.Array_Length` (`self.Carriers`)))
            (`KismetArrayLibrary.Array_Add` (`self.Distance`) (`self.GetDistanceTo` (`self.Referent`) (`|GetArrayItem` (`self.Carriers`) _index)))))
        (bind _result (`/Engine/EditorBlueprintResources/StandardMacros.NegateFloat` (`KismetMathLibrary.FClamp` (`.MaxValue` (`KismetMathLibrary.MaxOfFloatArray` (`self.Distance`))) (`self.MinSpeedLost`) (`self.MaxSpeedLost`)))
          (:`  `
            (`|ExecutionSequence`
              (:`then_0`
                (bind _asthird_person_character (cast `/Game/ThirdPersonBP/Blueprints/ThirdPersonCharacter` (`self.BackCarrier`)))
                (set `CharacterMovementComponent.MaxWalkSpeed` (+ (`/Game/ThirdPersonBP/Blueprints/ThirdPersonCharacter.BaseWalkSpeed` _asthird_person_character) _result) (`Character.CharacterMovement` _asthird_person_character)))
              (:`then_1`
                (bind _asthird_person_character_2 (cast `/Game/ThirdPersonBP/Blueprints/ThirdPersonCharacter` (`self.FrontCarrier`)))
                (set `CharacterMovementComponent.MaxWalkSpeed` (+ (`/Game/ThirdPersonBP/Blueprints/ThirdPersonCharacter.BaseWalkSpeed` _asthird_person_character_2) _result) (`Character.CharacterMovement` _asthird_person_character_2))))
            (`KismetArrayLibrary.Array_Clear` (`self.Distance`))))))
    (:`then_1`
      (if (== (`KismetArrayLibrary.Array_Length` (`self.Carriers`)) 1)
        (bind _asthird_person_character_3 (cast `/Game/ThirdPersonBP/Blueprints/ThirdPersonCharacter` (`|GetArrayItem` (`self.Carriers`))))
        (set `CharacterMovementComponent.MaxWalkSpeed` (- (`/Game/ThirdPersonBP/Blueprints/ThirdPersonCharacter.BaseWalkSpeed` _asthird_person_character_3) (`self.SingleCarrierSpeedMalus`)) (`Character.CharacterMovement` _asthird_person_character_3))
        (bind _output_get (set `self.PreviousLocationChest` (`SceneComponent.K2_GetComponentLocation` (`self.ChestBot`))))
        (`SceneComponent.K2_SetWorldLocation` (`self.ChestBot`) (`KismetMathLibrary.VLerp` _output_get (`KismetMathLibrary.GetVectorArrayAverage` (`|MakeArray` (`SceneComponent.K2_GetComponentLocation` (`self.HandleConstraintBack`)) (`SceneComponent.K2_GetComponentLocation` (`Actor.RootComponent` (`self.FrontCarrier`))))) 0.2) false true)))
    (:`then_2`
      (if (!= (`self.FrontCarrier`) (`self.FrontCarrierNone`))
        (bind _asthird_person_character_4 (cast `/Game/ThirdPersonBP/Blueprints/ThirdPersonCharacter` (`self.FrontCarrier`)))
        (if (`/Game/ThirdPersonBP/Blueprints/ThirdPersonCharacter.IsCarrying` _asthird_person_character_4)
          (`KismetArrayLibrary.Array_AddUnique` (`self.Carriers`) _asthird_person_character_4)
          (`SceneComponent.K2_SetWorldLocation` (`self.HandleConstraintFront`) (`SceneComponent.K2_GetComponentLocation` (`/Game/ThirdPersonBP/Blueprints/ThirdPersonCharacter.GrabLocation` _asthird_person_character_4)) false false)
          (`PrimitiveComponent.SetConstraintMode` (`self.HandleConstraintFront`) "XYPlane")
          (else
            (set `self.FrontCarrier` (`self.FrontCarrierNone`))
            (`KismetArrayLibrary.Array_RemoveItem` (`self.Carriers`) _asthird_person_character_4)
            (set `CharacterMovementComponent.MaxWalkSpeed` (`/Game/ThirdPersonBP/Blueprints/ThirdPersonCharacter.BaseWalkSpeed` _asthird_person_character_4) (`Character.CharacterMovement` _asthird_person_character_4))
            (`PrimitiveComponent.SetConstraintMode` (`self.HandleConstraintFront`) "Default")
            (`SceneComponent.K2_SetRelativeLocation` (`self.HandleConstraintFront`) (-70.0 0.0 40.0) false false)))))
    (:`then_3`
      (if (!= (`self.BackCarrier`) (`self.BackCarrierNone`))
        (bind _asthird_person_character_5 (cast `/Game/ThirdPersonBP/Blueprints/ThirdPersonCharacter` (`self.BackCarrier`)))
        (if (`/Game/ThirdPersonBP/Blueprints/ThirdPersonCharacter.IsCarrying` _asthird_person_character_5)
          (`KismetArrayLibrary.Array_AddUnique` (`self.Carriers`) _asthird_person_character_5)
          (`SceneComponent.K2_SetWorldLocation` (`self.HandleConstraintBack`) (`SceneComponent.K2_GetComponentLocation` (`/Game/ThirdPersonBP/Blueprints/ThirdPersonCharacter.GrabLocation` _asthird_person_character_5)) false false)
          (`PrimitiveComponent.SetConstraintMode` (`self.HandleConstraintBack`) "XYPlane")
          (else
            (set `self.BackCarrier` (`self.BackCarrierNone`))
            (`KismetArrayLibrary.Array_RemoveItem` (`self.Carriers`) _asthird_person_character_5)
            (set `CharacterMovementComponent.MaxWalkSpeed` (`/Game/ThirdPersonBP/Blueprints/ThirdPersonCharacter.BaseWalkSpeed` _asthird_person_character_5) (`Character.CharacterMovement` _asthird_person_character_5))
            (`PrimitiveComponent.SetConstraintMode` (`self.HandleConstraintBack`) "Default")
            (`SceneComponent.K2_SetRelativeLocation` (`self.HandleConstraintBack`) (70.0 0.0 40.0) false false)))))
    (:`then_4`
      (`self.GiveGold`))
    (:`then_5`
      ;;[1 0 0.1367] Détruire le coffre quand GoldAtStart == 0
      (if (<= (`self.GoldAtStart`) 0)
        (`self.ChestDestroy`)))))

(event `GiveGold`
  (switch `int` (`KismetArrayLibrary.Array_Length` (`self.Carriers`))
    (:`2`
      (if (>= (`self.GoldAtStart`) (* (`self.CoinsGiven`) 2))
        (`/Engine/EditorBlueprintResources/StandardMacros.DoOnce` false :!label _label
          (:`Completed`
            (for _array_element (`self.Carriers`)
              (bind _asthird_person_character (cast `/Game/ThirdPersonBP/Blueprints/ThirdPersonCharacter` _array_element))
              (set `/Game/ThirdPersonBP/Blueprints/ThirdPersonCharacter.Coins` (+ (`/Game/ThirdPersonBP/Blueprints/ThirdPersonCharacter.Coins` _asthird_person_character) (`self.CoinsGiven`)) _asthird_person_character)
              (bind _aswbp_player_score_increase (cast `/Game/ThirdPersonBP/Blueprints/UI/WBP_PlayerScoreIncrease` (`WidgetComponent.GetUserWidgetObject` (`/Game/ThirdPersonBP/Blueprints/ThirdPersonCharacter.ScoreIncrease` _asthird_person_character))))
              (set `/Game/ThirdPersonBP/Blueprints/UI/WBP_PlayerScoreIncrease.ScoreInt` (`self.CoinsGiven`) _aswbp_player_score_increase)
              (`/Game/ThirdPersonBP/Blueprints/UI/WBP_PlayerScoreIncrease.PlayAnimIncrease` _aswbp_player_score_increase))
            (set `self.GoldAtStart` (- (`self.GoldAtStart`) (* (`self.CoinsGiven`) 2)))
            (`KismetSystemLibrary.Delay` (`self.DelayGiveCoin`))
            (goto _label :!via `Reset`)))))))

(event `ChestDestroy`
  (bind _pointlight1 (`self.PointLight1`))
  (bind _pointlight (`self.PointLight`))
  (bind _chestbot (`self.ChestBot`))
  (`SceneComponent.SetVisibility` (`self.Gold`) false false)
  (`|ExecutionSequence`
    (:`then_0`
      (`SceneComponent.SetWorldScale3D` _chestbot (`|EaseFunction` "EaseIn" 0.05 (`SceneComponent.K2_GetComponentScale` _chestbot) (0.5 0.5 0.5) 1.0))
      (if (== (`SceneComponent.K2_GetComponentScale` (`self.ChestBot`)) (0.7 0.7 0.7) :`ErrorTolerance` 0.01)
        (`SceneComponent.K2_DetachFromComponent` (`self.HandleConstraintBack`) "KeepWorld" "KeepWorld" "KeepWorld" true)
        (`SceneComponent.K2_DetachFromComponent` (`self.HandleConstraintFront`) "KeepWorld" "KeepWorld" "KeepWorld" true)
        (`GameplayStatics.SpawnEmitterAtLocation` "/Game/PolygonPirates/ParticleFX/P_FX_MagicChestDestroy.P_FX_MagicChestDestroy" (`SceneComponent.K2_GetComponentLocation` (`self.ChestBot`)) (struct :`Pitch` 90.0))
        (`self.K2_DestroyActor` self)))
    (:`then_1`
      (`LightComponent.SetIntensity` _pointlight (`KismetMathLibrary.Lerp` (`LightComponentBase.Intensity` _pointlight) 0.0 0.05))
      (`LightComponent.SetIntensity` _pointlight1 (`KismetMathLibrary.Lerp` (`LightComponentBase.Intensity` _pointlight1) 0.0 0.05)))))

(fn `UserConstructionScript`)