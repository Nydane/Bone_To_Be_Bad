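; Carryable beer mug that the player delivers to a client who has ordered, in exchange for coins.
; On BeginPlay it tags itself Carry and Sell, rolls a random tip and displays its value.
; While attached to a carrying character, Tick snaps the mesh to GrabLocation with an XY-plane constraint, otherwise detaching it.
; Trigger overlap with that client credits the carrier, spawns tip coins nearby and destroys the mug.
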(event `self.Trigger.OnComponentBeginOverlap`
  (params (OverlappedComponent :type "PrimitiveComponent Object Reference") (OtherActor :type "Actor Object Reference") (OtherComp :type "PrimitiveComponent Object Reference") (OtherBodyIndex :type Integer) (bFromSweep :type Boolean) (SweepResult :type "HitResult Structure (by ref)"))
  (if (and (== (`GameplayStatics.GetObjectClass` OtherActor) "/Game/(PRG)Everyone/BP_Client.BP_Client_C") (`self.ActorHasTag` OtherActor "HasOrdered"))
    (message `/Game/(PRG)Everyone/BPI_Interact.FoodDelivered` OtherActor (`GameplayStatics.GetObjectClass` self))
    (bind _asthird_person_character (cast `/Game/ThirdPersonBP/Blueprints/ThirdPersonCharacter` (`self.Carrier`)))
    (set `/Game/ThirdPersonBP/Blueprints/ThirdPersonCharacter.Coins` (+ (`/Game/ThirdPersonBP/Blueprints/ThirdPersonCharacter.Coins` _asthird_person_character) (`self.MugValue`)) _asthird_person_character)
    (set `/Game/ThirdPersonBP/Blueprints/ThirdPersonCharacter.IsCarrying` false _asthird_person_character)
    (`/Game/(PRG)Everyone/BP_Spawners.Spawner In Radius` (`self.TipValue`) self (200.0 200.0 200.0) "/Game/Ingredients/Ingredients/Coin.Coin_C"
      (:`Completed`
        (`SceneComponent.K2_DetachFromComponent` (`self.bucketMesh`) "KeepWorld" "KeepWorld" "KeepWorld" true)
        (`SceneComponent.K2_DetachFromComponent` (`self.RootComponent`) "KeepWorld" "KeepWorld" "KeepWorld" true)
        (`PrimitiveComponent.SetConstraintMode` (`self.bucketMesh`) "Default")
        (`self.K2_DestroyActor`)))))

(event `self.ReceiveBeginPlay`
  (set `self.Tags` (`|MakeArray` "Carry" "Sell" :!type "Name"))
  (set `self.TipValue` (`KismetMathLibrary.RandomIntegerInRange` (`self.MugTipMin`) (`self.MugTipMax`)))
  (`TextRenderComponent.K2_SetText` (`self.Value`) (`KismetTextLibrary.Conv_IntToText` (`self.MugValue`))))

(event `self.ReceiveTick`
  (params (DeltaSeconds :type "Float (single-precision)"))
  (if (== (`GameplayStatics.GetObjectClass` (`self.GetAttachParentActor` self)) "/Game/ThirdPersonBP/Blueprints/ThirdPersonCharacter.ThirdPersonCharacter_C")
    (bind _asthird_person_character (cast `/Game/ThirdPersonBP/Blueprints/ThirdPersonCharacter` (`self.GetAttachParentActor` self)))
    (if (`/Game/ThirdPersonBP/Blueprints/ThirdPersonCharacter.IsCarrying` _asthird_person_character)
      (set `self.Carrier` _asthird_person_character)
      (`SceneComponent.K2_SetWorldLocation` (`self.bucketMesh`) (`SceneComponent.K2_GetComponentLocation` (`/Game/ThirdPersonBP/Blueprints/ThirdPersonCharacter.GrabLocation` _asthird_person_character)) false true)
      (`PrimitiveComponent.SetConstraintMode` (`self.bucketMesh`) "XYPlane")
      (else
        ;[1 1 1] A terme, détruire le Seau !
        (`SceneComponent.K2_DetachFromComponent` (`self.bucketMesh`) "KeepWorld" "KeepWorld" "KeepWorld" true)
        (`SceneComponent.K2_DetachFromComponent` (`self.RootComponent`) "KeepWorld" "KeepWorld" "KeepWorld" true)
        (`PrimitiveComponent.SetConstraintMode` (`self.bucketMesh`) "Default")))))

(fn `UserConstructionScript`)