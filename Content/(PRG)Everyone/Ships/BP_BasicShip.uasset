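; BP_BasicShip is a basic ship Blueprint that sets up health and movement mode for Civil, Merchant, War and Ghost ship types.
; The Construction Script switches on ShipType to assign Health and the FollowingSpline flag, which is enabled only for Civil and Merchant ships.
; Tick calls a KillShip event every frame, but that event has no logic in this Blueprint.
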(event `self.ReceiveTick`
  (params (DeltaSeconds :type "Float (single-precision)"))
  (`self.KillShip`))

(event `KillShip`)

(fn `UserConstructionScript`
  (switch `string` (`self.ShipType`)
    (:`Civil`
      (set `self.Health` 2)
      (set `self.followingSpline` true))
    (:`Merchant`
      (set `self.Health` 2)
      (set `self.followingSpline` true))
    (:`War`
      (set `self.Health` 2)
      (set `self.followingSpline` false))
    (:`Ghost`
      (set `self.Health` 4)
      (set `self.followingSpline` false))))