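; Ground spike trap that kills the player character when it is caught on fully extended spikes.
; A timeline started on BeginPlay lerps the Base between start and end locations and restarts each time it finishes.
; The trigger overlap stores the player, then Tick checks for continued overlap while Base height exactly equals the end height.
; A victim in the default state is switched to "Headless" and the character's CheckState is called.
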(event `self.ReceiveBeginPlay`
  ;[1 1 1] Cree une timeline et set la location de l'element
  (bind (_direction _spikemovement) (`Timeline|SpikeTrap` :!label _label)
    (:`Update`
      (`SceneComponent.K2_SetRelativeLocation` (`self.Base`) (`KismetMathLibrary.VLerp` (`self.StartLocation`) (`self.EndLocation`) _spikemovement) false false))
    (:`Finished`
      ;[1 1 1] Recommence la timeline du debut lorsqu'elle se termine
      (switch `ETimelineDirection` "Forward"
        (:`Forward`
          (goto _label :!via `PlayFromStart`))
        (:`Backward`
          (goto _label :!via `ReverseFromEnd`))))))

(event `self.SpikeTrigger.OnComponentBeginOverlap`
  (params (OverlappedComponent :type "PrimitiveComponent Object Reference") (OtherActor :type "Actor Object Reference") (OtherComp :type "PrimitiveComponent Object Reference") (OtherBodyIndex :type Integer) (bFromSweep :type Boolean) (SweepResult :type "HitResult Structure (by ref)"))
  ;[1 1 1] Have we hit a player? If so, we set "Player Hit" to make sure that the rest happens to the right victim.
  (if (== (`GameplayStatics.GetObjectClass` OtherActor) "/Game/ThirdPersonBP/Blueprints/ThirdPersonCharacter.ThirdPersonCharacter_C")
    (set `self.PlayerHit` OtherActor)))

(event `self.ReceiveTick`
  (params (DeltaSeconds :type "Float (single-precision)"))
  (bind (_endlocation_x _endlocation_y _endlocation_z) (`KismetMathLibrary.BreakVector` (`self.EndLocation`)))
  (bind (_relativelocation_x _relativelocation_y _relativelocation_z) (`KismetMathLibrary.BreakVector` (`SceneComponent.RelativeLocation` (`self.Base`))))
  ;[1 1 1] Is there a player overlapping with the trigger?
  (if (`PrimitiveComponent.IsOverlappingActor` (`self.SpikeTrigger`) (`self.PlayerHit`))
    ;[1 1 1] Depending on the trigger's position, we will kill "Player Hit"
    (bind _asthird_person_character (cast `/Game/ThirdPersonBP/Blueprints/ThirdPersonCharacter` (`self.PlayerHit`)))
    (if (== _relativelocation_z _endlocation_z)
      (if (`|EnumEquality` (`/Game/ThirdPersonBP/Blueprints/ThirdPersonCharacter.CurrentState` _asthird_person_character) "NewEnumerator0")
        ;;[1 1 1] Change their State to "Headless"
        (set `/Game/ThirdPersonBP/Blueprints/ThirdPersonCharacter.CurrentState` "NewEnumerator1" _asthird_person_character)
        ;;[1 1 1] Call "Check State", stored within the Player Character.
        (`/Game/ThirdPersonBP/Blueprints/ThirdPersonCharacter.Check State` _asthird_person_character)))))

(fn `UserConstructionScript`)