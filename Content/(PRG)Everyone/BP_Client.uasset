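; BP_Client is a customer that cycles through idle, ordering and timed delivery states, driven from Tick.
; After a random idle wait it orders, unless two or more clients already have orders.
; Solo orders spawn beer, apples or ribs at tagged targets; two-player Grog orders use a food spawner.
; Each order sets a tag and colored lights; tags clear when the delivery wait ends, alongside a widget countdown.
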(event `self.ReceiveBeginPlay`
  ;[1 1 1] Comment
  (`|ExecutionSequence`
    (:`then_0`
      (set `self.StartMinIdleWait` (`self.minIdleWait`))
      (set `self.StartMaxIdleWait` (`self.maxIdleWait`))
      (bind _outactors (`GameplayStatics.GetAllActorsOfClass` "BP_Client_C"))
      (set `self.otherClients` _outactors)
      (bind _aswbp_deliver_timer (cast `/Game/ThirdPersonBP/Blueprints/UI/WBP_DeliverTimer` (`WidgetComponent.GetUserWidgetObject` (`self.DeliveryTimer`))))
      (set `/Game/ThirdPersonBP/Blueprints/UI/WBP_DeliverTimer.DeliverRef` self _aswbp_deliver_timer)
      (bind _aswbp_order_numbers (cast `/Game/ThirdPersonBP/Blueprints/UI/WBP_OrderNumbers` (`WidgetComponent.GetUserWidgetObject` (`self.OrderNumber`))))
      (set `/Game/ThirdPersonBP/Blueprints/UI/WBP_OrderNumbers.ClientOrderNumber` self _aswbp_order_numbers))
    (:`then_1`
      (bind _outactors_2 (`GameplayStatics.GetAllActorsOfClassWithTag` "/Game/(PRG)Everyone/BP_SpawnManagerTarget.BP_SpawnManagerTarget_C" "Meat"))
      (set `self.SpawnTargetMeat` _outactors_2))
    (:`then_2`
      (bind _outactors_3 (`GameplayStatics.GetAllActorsOfClassWithTag` "/Game/(PRG)Everyone/BP_SpawnManagerTarget.BP_SpawnManagerTarget_C" "Veggies"))
      (set `self.SpawnTargetVeggies` _outactors_3))
    (:`then_3`
      (bind _outactors_4 (`GameplayStatics.GetAllActorsOfClassWithTag` "/Game/(PRG)Everyone/BP_SpawnManagerTarget.BP_SpawnManagerTarget_C" "Alcohol"))
      (set `self.SpawnTargetAlcohol` _outactors_4))))

(event `Spawn2Player`
  (bind _rectlight (`self.RectLight`))
  (bind _pointlight (`/Game/(PRG)Everyone/Art/LitTorch.PointLight` (`self.LitCandle`)))
  ;[0.1269 1 0.211 1 56] Spawn2P, To be called by changing the Client's State in a Level Blueprint.
  (set `self.Wants2P` true)
  (`KismetArrayLibrary.Array_AddUnique` (`self.Tags`) "HasOrderedGrog")
  ;;[1 1 1] A refaire sans le food spawner (see 1P Spawn)
  (`/Game/(PRG)Everyone/BP_FoodSpawner.SpawnFood` (`self.FoodSpawnerRef`) 0 1 (`self.Wants1P`) (`self.Wants2P`))
  (set `self.DeliveryWait` (`self.2PlayersWait`))
  (set `self.State` "NewEnumerator5")
  (`LightComponent.SetLightColor` _pointlight (struct :`R` 0.188235 :`G` 0.780392 :`A` 1.0) true)
  (`LightComponent.SetIntensity` _pointlight 6500.0)
  (`LightComponent.SetLightColor` _rectlight (struct :`R` 0.188235 :`G` 0.780392 :`A` 1.0) true)
  (`LightComponent.SetIntensity` _rectlight 2500.0))

(event `TryOrder`
  ;[1 0.8306 0.3224 1 56] TryOrder: Counts how many Clients are already waiting for a Beer, then sets the Client's State accordingly.
  (set `self.beersAlreadyOrdered` 0)
  (for _array_element (`self.otherClients`)
    (bind _state (`/Game/(PRG)Everyone/BP_Client.State` _array_element))
    (if (or (`|EnumEquality` _state "NewEnumerator5") (`|EnumEquality` _state "NewEnumerator2"))
      (`/Engine/EditorBlueprintResources/StandardMacros.IncrementInt` (`self.beersAlreadyOrdered`))))
  (if (< (`self.beersAlreadyOrdered`) 2)
    (set `self.State` "NewEnumerator2")
    (else
      (set `self.State` "NewEnumerator0"))))

(event `self.ReceiveTick`
  (params (DeltaSeconds :type "Float (single-precision)"))
  ;[1 1 1 1 56] State Manager
  (`/Engine/EditorBlueprintResources/StandardMacros.DoOnce` false :!label _label
    (:`Completed`
      (switch `/Game/(PRG)Everyone/Enum_ClientStateRework` (`self.State`)
        (:`NewEnumerator0`
          (`self.IdleTimer`)
          (goto _label :!via `Reset`))
        (:`NewEnumerator1`
          (`self.TryOrder`)
          (goto _label :!via `Reset`))
        (:`NewEnumerator2`
          (`self.Spawn1Player`)
          (goto _label :!via `Reset`))
        (:`NewEnumerator3`
          (`self.Spawn2Player`)
          (goto _label :!via `Reset`))
        (:`NewEnumerator5`
          (`self.TimerDelivery`)
          (goto _label :!via `Reset`))))))

(event `PlayDeliveryValidate`
  (`GameplayStatics.SpawnSoundAtLocation` "/Game/_ART_Everyone/Music/Bruitages/Service_validé.Service_validé" (0.0 0.0 0.0) (struct) 1.0 1.0 0.0 null null))

(event `IdleTimer`
  (bind _litcandle (`self.LitCandle`))
  (bind _pointlight (`/Game/(PRG)Everyone/Art/LitTorch.PointLight` _litcandle))
  ;[0.5172 0.1739 1 1 56] IdleTimer: Makes the transition between wanting to order something and actually doing it.
  (`|ExecutionSequence`
    (:`then_0`
      (`KismetArrayLibrary.Array_Clear` (`self.Tags`))
      (`SceneComponent.SetHiddenInGame` (`self.WantsADrinkVis`) true false)
      (`LightComponent.SetLightColor` _pointlight (`/Game/(PRG)Everyone/Art/LitTorch.StartLightColor` _litcandle) true)
      (`LightComponent.SetIntensity` _pointlight 500.0)
      (`LightComponent.SetIntensity` (`self.RectLight`) 300.0)
      (`KismetSystemLibrary.Delay` (+ (`KismetMathLibrary.Conv_IntToDouble` (`KismetMathLibrary.RandomIntegerInRange` (`self.minIdleWait`) (`self.maxIdleWait`))) (`KismetMathLibrary.RandomFloatInRange` 0.1 0.5)) :!label _label_2)
      (if (>= (`KismetMathLibrary.RandomIntegerInRange` 0 10) 5)
        (set `self.State` "NewEnumerator1")
        (else
          (goto _label_2))))
    (:`then_1`
      (set `self.Wants1P` false)
      (set `self.Wants2P` false))))

(event `TimerDelivery`
  ;[0.2776 0.9303 1 1 56] Delivery: Handles both the Tag allowing a client to take an item and its associated timer.
  (`|ExecutionSequence`
    (:`then_0`
      (`KismetSystemLibrary.Delay` (`KismetMathLibrary.Conv_IntToDouble` (`self.DeliveryWait`)))
      (`KismetArrayLibrary.Array_Clear` (`self.Tags`))
      (set `self.State` "NewEnumerator0"))
    (:`then_1`
      ;;[1 0.5601 0.1227 1 27] Order Timer
      (`/Engine/EditorBlueprintResources/StandardMacros.DoOnce` false :!label _label_3
        (:`Completed`
          (`KismetSystemLibrary.Delay` 0.05)
          (set `self.DeliverySeconds` (`self.DeliveryWait`))
          (`SceneComponent.SetHiddenInGame` (`self.DeliveryTimer`) false false)
          (`KismetSystemLibrary.Delay` 1.0 :!label _label_4)
          (if (>= (`KismetArrayLibrary.Array_Length` (`self.Tags`)) 1)
            (if (> (`self.DeliverySeconds`) 0)
              (set `self.DeliverySeconds` (- (`self.DeliverySeconds`) 1))
              (if (== (`self.DeliverySeconds`) 0)
                (`SceneComponent.SetHiddenInGame` (`self.DeliveryTimer`) true false)
                (goto _label_3 :!via `Reset`)
                (else
                  (goto _label_4))))
            (else
              (`SceneComponent.SetHiddenInGame` (`self.DeliveryTimer`) true false)
              (goto _label_3 :!via `Reset`))))))))

(event `Spawn1Player`
  (bind _rectlight (`self.RectLight`))
  (bind _spawntargetalcohol (`self.SpawnTargetAlcohol`))
  (bind _spawntargetmeat (`self.SpawnTargetMeat`))
  (bind _rectlight_2 (`self.RectLight`))
  (bind _rectlight_3 (`self.RectLight`))
  (bind _spawntargetveggies (`self.SpawnTargetVeggies`))
  (bind _pointlight (`/Game/(PRG)Everyone/Art/LitTorch.PointLight` (`self.LitCandle`)))
  (bind _pointlight_2 (`/Game/(PRG)Everyone/Art/LitTorch.PointLight` (`self.LitCandle`)))
  (bind _pointlight_3 (`/Game/(PRG)Everyone/Art/LitTorch.PointLight` (`self.LitCandle`)))
  ;[0.1073 0.2812 1 1 56] Spawn1P: Spawns an object that can be carried by one player.
  (set `self.Wants1P` true)
  (set `self.DeliveryWait` (`self.1PlayerWait`))
  (switch `int` (`KismetMathLibrary.RandomIntegerInRange` 1 20)
    (:`Default`
      (`|SpawnActorFromClass` "/Game/(PRG)Everyone/BP_BeerMugWithGrab.BP_BeerMugWithGrab_C" (`KismetMathLibrary.Conv_VectorToTransform` (`SceneComponent.K2_GetComponentLocation` (`/Game/(PRG)Everyone/BP_SpawnManagerTarget.DefaultSceneRoot` (`|GetArrayItem` _spawntargetalcohol (`KismetMathLibrary.RandomIntegerInRange` 0 (- (`KismetArrayLibrary.Array_Length` _spawntargetalcohol) 1)))))) "Undefined" "OverrideRootScale" null 4 0 null)
      (`KismetArrayLibrary.Array_AddUnique` (`self.Tags`) "HasOrderedBeer")
      (`LightComponent.SetLightColor` _pointlight (`self.LightColAlcohol`) true)
      (`LightComponent.SetIntensity` _pointlight 4500.0)
      ;;[1 1 1] Corriger Widget UI : "Order Number"
      (`LightComponent.SetLightColor` _rectlight (`self.LightColAlcohol`) true)
      (`LightComponent.SetIntensity` _rectlight 1500.0)
      (set `self.UIIndex` 0))
    (:`7`
      (`|SpawnActorFromClass` "/Game/(PRG)Everyone/BP_AppleBasket.BP_AppleBasket_C" (`KismetMathLibrary.Conv_VectorToTransform` (`SceneComponent.K2_GetComponentLocation` (`/Game/(PRG)Everyone/BP_SpawnManagerTarget.DefaultSceneRoot` (`|GetArrayItem` _spawntargetveggies (`KismetMathLibrary.RandomIntegerInRange` 0 (- (`KismetArrayLibrary.Array_Length` _spawntargetveggies) 1)))))) "Undefined" "OverrideRootScale" null 8 null :!label _label_5)
      (`KismetArrayLibrary.Array_AddUnique` (`self.Tags`) "HasOrderedAppleBasket")
      (`LightComponent.SetLightColor` _pointlight_2 (`self.LightColVeggies`) true)
      (`LightComponent.SetIntensity` _pointlight_2 4500.0)
      (`LightComponent.SetLightColor` _rectlight_2 (`self.LightColVeggies`) true)
      (`LightComponent.SetIntensity` _rectlight_2 1500.0)
      (set `self.UIIndex` 1))
    (:`8`
      (goto _label_5))
    (:`9`
      (goto _label_5))
    (:`10`
      (`|SpawnActorFromClass` "/Game/(PRG)Everyone/BP_Ribs.BP_Ribs_C" (`KismetMathLibrary.Conv_VectorToTransform` (`SceneComponent.K2_GetComponentLocation` (`/Game/(PRG)Everyone/BP_SpawnManagerTarget.DefaultSceneRoot` (`|GetArrayItem` _spawntargetmeat (`KismetMathLibrary.RandomIntegerInRange` 0 (- (`KismetArrayLibrary.Array_Length` _spawntargetmeat) 1)))))) "Undefined" "OverrideRootScale" null 16 null)
      (`KismetArrayLibrary.Array_AddUnique` (`self.Tags`) "HasOrderedRibs")
      (`LightComponent.SetLightColor` _pointlight_3 (`self.LightColMeat`) true)
      (`LightComponent.SetIntensity` _pointlight_3 4500.0)
      (`LightComponent.SetLightColor` _rectlight_3 (`self.LightColMeat`) true)
      (`LightComponent.SetIntensity` _rectlight_3 1500.0)
      (set `self.UIIndex` 2)))
  (set `self.State` "NewEnumerator5"))

(fn `UserConstructionScript`)