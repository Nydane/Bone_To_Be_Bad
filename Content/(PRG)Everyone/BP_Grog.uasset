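; Sellable grog cauldron that one or two players carry to clients who ordered grog.
; Tick pins the cable-linked front and back handles to carriers' grab points, lerps the cauldron toward their average location, and adjusts walk speed by carrier separation or a solo penalty.
; Overlapping a waiting client delivers it: gold is reported to the magic chest, carriers split the value, random tip coins spawn, and the actor is destroyed.
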(event `self.Trigger.OnComponentBeginOverlap`
  (params (OverlappedComponent :type "PrimitiveComponent Object Reference") (OtherActor :type "Actor Object Reference") (OtherComp :type "PrimitiveComponent Object Reference") (OtherBodyIndex :type Integer) (bFromSweep :type Boolean) (SweepResult :type "HitResult Structure (by ref)"))
  (if (and (== (`GameplayStatics.GetObjectClass` OtherActor) "/Game/(PRG)Everyone/BP_Client.BP_Client_C") (`self.ActorHasTag` OtherActor "HasOrdered"))
    (bind _asbp_client (cast `/Game/(PRG)Everyone/BP_Client` OtherActor))
    (if (`/Game/(PRG)Everyone/BP_Client.WantsGrog` _asbp_client)
      (message `/Game/(PRG)Everyone/BPI_Interact.FoodDelivered` OtherActor (`GameplayStatics.GetObjectClass` self))
      (message `/Game/(PRG)Everyone/BPI_Interact.CountGold` (`self.MagicChestRef`) (+ (`self.grogValue`) (`self.GrogTipValue`)))
      (switch `int` (`KismetArrayLibrary.Array_Length` (`self.Carriers`))
        (:`1`
          (bind _asthird_person_character (cast `/Game/ThirdPersonBP/Blueprints/ThirdPersonCharacter` (`|GetArrayItem` (`self.Carriers`))))
          (set `/Game/ThirdPersonBP/Blueprints/ThirdPersonCharacter.Coins` (+ (`/Game/ThirdPersonBP/Blueprints/ThirdPersonCharacter.Coins` _asthird_person_character) (`self.grogValue`)) _asthird_person_character)
          (set `/Game/ThirdPersonBP/Blueprints/ThirdPersonCharacter.IsCarrying` false _asthird_person_character)
          (set `CharacterMovementComponent.MaxWalkSpeed` (`/Game/ThirdPersonBP/Blueprints/ThirdPersonCharacter.BaseWalkSpeed` _asthird_person_character) (`Character.CharacterMovement` _asthird_person_character)))
        (:`2`
          (for _array_element (`self.Carriers`)
            (bind _asthird_person_character_2 (cast `/Game/ThirdPersonBP/Blueprints/ThirdPersonCharacter` _array_element))
            (set `/Game/ThirdPersonBP/Blueprints/ThirdPersonCharacter.Coins` (+ (`/Game/ThirdPersonBP/Blueprints/ThirdPersonCharacter.Coins` _asthird_person_character_2) (/ (`self.grogValue`) 2)) _asthird_person_character_2)
            (set `/Game/ThirdPersonBP/Blueprints/ThirdPersonCharacter.IsCarrying` false _asthird_person_character_2)
            (set `CharacterMovementComponent.MaxWalkSpeed` (`/Game/ThirdPersonBP/Blueprints/ThirdPersonCharacter.BaseWalkSpeed` _asthird_person_character_2) (`Character.CharacterMovement` _asthird_person_character_2)))))
      (`/Game/(PRG)Everyone/BP_Spawners.Spawner In Radius` (`self.GrogTipValue`) self (200.0 200.0 200.0) "/Game/Ingredients/Ingredients/Coin.Coin_C"
        (:`Completed`
          (`KismetArrayLibrary.Array_Clear` (`self.Carriers`))
          (`SceneComponent.K2_DetachFromComponent` (`self.HandleConstraintFront`) "KeepWorld" "KeepWorld" "KeepWorld" true)
          (`SceneComponent.K2_DetachFromComponent` (`self.HandleConstraintBack`) "KeepWorld" "KeepWorld" "KeepWorld" true)
          (`self.K2_DestroyActor`))))))

(event `self.ReceiveBeginPlay`
  ;[1 1 1] Setting up everything needed on Begin Play
  (set `self.Tags` (`|MakeArray` "Sell" :!type "Name"))
  (set `ActorComponent.ComponentTags` (`|MakeArray` "CarryFront" :!type "Name") (`self.HandleConstraintFront`))
  (set `ActorComponent.ComponentTags` (`|MakeArray` "CarryBack" :!type "Name") (`self.HandleConstraintBack`))
  (`CableComponent.SetAttachEndToComponent` (`self.CableFront`) (`self.HandleConstraintFront`) "None")
  (`CableComponent.SetAttachEndToComponent` (`self.CableBack`) (`self.HandleConstraintBack`) "None")
  (set `self.GrogTipValue` (`KismetMathLibrary.RandomIntegerInRange` (`self.grogTipMin`) (`self.grogTipMax`)))
  (`TextRenderComponent.K2_SetText` (`self.Value`) (`KismetTextLibrary.Conv_IntToText` (`self.grogValue`)))
  (bind _outactors (`GameplayStatics.GetAllActorsOfClass` "/Game/(PRG)Everyone/BP_MagicChest.BP_MagicChest_C"))
  (set `self.MagicChestRef` (`|GetArrayItem` _outactors)))

(event `self.ReceiveTick`
  (params (DeltaSeconds :type "Float (single-precision)"))
  ;[1 1 1 1 123] Promis je commente plus tard, pas taper s'il vous plait !
  (`|ExecutionSequence`
    (:`then_0`
      (if (!= (`KismetArrayLibrary.Array_Length` (`self.Carriers`)) 0)
        (set `self.PreviousLocationMarmite` (`SceneComponent.K2_GetComponentLocation` (`self.Marmite`)))
        (bind _returnvalue (`GameplayStatics.GetActorArrayAverageLocation` (`self.Carriers`)))
        (`SceneComponent.K2_SetWorldLocation` (`self.Marmite`) (`KismetMathLibrary.VLerp` (`self.PreviousLocationMarmite`) _returnvalue 0.01) false false)
        (for (_array_element _array_index) (`self.Carriers`)
          (set `self.Referent` _array_element)
          (for _index (range (+ _array_index 1) (`KismetArrayLibrary.Array_Length` (`self.Carriers`)))
            (`KismetArrayLibrary.Array_Add` (`self.Distance`) (`self.GetDistanceTo` (`self.Referent`) (`|GetArrayItem` (`self.Carriers`) _index)))))
        (bind _result (`/Engine/EditorBlueprintResources/StandardMacros.NegateFloat` (`KismetMathLibrary.FClamp` (`.MaxValue` (`KismetMathLibrary.MaxOfFloatArray` (`self.Distance`))) (`self.MinSpeedLost`) (`self.MaxSpeedLost`)))
          (:`  `
            (`|ExecutionSequence`
              (:`then_0`
                (bind _asthird_person_character (cast `/Game/ThirdPersonBP/Blueprints/ThirdPersonCharacter` (`self.BackCarrier`)))
                (set `CharacterMovementComponent.MaxWalkSpeed` (+ (`/Game/ThirdPersonBP/Blueprints/ThirdPersonCharacter.BaseWalkSpeed` _asthird_person_character) _result) (`Character.CharacterMovement` _asthird_person_character)))
              (:`then_1`
                (bind _asthird_person_character_2 (cast `/Game/ThirdPersonBP/Blueprints/ThirdPersonCharacter` (`self.FrontCarrier`)))
                (set `CharacterMovementComponent.MaxWalkSpeed` (+ (`/Game/ThirdPersonBP/Blueprints/ThirdPersonCharacter.BaseWalkSpeed` _asthird_person_character_2) _result) (`Character.CharacterMovement` _asthird_person_character_2))))
            (`KismetArrayLibrary.Array_Clear` (`self.Distance`))))))
    (:`then_1`
      (if (== (`KismetArrayLibrary.Array_Length` (`self.Carriers`)) 1)
        (bind _asthird_person_character_3 (cast `/Game/ThirdPersonBP/Blueprints/ThirdPersonCharacter` (`|GetArrayItem` (`self.Carriers`))))
        (set `CharacterMovementComponent.MaxWalkSpeed` (- (`/Game/ThirdPersonBP/Blueprints/ThirdPersonCharacter.BaseWalkSpeed` _asthird_person_character_3) (`self.SingleCarrierSpeedMalus`)) (`Character.CharacterMovement` _asthird_person_character_3))))
    (:`then_2`
      (if (!= (`self.FrontCarrier`) (`self.FrontCarrierNone`))
        (bind _asthird_person_character_4 (cast `/Game/ThirdPersonBP/Blueprints/ThirdPersonCharacter` (`self.FrontCarrier`)))
        (if (`/Game/ThirdPersonBP/Blueprints/ThirdPersonCharacter.IsCarrying` _asthird_person_character_4)
          (`KismetArrayLibrary.Array_AddUnique` (`self.Carriers`) _asthird_person_character_4)
          (`SceneComponent.K2_SetWorldLocation` (`self.HandleConstraintFront`) (`SceneComponent.K2_GetComponentLocation` (`/Game/ThirdPersonBP/Blueprints/ThirdPersonCharacter.GrabLocation` _asthird_person_character_4)) false false)
          (`PrimitiveComponent.SetConstraintMode` (`self.HandleConstraintFront`) "XYPlane")
          (else
            (set `self.FrontCarrier` (`self.FrontCarrierNone`))
            (`KismetArrayLibrary.Array_RemoveItem` (`self.Carriers`) _asthird_person_character_4)
            (set `CharacterMovementComponent.MaxWalkSpeed` (`/Game/ThirdPersonBP/Blueprints/ThirdPersonCharacter.BaseWalkSpeed` _asthird_person_character_4) (`Character.CharacterMovement` _asthird_person_character_4))
            (`PrimitiveComponent.SetConstraintMode` (`self.HandleConstraintFront`) "Default")))))
    (:`then_3`
      (if (!= (`self.BackCarrier`) (`self.BackCarrierNone`))
        (bind _asthird_person_character_5 (cast `/Game/ThirdPersonBP/Blueprints/ThirdPersonCharacter` (`self.BackCarrier`)))
        (if (`/Game/ThirdPersonBP/Blueprints/ThirdPersonCharacter.IsCarrying` _asthird_person_character_5)
          (`KismetArrayLibrary.Array_AddUnique` (`self.Carriers`) _asthird_person_character_5)
          (`SceneComponent.K2_SetWorldLocation` (`self.HandleConstraintBack`) (`SceneComponent.K2_GetComponentLocation` (`/Game/ThirdPersonBP/Blueprints/ThirdPersonCharacter.GrabLocation` _asthird_person_character_5)) false false)
          (`PrimitiveComponent.SetConstraintMode` (`self.HandleConstraintBack`) "XYPlane")
          (else
            (set `self.BackCarrier` (`self.BackCarrierNone`))
            (`KismetArrayLibrary.Array_RemoveItem` (`self.Carriers`) _asthird_person_character_5)
            (set `CharacterMovementComponent.MaxWalkSpeed` (`/Game/ThirdPersonBP/Blueprints/ThirdPersonCharacter.BaseWalkSpeed` _asthird_person_character_5) (`Character.CharacterMovement` _asthird_person_character_5))
            (`PrimitiveComponent.SetConstraintMode` (`self.HandleConstraintBack`) "Default")))))))

(fn `UserConstructionScript`)