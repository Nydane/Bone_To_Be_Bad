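; BP_GoldBagSpawner keeps spawning double-scale grabbable gold bags at random points inside a box around itself, up to a maximum count.
; Tick drives a self-resetting DoOnce that waits, counts all such bags in the level, then spawns one or waits again if at the limit.
; SpawnBag spawns immediately without the count check and resets the DoOnce.
; The construction script sizes the VisSpawn box to match the spawn area.
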(event `self.ReceiveTick`
  (params (DeltaSeconds :type "Float (single-precision)"))
  (`/Engine/EditorBlueprintResources/StandardMacros.DoOnce` false :!label _label
    (:`Completed`
      (`KismetSystemLibrary.Delay` (`self.WaitSpawn`))
      (bind _outactors (`GameplayStatics.GetAllActorsOfClass` "/Game/(PRG)Everyone/Deliveries/BP_GoldBag_WithGrab.BP_GoldBag_WithGrab_C"))
      (if (< (`KismetArrayLibrary.Array_Length` _outactors) (`self.MaxBagAllowed`))
        (`|SpawnActorFromClass` "/Game/(PRG)Everyone/Deliveries/BP_GoldBag_WithGrab.BP_GoldBag_WithGrab_C" (`KismetMathLibrary.MakeTransform` (`KismetMathLibrary.RandomPointInBoundingBox` (`self.K2_GetActorLocation` self) (`self.SpawnSize`)) (struct) (2.0 2.0 2.0)) "Undefined" "OverrideRootScale" null 4 0 null :!label _label_2)
        (goto _label :!via `Reset`)
        (else
          (`KismetSystemLibrary.Delay` (`self.FailWaitSpawn`))
          (goto _label :!via `Reset`))))))

(event `SpawnBag`
  (goto _label_2))

(fn `UserConstructionScript`
  (`BoxComponent.SetBoxExtent` (`self.VisSpawn`) (`self.SpawnSize`) true))