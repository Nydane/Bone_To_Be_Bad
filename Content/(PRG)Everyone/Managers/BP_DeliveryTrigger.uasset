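; BP_DeliveryTrigger is a delivery zone for BP_WS_Chest2P, marked by lit torches around it.
; On BeginPlay, a sphere trace around its Box finds nearby Dynamic_LitTorch actors and unhides their light and flame.
; When the chest overlaps the Box, the same trace hides those effects, and the trigger destroys itself after a short delay.
; Both traces have timed debug drawing enabled.
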(event `self.ReceiveBeginPlay`
  (bind _returnvalue (`SceneComponent.K2_GetComponentLocation` (`self.Box`)))
  (bind _outhits (`KismetSystemLibrary.SphereTraceMultiForObjects` :`Start` _returnvalue :`End` (+ _returnvalue 1.0) :`Radius` 600.0 :`ObjectTypes` (`|MakeArray` "ObjectTypeQuery1" :!type "EObjectTypeQuery Enum") :`DrawDebugType` "ForDuration"))
  (for _array_element _outhits
    (bind (_bblockinghit _binitialoverlap _time _distance _location _impactpoint _normal _impactnormal _physmat _hitactor) (`GameplayStatics.BreakHitResult` _array_element))
    (if (== (`GameplayStatics.GetObjectClass` _hitactor) "/Game/(PRG)Everyone/Art/Dynamic_LitTorch.Dynamic_LitTorch_C")
      (bind _asdynamic_lit_torch (cast `/Game/(PRG)Everyone/Art/Dynamic_LitTorch` _hitactor))
      (`SceneComponent.SetHiddenInGame` (`/Game/(PRG)Everyone/Art/Dynamic_LitTorch.PointLight` _asdynamic_lit_torch) false false)
      (`SceneComponent.SetHiddenInGame` (`/Game/(PRG)Everyone/Art/Dynamic_LitTorch.Flames (Tiny)` _asdynamic_lit_torch) false false))))

(event `self.Box.OnComponentBeginOverlap`
  (params (OverlappedComponent :type "PrimitiveComponent Object Reference") (OtherActor :type "Actor Object Reference") (OtherComp :type "PrimitiveComponent Object Reference") (OtherBodyIndex :type Integer) (bFromSweep :type Boolean) (SweepResult :type "HitResult Structure (by ref)"))
  (bind _returnvalue (`SceneComponent.K2_GetComponentLocation` (`self.Box`)))
  (if (== (`GameplayStatics.GetObjectClass` OtherActor) "/Game/(PRG)Everyone/Deliveries/BP_WS_Chest2P.BP_WS_Chest2P_C")
    (`|ExecutionSequence`
      (:`then_0`
        (`KismetSystemLibrary.Delay` 0.2)
        (`self.K2_DestroyActor`))
      (:`then_1`
        (bind _outhits (`KismetSystemLibrary.SphereTraceMultiForObjects` :`Start` _returnvalue :`End` (+ _returnvalue 1.0) :`Radius` 600.0 :`ObjectTypes` (`|MakeArray` "ObjectTypeQuery1" :!type "EObjectTypeQuery Enum") :`DrawDebugType` "ForDuration"))
        (for _array_element _outhits
          (bind (_bblockinghit _binitialoverlap _time _distance _location _impactpoint _normal _impactnormal _physmat _hitactor) (`GameplayStatics.BreakHitResult` _array_element))
          (if (== (`GameplayStatics.GetObjectClass` _hitactor) "/Game/(PRG)Everyone/Art/Dynamic_LitTorch.Dynamic_LitTorch_C")
            (bind _asdynamic_lit_torch (cast `/Game/(PRG)Everyone/Art/Dynamic_LitTorch` _hitactor))
            (`SceneComponent.SetHiddenInGame` (`/Game/(PRG)Everyone/Art/Dynamic_LitTorch.PointLight` _asdynamic_lit_torch) true false)
            (`SceneComponent.SetHiddenInGame` (`/Game/(PRG)Everyone/Art/Dynamic_LitTorch.Flames (Tiny)` _asdynamic_lit_torch) true false)))))))

(fn `UserConstructionScript`)