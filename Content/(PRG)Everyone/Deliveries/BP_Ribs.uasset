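; BP_Ribs is a carryable food plate that players deliver to clients tagged HasOrderedRibs.
; Tick follows the attached ThirdPersonCharacter's grab point, slows the carrier, and toggles a carried tag against stealing, restoring speed on release.
; Overlapping a matching client resets its order, pays the carrier coins with a score popup, reports gold to the MagicChestPinata and destroys the plate.
; Ribs left uncarried destroy themselves after a delay.
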(event `self.Trigger.OnComponentBeginOverlap`
  (params (OverlappedComponent :type "PrimitiveComponent Object Reference") (OtherActor :type "Actor Object Reference") (OtherComp :type "PrimitiveComponent Object Reference") (OtherBodyIndex :type Integer) (bFromSweep :type Boolean) (SweepResult :type "HitResult Structure (by ref)"))
  (if (and (== (`GameplayStatics.GetObjectClass` OtherActor) "/Game/(PRG)Everyone/BP_Client.BP_Client_C") (`self.ActorHasTag` OtherActor "HasOrderedRibs"))
    (bind _asbp_client (cast `/Game/(PRG)Everyone/BP_Client` OtherActor))
    (`/Game/(PRG)Everyone/BP_Client.PlayDeliveryValidate` _asbp_client)
    (`KismetArrayLibrary.Array_Clear` (`Actor.Tags` _asbp_client))
    (set `/Game/(PRG)Everyone/BP_Client.State` "NewEnumerator0" _asbp_client)
    (`|ExecutionSequence`
      (:`then_0`
        (message `/Game/(PRG)Everyone/BPI_Interact.FoodDelivered` OtherActor (`GameplayStatics.GetObjectClass` self))
        (bind _asthird_person_character (cast `/Game/ThirdPersonBP/Blueprints/ThirdPersonCharacter` (`self.Carrier`)))
        (set `/Game/ThirdPersonBP/Blueprints/ThirdPersonCharacter.Coins` (+ (`/Game/ThirdPersonBP/Blueprints/ThirdPersonCharacter.Coins` _asthird_person_character) (`self.RibsValue`)) _asthird_person_character)
        (set `/Game/ThirdPersonBP/Blueprints/ThirdPersonCharacter.IsCarrying` false _asthird_person_character)
        (bind _aswbp_player_score_increase (cast `/Game/ThirdPersonBP/Blueprints/UI/WBP_PlayerScoreIncrease` (`WidgetComponent.GetUserWidgetObject` (`/Game/ThirdPersonBP/Blueprints/ThirdPersonCharacter.ScoreIncrease` _asthird_person_character))))
        (set `/Game/ThirdPersonBP/Blueprints/UI/WBP_PlayerScoreIncrease.ScoreInt` (`self.RibsValue`) _aswbp_player_score_increase)
        (`/Game/ThirdPersonBP/Blueprints/UI/WBP_PlayerScoreIncrease.PlayAnimIncrease` _aswbp_player_score_increase)
        (`SceneComponent.K2_DetachFromComponent` (`self.plateMesh`) "KeepWorld" "KeepWorld" "KeepWorld" true)
        (`SceneComponent.K2_DetachFromComponent` (`self.RootComponent`) "KeepWorld" "KeepWorld" "KeepWorld" true)
        (`PrimitiveComponent.SetConstraintMode` (`self.plateMesh`) "Default")
        (bind _asthird_person_character_2 (cast `/Game/ThirdPersonBP/Blueprints/ThirdPersonCharacter` (`self.Carrier`)))
        (set `CharacterMovementComponent.MaxWalkSpeed` (`/Game/ThirdPersonBP/Blueprints/ThirdPersonCharacter.BaseWalkSpeed` _asthird_person_character_2) (`Character.CharacterMovement` _asthird_person_character_2))
        (`self.K2_DestroyActor`))
      (:`then_1`
        (message `/Game/(PRG)Everyone/BPI_Interact.CountGold` (`self.MagicChestRef`) (`self.RibsValue`))
        (`GameplayStatics.SpawnSoundAtLocation` "/Game/_ART_Everyone/Music/Bruitages/Bouche_3_-_Nourriture__pomme_.Bouche_3_-_Nourriture__pomme_" (`SceneComponent.K2_GetComponentLocation` (`self.DefaultSceneRoot`)) (struct) 1.0 1.0 0.0 "/Game/(ART)Everyone/Music/AttenuationSettings/Test.Test" null)))))

(event `self.ReceiveBeginPlay`
  (set `self.Tags` (`|MakeArray` "Carry" "Sell" :!type "Name"))
  (bind _outactors (`GameplayStatics.GetAllActorsOfClass` "/Game/(PRG)Everyone/BP_MagicChestPinata.BP_MagicChestPinata_C"))
  (set `self.MagicChestRef` (`|GetArrayItem` _outactors)))

(event `self.ReceiveTick`
  (params (DeltaSeconds :type "Float (single-precision)"))
  (`|ExecutionSequence`
    (:`then_0`
      (if (== (`GameplayStatics.GetObjectClass` (`self.GetAttachParentActor` self)) "/Game/ThirdPersonBP/Blueprints/ThirdPersonCharacter.ThirdPersonCharacter_C")
        (bind _asthird_person_character (cast `/Game/ThirdPersonBP/Blueprints/ThirdPersonCharacter` (`self.GetAttachParentActor` self)))
        (if (`/Game/ThirdPersonBP/Blueprints/ThirdPersonCharacter.IsCarrying` _asthird_person_character)
          (set `self.Carrier` _asthird_person_character)
          (set `CharacterMovementComponent.MaxWalkSpeed` (- (`/Game/ThirdPersonBP/Blueprints/ThirdPersonCharacter.BaseWalkSpeed` _asthird_person_character) (`self.SpeedMalus`)) (`Character.CharacterMovement` _asthird_person_character))
          (`SceneComponent.K2_SetWorldLocation` (`self.plateMesh`) (`SceneComponent.K2_GetComponentLocation` (`/Game/ThirdPersonBP/Blueprints/ThirdPersonCharacter.GrabLocation` _asthird_person_character)) false true)
          (`PrimitiveComponent.SetConstraintMode` (`self.plateMesh`) "XYPlane")
          ;[1 1 1] This Tag allows us to make sure that the object cannot be "stolen" simply by pressing the Grab Button.
          (`/Engine/EditorBlueprintResources/StandardMacros.DoOnce` false :!label _label
            (:`Completed`
              (`KismetArrayLibrary.Array_AddUnique` (`self.Tags`) (`self.CarriedTag`))
              (set `self.isCarried` true)
              (goto _label_2 :!via `Reset`)))
          (else
            ;[1 1 1] A terme, détruire le Seau !
            (`SceneComponent.K2_DetachFromComponent` (`self.plateMesh`) "KeepWorld" "KeepWorld" "KeepWorld" true)
            (`SceneComponent.K2_DetachFromComponent` (`self.RootComponent`) "KeepWorld" "KeepWorld" "KeepWorld" true)
            (`PrimitiveComponent.SetConstraintMode` (`self.plateMesh`) "Default")
            (bind _asthird_person_character_2 (cast `/Game/ThirdPersonBP/Blueprints/ThirdPersonCharacter` (`self.Carrier`)))
            (if (not (`|EnumEquality` (`/Game/ThirdPersonBP/Blueprints/ThirdPersonCharacter.CurrentState` _asthird_person_character_2) "NewEnumerator2"))
              (set `CharacterMovementComponent.MaxWalkSpeed` (`/Game/ThirdPersonBP/Blueprints/ThirdPersonCharacter.BaseWalkSpeed` _asthird_person_character_2) (`Character.CharacterMovement` _asthird_person_character_2)))
            (`KismetSystemLibrary.Delay` 1.0)
            (set `self.Carrier` (`self.CarrierNone`))
            (`/Engine/EditorBlueprintResources/StandardMacros.DoOnce` false :!label _label_2
              (:`Completed`
                (`KismetArrayLibrary.Array_RemoveItem` (`self.Tags`) (`self.CarriedTag`))
                (set `self.isCarried` false)
                (goto _label :!via `Reset`)))))))
    (:`then_1`
      (if (not (`self.isCarried`))
        (`KismetSystemLibrary.Delay` (`self.DelayDestroy`))
        (if (not (`self.isCarried`))
          (`self.K2_DestroyActor`))))))

(fn `UserConstructionScript`)