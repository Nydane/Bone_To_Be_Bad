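; Food spawner actor that places beer mugs and grog (BP_Soup) at target spawn points on request, passing each its price.
; SpawnFood takes counts and want flags, then loops per drink type, picking random targets and checking their Filled flag.
; Occupied picks decrement the loop index, apparently as a retry.
; The check and spawn location roll separately, so drinks can land on filled targets; an author note flags this random bug.
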(event `self.ReceiveBeginPlay`
  ;[1 1 1 1 123] Problème vient de la façon dont on calcule le "random", il faut trouver comment corriger ça !
)

(event `SpawnFood`
  (params (BeersToSpawn :type Integer) (GrogsToSpawn :type Integer) (WantsBeer :type Boolean) (WantsGrog :type Boolean))
  (bind _grogtargetspawns (`self.GrogTargetSpawns`))
  (bind _beertargetspawns (`self.BeerTargetSpawns`))
  (bind _output (`|GetArrayItem` _beertargetspawns (`KismetMathLibrary.RandomIntegerInRange` 0 (- (`KismetArrayLibrary.Array_Length` _beertargetspawns) 1))))
  (bind _output_2 (`|GetArrayItem` _grogtargetspawns (`KismetMathLibrary.RandomIntegerInRange` 0 (- (`KismetArrayLibrary.Array_Length` _grogtargetspawns) 1))))
  ;[1 1 1 1 123] Problème vient de la façon dont on calcule le "random", il faut trouver comment corriger ça !
  (`|ExecutionSequence`
    (:`then_0`
      (if (and WantsBeer (> BeersToSpawn 0))
        (for _index (range 1 (+ BeersToSpawn 1))
          (if (not (`/Game/(PRG)Everyone/BP_SpawnManagerTarget.Filled` _output))
            (bind _returnvalue (`|SpawnActorFromClass` "/Game/(PRG)Everyone/BP_BeerMugWithGrab.BP_BeerMugWithGrab_C" (`KismetMathLibrary.Conv_VectorToTransform` (`self.K2_GetActorLocation` _output)) "Undefined" "OverrideRootScale" null (`self.BeerPrice`) 0 null))
            (if (`KismetSystemLibrary.IsValid` _returnvalue)
              _)
            (else
              (`/Engine/EditorBlueprintResources/StandardMacros.DecrementInt` _index))))))
    (:`then_1`
      (if (and WantsGrog (> GrogsToSpawn 0))
        (for _index_2 (range 1 (+ GrogsToSpawn 1))
          (if (not (`/Game/(PRG)Everyone/BP_SpawnManagerTarget.Filled` _output_2))
            (`|SpawnActorFromClass` "/Game/(PRG)Everyone/BP_Soup.BP_Soup_C" (`KismetMathLibrary.MakeTransform` (`self.K2_GetActorLocation` _output_2) (struct) (1.65 1.65 1.65)) "Undefined" "OverrideRootScale" null (`self.GrogPrice`) null)
            (else
              (`/Engine/EditorBlueprintResources/StandardMacros.DecrementInt` _index_2))))))))

(event `self.ReceiveTick`
  (params (DeltaSeconds :type "Float (single-precision)"))
  ;[1 1 1 1 123] Problème vient de la façon dont on calcule le "random", il faut trouver comment corriger ça !
)

(fn `UserConstructionScript`)