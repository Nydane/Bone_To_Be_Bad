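; Two-player co-op treasure chest that moves on cables while players stand in its trigger box, rewarding gold at the end position.
; Tick counts overlapping characters, easing the pressure plate to a per-count position and the chest forward with two players, back otherwise, via VInterpTo.
; With both players present near the end, GiveGold fires once, adding coins, animating score widgets, freezing movement and hiding the treasure and light.
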(event `self.ReceiveBeginPlay`
  ;[1 0.204 0.2837] BEGIN PLAY
  ; Vis : Set the attachments for the ropes.
  ; Set the position of the Chest and and end position
  (`CableComponent.SetAttachEndToComponent` (`self.Cable1`) (`self.CableAttach1`) "None")
  (`CableComponent.SetAttachEndToComponent` (`self.Cable2`) (`self.CableAttach2`) "None")
  (set `self.StartPosChest` (`SceneComponent.K2_GetComponentLocation` (`self.ChestBot`)))
  (set `self.EndPosChest` (`SceneComponent.K2_GetComponentLocation` (`self.EndPos`)))
  (set `self.PressureStartPos` (`SceneComponent.K2_GetComponentLocation` (`self.VisPressurePlate`)))
  (set `self.PressureEndPos1P` (`SceneComponent.K2_GetComponentLocation` (`self.PressureVisPos1P`)))
  (set `self.PressureEndPos2P` (`SceneComponent.K2_GetComponentLocation` (`self.PressureVisPos2P`))))

(event `MovePressurePlate`
  (params (PlayersInTrigger :type Integer) (DeltaSeconds :type "Float (double-precision)"))
  (if (`self.canMove`)
    (switch `int` PlayersInTrigger
      (:`0`
        (`SceneComponent.K2_SetWorldLocation` (`self.VisPressurePlate`) (`KismetMathLibrary.VInterpTo` (`SceneComponent.K2_GetComponentLocation` (`self.VisPressurePlate`)) (`self.PressureStartPos`) DeltaSeconds 0.8) false false))
      (:`1`
        (`SceneComponent.K2_SetWorldLocation` (`self.VisPressurePlate`) (`KismetMathLibrary.VInterpTo` (`SceneComponent.K2_GetComponentLocation` (`self.VisPressurePlate`)) (`self.PressureEndPos1P`) DeltaSeconds 0.8) false false))
      (:`2`
        (`SceneComponent.K2_SetWorldLocation` (`self.VisPressurePlate`) (`KismetMathLibrary.VInterpTo` (`SceneComponent.K2_GetComponentLocation` (`self.VisPressurePlate`)) (`self.PressureEndPos2P`) DeltaSeconds 0.8) false false)))))

(event `self.ReceiveTick`
  (params (DeltaSeconds :type "Float (single-precision)"))
  (bind _returnvalue (`KismetArrayLibrary.Array_Length` (`self.PlayersInTrigger`)))
  (`|ExecutionSequence`
    (:`then_0`
      (set `self.PlayersInTrigger` (`PrimitiveComponent.GetOverlappingActors` (`self.Box`) "/Game/ThirdPersonBP/Blueprints/ThirdPersonCharacter.ThirdPersonCharacter_C")))
    (:`then_1`
      (`self.MoveChest` _returnvalue DeltaSeconds))
    (:`then_2`
      (`self.MovePressurePlate` _returnvalue DeltaSeconds))
    (:`then_3`
      (if (== (`SceneComponent.K2_GetComponentLocation` (`self.ChestBot`)) (`self.EndPosChest`) :`ErrorTolerance` 50.0)
        (if (== (`KismetArrayLibrary.Array_Length` (`self.PlayersInTrigger`)) 2)
          (`/Engine/EditorBlueprintResources/StandardMacros.DoOnce` false
            (:`Completed`
              (`self.GiveGold`))))))))

(event `MoveChest`
  (params (PlayersInTrigger :type Integer) (deltaSeconds :type "Float (double-precision)"))
  (if (`self.canMove`)
    (switch `int` PlayersInTrigger
      (:`Default`
        (`SceneComponent.K2_SetWorldLocation` (`self.ChestBot`) (`KismetMathLibrary.VInterpTo` (`SceneComponent.K2_GetComponentLocation` (`self.ChestBot`)) (`self.StartPosChest`) deltaSeconds 0.15) false false :!label _label))
      (:`0`
        (`SceneComponent.K2_SetWorldLocation` (`self.ChestBot`) (`KismetMathLibrary.VInterpTo` (`SceneComponent.K2_GetComponentLocation` (`self.ChestBot`)) (`self.StartPosChest`) deltaSeconds 0.5) false false))
      (:`1`
        (goto _label))
      (:`2`
        (`SceneComponent.K2_SetWorldLocation` (`self.ChestBot`) (`KismetMathLibrary.VInterpTo` (`SceneComponent.K2_GetComponentLocation` (`self.ChestBot`)) (`self.EndPosChest`) deltaSeconds 0.3) false false)))))

(event `GiveGold`
  (for _array_element (`self.PlayersInTrigger`)
    (bind _asthird_person_character (cast `/Game/ThirdPersonBP/Blueprints/ThirdPersonCharacter` _array_element))
    (set `/Game/ThirdPersonBP/Blueprints/ThirdPersonCharacter.Coins` (+ (`/Game/ThirdPersonBP/Blueprints/ThirdPersonCharacter.Coins` _asthird_person_character) (`self.GoldToGive`)) _asthird_person_character)
    (bind _aswbp_player_score_increase (cast `/Game/ThirdPersonBP/Blueprints/UI/WBP_PlayerScoreIncrease` (`WidgetComponent.GetUserWidgetObject` (`/Game/ThirdPersonBP/Blueprints/ThirdPersonCharacter.ScoreIncrease` _asthird_person_character))))
    (set `/Game/ThirdPersonBP/Blueprints/UI/WBP_PlayerScoreIncrease.ScoreInt` (`self.GoldToGive`) _aswbp_player_score_increase)
    (`/Game/ThirdPersonBP/Blueprints/UI/WBP_PlayerScoreIncrease.PlayAnimIncrease` _aswbp_player_score_increase))
  (set `self.canMove` false)
  (`LightComponent.SetIntensity` (`self.PointLight`) 0.0)
  (`SceneComponent.SetVisibility` (`self.GoldPileGround`) false false)
  (`SceneComponent.SetVisibility` (`self.GoldPileGround2`) false false)
  (`SceneComponent.SetVisibility` (`self.Treasure`) false false))

(fn `UserConstructionScript`
  (`CableComponent.SetAttachEndToComponent` (`self.Cable1`) (`self.CableAttach1`) "None")
  (`CableComponent.SetAttachEndToComponent` (`self.Cable2`) (`self.CableAttach2`) "None"))